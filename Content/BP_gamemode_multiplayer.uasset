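; Local multiplayer game mode that creates players on a shared BP_camera and manages game start.
; On BeginPlay it matches PlayerStart tags to array indices, creates a player at each and possesses a spawned BP_InputReciever, removing CameraActors.
; SpawnPlayer temporarily handles spawning the character selected in BP_GameInstance at its input receiver and possessing it.
; StartGame flags the game as running and notifies the camera once enough players are active.
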(event `self.ReceiveBeginPlay`
  (bind _outactors (`GameplayStatics.GetAllActorsOfClass` "/Game/BP_camera.BP_camera_C"))
  (set `self.CameraRef` (`|GetArrayItem` _outactors))
  (`self.Get Player Start Point`)
  (`self.SpawnInputRecievers`))

(fn `GameStarted`
  (set `self.BIsInGame` true)
  (`/Game/BP_camera.GameStarted` (`self.CameraRef`))
  (`KismetSystemLibrary.PrintString` "Hello"))

(fn `Get Player Start Point`
  (bind _outactors (`GameplayStatics.GetAllActorsOfClass` "/Script/Engine.PlayerStart"))
  (set `self.PlayerStartArray` _outactors))

(fn `GetIsInGame`
  (returns (IsInGame :type Boolean))
  (return false))

(fn `NameToInt`
  (params (self2 :type "PlayerStart Object Reference"))
  (returns (ReturnValue :type Integer))
  (return (`KismetStringLibrary.Conv_StringToInt` (`KismetStringLibrary.Conv_NameToString` (`PlayerStart.PlayerStartTag` self2)))))

(fn `RemoveUnusedCameras`
  (bind _outactors (`GameplayStatics.GetAllActorsOfClass` "/Script/Engine.CameraActor"))
  (for _array_element _outactors
    (`self.K2_DestroyActor` _array_element)))

(fn `SpawnInputRecievers`
  (locals (Index :type Integer))
  (bind _returnvalue (`GameplayStatics.GetPlayerController` (`local.Index`)))
  (for (_ _array_index) (`self.PlayerStartArray`)
    (set `local.Index` _array_index)
    (for _array_element (`self.PlayerStartArray`)
      (if (== (`self.NameToInt` _array_element) (`local.Index`))
        (`GameplayStatics.CreatePlayer` -1)
        (bind _returnvalue_2 (`|SpawnActorFromClass` "/Game/BP_InputReciever.BP_InputReciever_C" (`self.GetTransform` (`|GetArrayItem` (`self.PlayerStartArray`) (`local.Index`))) "Undefined" "OverrideRootScale" null (`local.Index`) null))
        (`KismetArrayLibrary.Array_AddUnique` (`self.PlayerInputReciverArray`) _returnvalue_2)
        (`Controller.Possess` _returnvalue _returnvalue_2)
        (`KismetArrayLibrary.Array_AddUnique` (`self.PlayerControlerArray`) _returnvalue)
        (`PlayerController.SetViewTargetWithBlend` (`GameplayStatics.GetPlayerController` (`local.Index`)) (`self.CameraRef`) 0.0 "VTBlend_Linear" 0.0 false)))
    (`self.RemoveUnusedCameras`)))

(fn `SpawnPlayer__`
  (params (CurrentPlayerIndex :type Integer) (InputReceiver :type "/Game/BP_InputReciever Object Reference"))
  (returns (Return :type Boolean))
  (bind _currentplayerindex (`local.CurrentPlayerIndex`))
  (bind _returnvalue (`|SpawnActorFromClass` (`|GetArrayItem` (`/Game/BP_GameInstance.SelectedCharacters` (cast `/Game/BP_GameInstance` (`GameplayStatics.GetGameInstance`) :!pure true)) _currentplayerindex) (`self.GetTransform` (`local.InputReceiver`)) "Undefined" "OverrideRootScale" null _currentplayerindex null))
  (`KismetArrayLibrary.Array_Add` (`self.ActivePlayers`) _returnvalue)
  (`Controller.Possess` (`GameplayStatics.GetPlayerController` (`local.CurrentPlayerIndex`)) _returnvalue)
  (`PlayerController.SetViewTargetWithBlend` (`GameplayStatics.GetPlayerController` (`local.CurrentPlayerIndex`)) (`self.CameraRef`) 0.0 "VTBlend_Linear" 0.0 false)
  (return false))

(fn `StartGame`
  (returns (return :type Boolean))
  (if (>= (`KismetArrayLibrary.Array_Length` (`self.ActivePlayers`)) (`self.MinimumPlayers`))
    (`self.GameStarted`)
    (return false)))

(fn `UserConstructionScript`)