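; BP_CapturePointIndicator is the King of the Hill actor that marks a capture point with a screen-space indicator.
; Activate creates and letters a WBP_CapPointOffScreen widget; Deactivate removes it from the viewport.
; While active, Tick projects the actor's location, clamped near screen edges, rotating the widget toward off-screen points or to a fixed angle when on-screen.
; SetClockPercent and SetWidgetColor forward progress and color to the widget.
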(event `Activate`
  (`self.SetActorTickEnabled` true)
  (bind _returnvalue (`|CreateWidget` "/Game/GameMode/KotH/CapturePointIndicator/WBP_CapPointOffScreen.WBP_CapPointOffScreen_C"))
  (set `self.OffScreenWidget` _returnvalue)
  (`UserWidget.AddToViewport` _returnvalue 0)
  (`/Game/GameMode/KotH/CapturePointIndicator/WBP_CapPointOffScreen.SetLetter` (`self.OffScreenWidget`) (`self.Letter`))
  (set `self.IsActive` true))

(event `self.ReceiveTick`
  (params (DeltaSeconds :type "Float (single-precision)"))
  (bind _offscreenwidget (`self.OffScreenWidget`))
  (bind (_outscreenposition _outrotationangledegrees _bisonscreen) (`HUDBlueprintLibrary.FindScreenEdgeLocationForWorldLocation` (`self.K2_GetActorLocation`) 0.85 (0.5 0.45)))
  (if (`self.IsActive`)
    (`UserWidget.SetPositionInViewport` (`self.OffScreenWidget`) _outscreenposition true)
    (if _bisonscreen
      (`/Game/GameMode/KotH/CapturePointIndicator/WBP_CapPointOffScreen.SetAngle` _offscreenwidget 180.0)
      (else
        (`/Game/GameMode/KotH/CapturePointIndicator/WBP_CapPointOffScreen.SetAngle` _offscreenwidget _outrotationangledegrees)))))

(event `Deactivate`
  (bind _offscreenwidget (`self.OffScreenWidget`)
    (:`then`
      (`Widget.RemoveFromParent` _offscreenwidget))
    (:`else`)))

(fn `SetClockPercent`
  (params (Percent :type "Float (double-precision)"))
  (`/Game/GameMode/KotH/CapturePointIndicator/WBP_CapPointOffScreen.SetPercent` (`self.OffScreenWidget`) Percent))

(fn `SetWidgetColor`
  (params (Color :type "LinearColor Structure"))
  (`/Game/GameMode/KotH/CapturePointIndicator/WBP_CapPointOffScreen.SetColor` (`self.OffScreenWidget`) Color))

(fn `UserConstructionScript`)