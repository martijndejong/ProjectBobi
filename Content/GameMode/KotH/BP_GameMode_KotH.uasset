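; King of the Hill game mode that rotates an active capture point during a match.
; After BeginPlay, a timer activates a random BP_CapturePoint found in the level, which stays active for a fixed window.
; A second timer then deactivates every capture point and schedules the next random activation, so the two functions chain into an endless cycle with idle gaps between points.
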(event `self.ReceiveBeginPlay`
  (`parent.ReceiveBeginPlay`)
  (`KismetSystemLibrary.K2_SetTimer` null "ActivateRandomPoint" 15.0))

(fn `ActivateRandomPoint`
  (bind _outactors (`GameplayStatics.GetAllActorsOfClass` "/Game/GameMode/KotH/BP_CapturePoint.BP_CapturePoint_C"))
  (`/Game/GameMode/KotH/BP_CapturePoint.ActivatePoint` (`KismetArrayLibrary.Array_Random` _outactors))
  (`KismetSystemLibrary.K2_SetTimer` null "DeactivateAllPoints" 30.0))

(fn `DeactivateAllPoints`
  (bind _outactors (`GameplayStatics.GetAllActorsOfClass` "/Game/GameMode/KotH/BP_CapturePoint.BP_CapturePoint_C"))
  (for _array_element _outactors
    (`/Game/GameMode/KotH/BP_CapturePoint.DeactivePoint` _array_element))
  (`KismetSystemLibrary.K2_SetTimer` null "ActivateRandomPoint" 15.0))

(fn `UserConstructionScript`
  (`parent.UserConstructionScript`))