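; Timed King of the Hill capture point that players capture to earn score.
; A lone occupant drains rival possession before building their own; multiple occupants freeze it, and uncaptured progress decays when empty.
; Full possession crowns that player king, awarding points each second based on other player characters until possession empties or the point deactivates.
; Dynamic materials and spawned indicator and UI actors show progress, owner color and remaining time.
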(event `self.ReceiveBeginPlay`
  ;[1 1 1] All controllers in use (have Map in GameInstance) get zero possession
  (bind _asbp_game_instance (cast `/Game/BP_GameInstance` (`GameplayStatics.GetGameInstance`)))
  (bind _keys (`BlueprintMapLibrary.Map_Keys` (`/Game/BP_GameInstance.MapPlayerIndex` _asbp_game_instance)))
  (for _array_element _keys
    (`BlueprintMapLibrary.Map_Add` (`self.DictPossession`) _array_element)
    (bind _returnvalue (`PrimitiveComponent.CreateDynamicMaterialInstance` (`self.Plane`) 0 null "None"))
    (set `self.DynamicMaterialPlane` _returnvalue)
    (bind _returnvalue_2 (`|SpawnActorFromClass` "/Game/GameMode/KotH/CapturePointIndicator/BP_CapturePointIndicator.BP_CapturePointIndicator_C" (`KismetMathLibrary.MakeTransform` (+ (`self.K2_GetActorLocation`) (0.0 0.0 500.0))) "Undefined" "OverrideRootScale" null (`self.Letter`) null))
    (set `self.PointIndicator` _returnvalue_2)
    (bind _returnvalue_3 (`|SpawnActorFromClass` "/Game/GameMode/KotH/BP_CapturePointUI.BP_CapturePointUI_C" (`KismetMathLibrary.MakeTransform` (`self.K2_GetActorLocation`) (struct :`Yaw` -45.0)) "Undefined" "OverrideRootScale" null null))
    (set `self.PointUI` _returnvalue_3)
    (bind _returnvalue_4 (`PrimitiveComponent.CreateDynamicMaterialInstance` (`/Game/GameMode/KotH/BP_CapturePointUI.PlaneCirc` (`self.PointUI`)) 0 null "None"))
    (set `self.DynamicMaterialCircle` _returnvalue_4)
    (`/Game/GameMode/KotH/BP_CapturePointUI.SetLetter` (`self.PointUI`) (`self.Letter`))))

(event `self.ReceiveTick`
  (params (DeltaSeconds :type "Float (single-precision)"))
  (bind _dictpossession (`self.DictPossession`))
  (bind _pointactivetimer (`self.PointActiveTimer`))
  (bind _overlappingactors (`PrimitiveComponent.GetOverlappingActors` (`self.Box`) "/Game/Bobi/BobiCharacter.BobiCharacter_C"))
  (bind _returnvalue (`KismetSystemLibrary.K2_GetTimerRemainingTimeHandle` _pointactivetimer))
  (bind _returnvalue_2 (`KismetArrayLibrary.Array_Length` _overlappingactors))
  (if (`self.IsActive`)
    (`/Game/GameMode/KotH/CapturePointIndicator/BP_CapturePointIndicator.SetClockPercent` (`self.PointIndicator`) (/ _returnvalue (+ _returnvalue (`KismetSystemLibrary.K2_GetTimerElapsedTimeHandle` _pointactivetimer))))
    (`self.CrownFollowCharacter`)
    (if (== 1 _returnvalue_2)
      (`self.UpdatePossession` (cast `/Game/Bobi/BobiCharacter` (`|GetArrayItem` _overlappingactors) :!pure true))
      (`self.UpdateKing`)
      (elif (and (== _returnvalue_2 0) (== (`self.KingControllerID`) -1))
        (bind _maxid (`self.GetMaxPossID` (`self.DictPossession`)))
        ;[1 0.4888 0.3989] Decrease possession of highest player when not standing on uncapped point
        (`BlueprintMapLibrary.Map_Add` _dictpossession _maxid (`KismetMathLibrary.FClamp` (- (`BlueprintMapLibrary.Map_Find` _dictpossession _maxid) (/ (`self.PossPerTick`) 4.0))))
        (`self.UpdateAppearance`)))))

(fn `ActivatePoint`
  (params (Duration :type "Float (double-precision)"))
  (set `self.IsActive` true)
  (`self.SetActorHiddenInGame` false)
  (`self.SetActorTickEnabled` true)
  (`self.SetActorHiddenInGame` (`self.PointUI`) false)
  (bind _returnvalue (`KismetSystemLibrary.K2_SetTimer` null "DeactivatePoint" Duration))
  (set `self.PointActiveTimer` _returnvalue)
  (`/Game/GameMode/KotH/CapturePointIndicator/BP_CapturePointIndicator.Activate` (`self.PointIndicator`))
  (message `/Game/GameMode/BPI_GameMode.PutTextOnScreen` (`GameplayStatics.GetGameMode`) (`|FormatText` "CAPTURE POINT {x}!" (`self.Letter`)) 3.0))

(fn `Check Decrease Increase`
  (params (SelfControllerID :type Integer))
  (returns (Decrease :type Boolean) (ControllerID :type Integer))
  (locals (KingToDecrease :type Integer :default -1))
  (bind _keys (`BlueprintMapLibrary.Map_Keys` (`self.DictPossession`)))
  (for _array_element _keys
    (if (and (> (`BlueprintMapLibrary.Map_Find` (`self.DictPossession`) _array_element) 0.0) (!= _array_element SelfControllerID))
      (set `local.KingToDecrease` _array_element)))
  (if (!= (`local.KingToDecrease`) -1)
    (return true (`local.KingToDecrease`))
    (else
      (return false -1))))

(fn `ClearPossession`
  (bind _keys (`BlueprintMapLibrary.Map_Keys` (`self.DictPossession`)))
  (for _array_element _keys
    (`BlueprintMapLibrary.Map_Add` (`self.DictPossession`) _array_element)))

(fn `CrownFollowCharacter`
  (bind _crown (`self.Crown`))
  (bind _kingcontrollerid (`self.KingControllerID`))
  (if (== _kingcontrollerid -1)
    (`SceneComponent.SetVisibility` (`self.Crown`) false false :!label _label)
    (else
      (bind _bobicharacter (`/Game/Bobi/BP_PlayerController.BobiCharacter` (cast `/Game/Bobi/BP_PlayerController` (`GameplayStatics.GetPlayerControllerFromID` _kingcontrollerid) :!pure true))
        (:`then`
          (bind (_returnvalue_location _returnvalue_rotation) (`KismetMathLibrary.BreakTransform` (`self.GetTransform` _bobicharacter)))
          (`SceneComponent.K2_SetWorldTransform` (`self.Crown`) (`KismetMathLibrary.MakeTransform` (+ _returnvalue_location (0.0 0.0 130.0)) _returnvalue_rotation) false false)
          (if (not (`SceneComponent.IsVisible` _crown))
            (`SceneComponent.SetVisibility` _crown true false)))
        (:`else`
          (goto _label))))))

(fn `DeactivatePoint`
  (set `self.IsActive` false)
  (`self.SetActorHiddenInGame` true)
  (`self.SetActorTickEnabled` false)
  (`self.ClearPossession`)
  (`self.SetActorHiddenInGame` (`self.PointUI`) true)
  (`KismetSystemLibrary.K2_ClearAndInvalidateTimerHandle` (`self.GivePointLoopTimer`))
  (set `self.KingControllerID` -1)
  (`self.UpdateAppearance`)
  (`/Game/GameMode/KotH/CapturePointIndicator/BP_CapturePointIndicator.Deactivate` (`self.PointIndicator`)))

(fn `GetMaxPossID`
  (params (DictIntFloat :type "Map of Integer to Float (double-precision)"))
  (returns (MaxID :type Integer) (MaxPoss :type "Float (double-precision)"))
  (locals (CurrentHighValue :type "Float (double-precision)") (LocalCurrentMaxID :type Integer :default -1))
  (bind _currenthighvalue (`local.CurrentHighValue`))
  (bind _localcurrentmaxid (`local.LocalCurrentMaxID`))
  (bind _values (`BlueprintMapLibrary.Map_Values` DictIntFloat))
  (set `local.CurrentHighValue` (`.MaxValue` (`KismetMathLibrary.MaxOfFloatArray` _values)))
  (bind _keys (`BlueprintMapLibrary.Map_Keys` DictIntFloat))
  (for _array_element _keys
    (if (>= (`BlueprintMapLibrary.Map_Find` (`self.DictPossession`) _array_element) _currenthighvalue)
      (set `local.CurrentHighValue` _currenthighvalue)
      (set `local.LocalCurrentMaxID` _array_element)))
  (set `self.CurrentMaxID` _localcurrentmaxid)
  (return _localcurrentmaxid (`local.CurrentHighValue`)))

(fn `GivePoints`
  (bind _kingcontrollerid (`self.KingControllerID`))
  (if (!= _kingcontrollerid -1)
    (bind _outactors (`GameplayStatics.GetAllActorsOfClassWithTag` "/Game/Bobi/BobiCharacter.BobiCharacter_C" "PlayerCharacter"))
    (message `/Game/Bobi/BPI_PlayerState.IncrementScore` (`Controller.PlayerState` (`GameplayStatics.GetPlayerControllerFromID` _kingcontrollerid)) (`KismetMathLibrary.Clamp` (- (`KismetArrayLibrary.Array_Length` _outactors) 1) 0 100))))

(fn `PrintPossession`
  (bind _keys (`BlueprintMapLibrary.Map_Keys` (`self.DictPossession`)))
  (for _array_element _keys
    (`KismetSystemLibrary.PrintString` (`KismetStringLibrary.Conv_DoubleToString` (`BlueprintMapLibrary.Map_Find` (`self.DictPossession`) _array_element)) true true (`BlueprintMapLibrary.Map_Find` (`/Game/GameMode/BP_GameMode_Parent.PlayerToColor` (cast `/Game/GameMode/BP_GameMode_Parent` (`GameplayStatics.GetGameMode`) :!pure true)) _array_element))))

(fn `UpdateAppearance`
  (bind _dynamicmaterialcircle (`self.DynamicMaterialCircle`))
  (bind (_maxid _maxposs) (`self.GetMaxPossID` (`self.DictPossession`)))
  (`self.UpdateCurrentColor`)
  (`MaterialInstanceDynamic.SetVectorParameterValue` (`self.DynamicMaterialPlane`) "Color" (`KismetMathLibrary.LinearColorLerp` (struct :`R` 0.098958 :`G` 0.098958 :`B` 0.098958 :`A` 0.6) (`self.CurrentColor`) _maxposs))
  (`MaterialInstanceDynamic.SetScalarParameterValue` _dynamicmaterialcircle "Percent" _maxposs)
  (`MaterialInstanceDynamic.SetVectorParameterValue` _dynamicmaterialcircle "Color" (`self.CurrentColor`)))

(fn `UpdateCurrentColor`
  (bind _value (`BlueprintMapLibrary.Map_Find` (`/Game/GameMode/BP_GameMode_Parent.PlayerToColor` (cast `/Game/GameMode/BP_GameMode_Parent` (`GameplayStatics.GetGameMode`) :!pure true)) (`self.CurrentMaxID`)))
  (if (!= _value (`self.CurrentColor`))
    (set `self.CurrentColor` _value)))

(fn `UpdateKing`
  (locals (EncounteredKing :type Boolean))
  (set `local.EncounteredKing` false)
  (bind _keys (`BlueprintMapLibrary.Map_Keys` (`self.DictPossession`)))
  (for _array_element _keys
    (if (and (== (`BlueprintMapLibrary.Map_Find` (`self.DictPossession`) _array_element) 1.0) (!= _array_element (`self.KingControllerID`)))
      (set `self.KingControllerID` _array_element)
      (set `local.EncounteredKing` true)
      (bind _returnvalue (`KismetSystemLibrary.K2_SetTimer` null "GivePoints" 1.0 true))
      (set `self.GivePointLoopTimer` _returnvalue)
      (`/Game/GameMode/KotH/CapturePointIndicator/BP_CapturePointIndicator.SetWidgetColor` (`self.PointIndicator`) (`self.CurrentColor`))))
  (if (not (`local.EncounteredKing`))
    (if (== (`BlueprintMapLibrary.Map_Find` (`self.DictPossession`) (`self.KingControllerID`)) 0.0)
      (set `self.KingControllerID` -1)
      (set `self.CurrentColor` (struct :`R` 0.458333 :`G` 0.458333 :`B` 0.458333 :`A` 1.0))
      (`/Game/GameMode/KotH/CapturePointIndicator/BP_CapturePointIndicator.SetWidgetColor` (`self.PointIndicator`) (`self.CurrentColor`)))))

(fn `UpdatePossession`
  (params (BobiCharacter :type "/Game/Bobi/BobiCharacter Object Reference"))
  (bind _controllerid (`/Game/Bobi/BobiCharacter.ControllerID` BobiCharacter))
  (bind _dictpossession (`self.DictPossession`))
  (bind _dictpossession_2 (`self.DictPossession`))
  (bind (_decrease _controllerid_2) (`self.Check Decrease Increase` (`/Game/Bobi/BobiCharacter.ControllerID` BobiCharacter)))
  (if _decrease
    ;[1 0.4888 0.3989] Decrease possession of highest player
    (`BlueprintMapLibrary.Map_Add` _dictpossession _controllerid_2 (`KismetMathLibrary.FClamp` (- (`BlueprintMapLibrary.Map_Find` _dictpossession _controllerid_2) (* (`self.PossPerTick`) 2.0))))
    (else
      ;[0.5984 1 0.4792] Increase possession of player on point
      (`BlueprintMapLibrary.Map_Add` _dictpossession_2 _controllerid (`KismetMathLibrary.FClamp` (+ (`BlueprintMapLibrary.Map_Find` _dictpossession_2 _controllerid) (`self.PossPerTick`))))))
  (`self.UpdateAppearance`))

(fn `UserConstructionScript`)