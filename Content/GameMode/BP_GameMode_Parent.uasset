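; Parent game mode for a local multiplayer Bobi arena match on a shared camera, intended for child modes with their own rules.
; BeginPlay pulls character and player selections from BP_GameInstance, builds score HUDs and spawns players at indexed custom starts.
; Deaths update scores, spawn a BP_Respawner and trigger brief slow motion.
; Reaching the score limit ends the match with a victory screen; GameInstance reload calls temporarily work around material-loading bugs.
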(event `self.ReceiveBeginPlay`
  ;[1 1 1] Setting up / Starting game (we moeten dit als Parent GameMode houden, en dan children met eigen regels qua respawn en punten etc.)
  ;;[1 0.08294 0] TEMPORARY FIX TO INVISIBLE MATERIALS
  (bind _asbp_game_instance (cast `/Game/BP_GameInstance` (`GameplayStatics.GetGameInstance`)))
  (`/Game/BP_GameInstance.ReloadLevel` _asbp_game_instance)
  (bind _outactors (`GameplayStatics.GetAllActorsOfClass` "/Game/Bobi/BP_PlayerState.BP_PlayerState_C"))
  (for _array_element _outactors
    (add `/Game/Bobi/BP_PlayerState.UpdateScore` _array_element (delegate `HeardUpdateScore`)))
  ;;[1 1 1] Create container for player HUDs
  (bind _returnvalue (`|CreateWidget` "/Game/HUD/HUD_Container.HUD_Container_C"))
  (bind _output_get (set `self.HUDContainerRef` _returnvalue))
  (`UserWidget.AddToViewport` _output_get 0)
  ;;[1 1 1] Set reference to Camera
  (bind _outactors_2 (`GameplayStatics.GetAllActorsOfClass` "/Game/BP_CameraParent.BP_CameraParent_C"))
  (bind _output_get_2 (set `self.CameraRef` (`|GetArrayItem` _outactors_2)))
  (`PlayerController.SetViewTargetWithBlend` (`GameplayStatics.GetPlayerController` 0) _output_get_2 0.0 "VTBlend_Linear" 0.0 false)
  ;;[1 1 1] Populate PlayerStartArray
  (`self.OrganizeCustomStartArray`)
  ;;[1 1 1 1 16] Pull selected characters/Active controllers/Locked Players from GameInstance to GameMode and store
  (bind _asbp_game_instance_2 (cast `/Game/BP_GameInstance` (`GameplayStatics.GetGameInstance`)))
  (set `self.GM_MapSelectedCharacters` (`/Game/BP_GameInstance.MapSelectedCharacters` _asbp_game_instance_2))
  (set `self.GM_MapPlayerIndex` (`/Game/BP_GameInstance.MapPlayerIndex` _asbp_game_instance_2))
  (set `self.GM_MapLockedPlayers` (`/Game/BP_GameInstance.MapLockedPlayers` _asbp_game_instance_2))
  ;;[1 1 1] Spawn all locked players, and then start game
  (bind _keys (`BlueprintMapLibrary.Map_Keys` (`self.GM_MapPlayerIndex`)))
  (for _array_element_2 _keys
    (`self.AddPlayerScoreHUD` _array_element_2)
    (`self.SpawnPlayer` _array_element_2 (struct) true))
  (`KismetSystemLibrary.Delay` 2.0)
  (`self.StartGame`))

(event `HeardUpdateScore`
  (if (`self.IsGameActive`)
    (for _array_element (`self.HUDScoresRef`)
      (`/Game/HUD/HUD_Score.UpdateScore` _array_element)
      (`self.CheckEndGame`))))

(event `HeardBobiDie`
  (params (ControllerID :type Integer) (KillerID :type Integer) (DeathLocation :type "Transform Structure"))
  (if (`self.IsGameActive`)
    (`self.UpdatePlayerScore` ControllerID KillerID)
    (`|SpawnActorFromClass` "/Game/GameMode/BP_Respawner.BP_Respawner_C" DeathLocation "Undefined" "OverrideRootScale" null ControllerID DeathLocation 6.0 null)
    ;[1 1 1] Slow motion on death
    (`GameplayStatics.SetGlobalTimeDilation` 0.1)
    (bind (_direction _alpha) (`Timeline|FadeTimeSpeed` :!via `PlayFromStart`)
      (:`Update`
        (`GameplayStatics.SetGlobalTimeDilation` (`KismetMathLibrary.Lerp` (`GameplayStatics.GetGlobalTimeDilation`) 1.0 _alpha))))))

(event `/Game/GameMode/BPI_GameMode.RequestSpawnPlayer`
  (params (ControllerID :type Integer) (SpawnLocation :type "Transform Structure"))
  (`self.SpawnPlayer` ControllerID SpawnLocation (< (.z (.location SpawnLocation)) 0.0)))

(event `/Game/GameMode/BPI_GameMode.DisplayPauseMenu`
  ;[1 1 1] Pause menu
  (bind _returnvalue (`|CreateWidget` "/Game/GameMode/Pause/WBP_PauseMenu.WBP_PauseMenu_C"))
  (`UserWidget.AddToViewport` _returnvalue 0))

(fn `AddPlayerScoreHUD`
  (params (ControllerID :type Integer))
  (bind _hudscoreref (`/Game/HUD/HUD_Container.AddPlayerScoreHUD` (`self.HUDContainerRef`) ControllerID))
  (`KismetArrayLibrary.Array_AddUnique` (`self.HUDScoresRef`) _hudscoreref))

(fn `CheckEndGame`
  (if (`self.IsGameActive`)
    (bind _outactors (`GameplayStatics.GetAllActorsOfClass` "/Game/Bobi/BP_PlayerState.BP_PlayerState_C"))
    (for _array_element _outactors
      (if (>= (`/Game/Bobi/BP_PlayerState.CurrentScore` _array_element) 100)
        (set `self.IsGameActive` false)
        ;[1 0 0.02754] Find good delay value
        (`KismetSystemLibrary.K2_SetTimer` null "EndGame" 3.0)))))

(fn `DisplayPlayerHUD`
  (params (PlayerController :type "PlayerController Object Reference") (PlayerIndex :type Integer))
  (returns (PlayerHUD :type "/Game/HUD/HUD_Overhaul/HUD_PlayerCard Object Reference"))
  (bind _playerhud (`/Game/HUD/HUD_Container.AddPlayerHUD` (`self.HUDContainerRef`) PlayerController PlayerIndex))
  (return _playerhud))

(fn `EndGame`
  (set `self.IsGameActive` false)
  (`Widget.RemoveFromParent` (`self.HUDContainerRef`))
  (bind _outactors (`GameplayStatics.GetAllActorsOfClass` "/Game/Bobi/BobiCharacter.BobiCharacter_C"))
  (for _array_element _outactors
    (`self.K2_DestroyActor` _array_element))
  (bind _outactors_2 (`GameplayStatics.GetAllActorsOfClass` "/Game/GameMode/VictoryScreen/BP_VictoryScreen.BP_VictoryScreen_C"))
  (`/Game/GameMode/VictoryScreen/BP_VictoryScreen.ActivateVictorySCreen` (`|GetArrayItem` _outactors_2))
  ;[1 0 0] TEMPORARY FIX TO MATERIALS NOT LOADING BUG
  (bind _asbp_game_instance (cast `/Game/BP_GameInstance` (`GameplayStatics.GetGameInstance`)))
  (`/Game/BP_GameInstance.ResetReloadLevel` _asbp_game_instance))

(fn `NameToInt`
  (params (self2 :type "PlayerStart Object Reference"))
  (returns (ReturnValue :type Integer))
  (return (`KismetStringLibrary.Conv_StringToInt` (`KismetStringLibrary.Conv_NameToString` (`PlayerStart.PlayerStartTag` self2)))))

(fn `OrganizeCustomStartArray`
  (locals (EmptyArray :type "Array of /Game/CharacterSelectMenu/BP_CustomStart Object Reference"))
  (bind _outactors (`GameplayStatics.GetAllActorsOfClass` "/Game/CharacterSelectMenu/BP_CustomStart.BP_CustomStart_C"))
  (for _array_element _outactors
    (`KismetArrayLibrary.Array_Set` (`local.EmptyArray`) (`/Game/CharacterSelectMenu/BP_CustomStart.Index` _array_element) _array_element true)
    (set `self.CustomStartArray` (`local.EmptyArray`))))

(fn `PutTextOnScreen`
  (params (InputText :type Text) (Duration :type "Float (double-precision)"))
  (returns (dummy :type Boolean))
  (`/Game/HUD/HUD_Container.TextOnScreen` (`self.HUDContainerRef`) InputText Duration)
  (return false))

(fn `RemindCamera`
  (params (Controller :type "PlayerController Object Reference"))
  (returns (Dummy :type Boolean))
  (`PlayerController.SetViewTargetWithBlend` Controller (`self.CameraRef`) 0.0 "VTBlend_Linear" 0.0 false)
  (return false))

(fn `RemoveUnusedCameras`
  (bind _outactors (`GameplayStatics.GetAllActorsOfClass` "/Script/Engine.CameraActor"))
  (for _array_element _outactors
    (`self.K2_DestroyActor` _array_element)))

(fn `SpawnPlayer`
  (params (PlayerControllerID :type Integer) (SpawnLocation :type "Transform Structure") (SpawnAtBase :type Boolean) (SpawnAsGhost :type Boolean))
  (locals (DefiniteSpawnLocation :type "Transform Structure") (DefiniteSpawnClass :type "/Game/Bobi/BobiCharacter Class Reference"))
  (bind _playercontrollerid (`local.PlayerControllerID`))
  (if (`self.IsGameActive`)
    (set `local.DefiniteSpawnClass` (castclass `/Game/Bobi/BobiCharacter` (`KismetMathLibrary.SelectClass` "/Game/Bobi/BobiGhost/BP_BobiGhostCharacter.BP_BobiGhostCharacter_C" (`BlueprintMapLibrary.Map_Find` (`self.GM_MapSelectedCharacters`) (`local.PlayerControllerID`)) (`local.SpawnAsGhost`)) :!pure true))
    (set `local.DefiniteSpawnLocation` (select `bool` (`local.SpawnAtBase`) :`false` (`local.SpawnLocation`) :`true` (`self.GetTransform` (`|GetArrayItem` (`self.CustomStartArray`) (`BlueprintMapLibrary.Map_Find` (`self.GM_MapPlayerIndex`) (`local.PlayerControllerID`))))))
    (bind _returnvalue (`|SpawnActorFromClass` (`local.DefiniteSpawnClass`) (`local.DefiniteSpawnLocation`) "AlwaysSpawn" "OverrideRootScale" null _playercontrollerid (`GameplayStatics.GetPlayerController` _playercontrollerid) (`BlueprintMapLibrary.Map_Find` (`self.PlayerToColor`) _playercontrollerid) null))
    (`Controller.Possess` (`GameplayStatics.GetPlayerController` (`local.PlayerControllerID`)) _returnvalue)
    (`PlayerController.SetViewTargetWithBlend` (`GameplayStatics.GetPlayerController` (`local.PlayerControllerID`)) (`self.CameraRef`) 0.0 "VTBlend_Linear" 0.0 false)
    (`self.RemoveUnusedCameras`)
    (add `/Game/Bobi/BobiCharacter.BobiDied` _returnvalue (`|CreateDelegate` :!event `HeardBobiDie`))))

(fn `SpawnPlayer_legacy`
  (params (PlayerControllerID :type Integer) (SpawnLocation :type "Transform Structure") (SpawnAtBase :type Boolean) (SpawnAsGhost :type Boolean))
  (locals (DefiniteSpawnLocation :type "Transform Structure") (DefiniteSpawnClass :type "/Game/Bobi/BobiCharacter Class Reference"))
  (if SpawnAtBase
    (set `local.DefiniteSpawnLocation` (`self.GetTransform` (`|GetArrayItem` (`self.CustomStartArray`) (`BlueprintMapLibrary.Map_Find` (`self.GM_MapPlayerIndex`) PlayerControllerID))))
    (else
      (set `local.DefiniteSpawnLocation` SpawnLocation)))
  (if SpawnAsGhost
    (set `local.DefiniteSpawnClass` "/Game/Bobi/BobiGhost/BP_BobiGhostCharacter.BP_BobiGhostCharacter_C")
    (else
      (set `local.DefiniteSpawnClass` (`BlueprintMapLibrary.Map_Find` (`self.GM_MapSelectedCharacters`) PlayerControllerID))))
  (bind _returnvalue (`|SpawnActorFromClass` (`local.DefiniteSpawnClass`) (`local.DefiniteSpawnLocation`) "Undefined" "OverrideRootScale" null PlayerControllerID (`GameplayStatics.GetPlayerController` PlayerControllerID) (`BlueprintMapLibrary.Map_Find` (`self.PlayerToColor`) PlayerControllerID) null))
  (`Controller.Possess` (`GameplayStatics.GetPlayerController` (`local.PlayerControllerID`)) _returnvalue)
  (`PlayerController.SetViewTargetWithBlend` (`GameplayStatics.GetPlayerController` (`local.PlayerControllerID`)) (`self.CameraRef`) 0.0 "VTBlend_Linear" 0.0 false)
  (`self.RemoveUnusedCameras`)
  (add `/Game/Bobi/BobiCharacter.BobiDied` _returnvalue (`|CreateDelegate` :!event `HeardBobiDie`)))

(fn `StartGame`
  (`/Game/BP_CameraParent.GameStarted` (`self.CameraRef`)))

(fn `UpdatePlayerScore`
  (params (ControllerID :type Integer) (KillerID :type Integer))
  (if (== KillerID -1)
    ;[1 1 1] Suicide
    (message `/Game/Bobi/BPI_PlayerState.IncrementScore` (`Controller.PlayerState` (`GameplayStatics.GetPlayerControllerFromID` ControllerID)) -3)
    (else
      ;[1 1 1] Kill
      (message `/Game/Bobi/BPI_PlayerState.IncrementScore` (`Controller.PlayerState` (`GameplayStatics.GetPlayerControllerFromID` KillerID)) 5))))

(fn `UserConstructionScript`)