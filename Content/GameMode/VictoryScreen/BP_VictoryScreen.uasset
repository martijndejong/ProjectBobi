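; Victory screen actor that shows players' characters and a scoreboard ranked by score.
; On BeginPlay it hides four podium meshes and caches player index and color maps from the game instance and game mode.
; Activation sorts controller IDs by PlayerState score, then assigns each selected character mesh by rank with a per-controller custom depth stencil.
; It then switches all player views to itself and fills WBP_ScoreBoard in ranked order.
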(event `self.ReceiveBeginPlay`
  (bind _output_get (set `self.SkeletalMeshArray` (`|MakeArray` (`self.SkeletalMesh1`) (`self.SkeletalMesh2`) (`self.SkeletalMesh3`) (`self.SkeletalMesh4`))))
  (for _array_element _output_get
    (`SceneComponent.SetHiddenInGame` _array_element true false))
  (bind _asbp_game_instance (cast `/Game/BP_GameInstance` (`GameplayStatics.GetGameInstance`)))
  (set `self.ControllerToPlayerIndex` (`/Game/BP_GameInstance.MapPlayerIndex` _asbp_game_instance))
  (set `self.PlayerToColor` (`/Game/GameMode/BP_GameMode_Parent.PlayerToColor` (cast `/Game/GameMode/BP_GameMode_Parent` (`GameplayStatics.GetGameMode`) :!pure true)))
  (`self.SetActorTickEnabled` false))

(event `ActivateVictorySCreen`
  (`self.SetActorTickEnabled` true)
  (`self.SetActorHiddenInGame` false)
  (`self.Rank Players`)
  (`self.SetCharacterAppearances`)
  (`self.SetAllCamerasToVictoryScreen`)
  (bind _returnvalue (`|CreateWidget` "/Game/GameMode/VictoryScreen/WBP_ScoreBoard.WBP_ScoreBoard_C"))
  (bind _output_get (set `self.WBP_ScoreBoard` _returnvalue))
  (`UserWidget.AddToViewport` _output_get 0)
  (for _array_element (`self.SortedControllerIDs`)
    (`/Game/GameMode/VictoryScreen/WBP_ScoreBoard.AddPlayerRowToGrid` (`self.WBP_ScoreBoard`) _array_element (`BlueprintMapLibrary.Map_Find` (`self.ControllerToPlayerIndex`) _array_element) (`BlueprintMapLibrary.Map_Find` (`self.PlayerToColor`) _array_element))))

(fn `Rank Players`
  (locals (PlayerScores :type "Array of Integer") (ControllerIDs :type "Array of Integer") (IndexOfMaxScore :type Integer))
  (bind _indexofmaxscore (`local.IndexOfMaxScore`))
  (bind _keys (`BlueprintMapLibrary.Map_Keys` (`self.ControllerToPlayerIndex`)))
  (bind _output_get (set `local.ControllerIDs` _keys))
  (for _array_element _output_get
    (bind _asbp_player_state (cast `/Game/Bobi/BP_PlayerState` (`Controller.PlayerState` (`GameplayStatics.GetPlayerControllerFromID` _array_element))))
    (`KismetArrayLibrary.Array_Add` (`local.PlayerScores`) (`/Game/Bobi/BP_PlayerState.CurrentScore` _asbp_player_state)))
  (while (> (`KismetArrayLibrary.Array_Length` (`local.ControllerIDs`)) 0)
    (set `local.IndexOfMaxScore` (`KismetMathLibrary.MaxOfIntArray` (`local.PlayerScores`)))
    (`KismetArrayLibrary.Array_Add` (`self.SortedControllerIDs`) (`|GetArrayItem` (`local.ControllerIDs`) (`local.IndexOfMaxScore`)))
    (`KismetArrayLibrary.Array_Remove` (`local.PlayerScores`) _indexofmaxscore)
    (`KismetArrayLibrary.Array_Remove` (`local.ControllerIDs`) _indexofmaxscore)))

(fn `SetAllCamerasToVictoryScreen`
  (bind _outactors (`GameplayStatics.GetAllActorsOfClass` "/Script/Engine.PlayerController"))
  (for _array_element _outactors
    (`PlayerController.SetViewTargetWithBlend` _array_element self 0.0 "VTBlend_Linear" 0.0 false)))

(fn `SetCharacterAppearances`
  (locals (ControllerToCharacter :type "Map of Integer to /Game/Bobi/BobiCharacter Class Reference"))
  (bind _asbp_game_instance (cast `/Game/BP_GameInstance` (`GameplayStatics.GetGameInstance`)))
  (set `local.ControllerToCharacter` (`/Game/BP_GameInstance.MapSelectedCharacters` _asbp_game_instance))
  (for (_array_element _array_index) (`self.SortedControllerIDs`)
    (bind _output (`|GetArrayItem` (`self.SkeletalMeshArray`) _array_index))
    (`SceneComponent.SetHiddenInGame` _output false false)
    (`SkinnedMeshComponent.SetSkinnedAssetAndUpdate` _output (`.CharacterMesh` (defaults `Object` (`BlueprintMapLibrary.Map_Find` (`local.ControllerToCharacter`) _array_element))) true)
    (`PrimitiveComponent.SetCustomDepthStencilValue` _output (+ _array_element 1))))

(fn `UserConstructionScript`)