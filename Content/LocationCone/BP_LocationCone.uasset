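; BP_LocationCone is a player-colored ground marker that shows where its owning BobiCharacter is above the floor.
; On BeginPlay it attaches to its owner, tints the cone and aim circle through dynamic materials, and binds its destruction to the owner's.
; Each tick a capsule-radius sphere trace finds the floor below, places the actor there and stretches the cone up to the character, increasing its opacity with height.
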(event `self.ReceiveBeginPlay`
  (bind _returnvalue (`self.GetOwner`))
  (bind (_returnvalue_x _returnvalue_y _returnvalue_z) (`KismetMathLibrary.BreakVector` (`self.K2_GetActorLocation` _returnvalue)))
  (set `self.PlaneHeight` _returnvalue_z)
  (`self.K2_AttachToActor` _returnvalue "None" "SnapToTarget" "SnapToTarget" "SnapToTarget" false)
  (bind _returnvalue_2 (`PrimitiveComponent.CreateDynamicMaterialInstance` (`self.LocationCone`) 0 null "None"))
  (bind _output_get (set `self.ConeMaterial` _returnvalue_2))
  (`MaterialInstanceDynamic.SetVectorParameterValue` _output_get "color" (`self.Color`))
  (bind _returnvalue_3 (`PrimitiveComponent.CreateDynamicMaterialInstance` (`self.AimCircle`) 0 null "None"))
  (`MaterialInstanceDynamic.SetVectorParameterValue` _returnvalue_3 "PlayerColor" (`self.Color`))
  (add `self.OnDestroyed` (`self.GetOwner`) (delegate `DestroyActor`)))

(event `DestroyActor` :!signature `self.OnDestroyed`
  (params (DestroyedActor :type "Actor Object Reference"))
  (`self.K2_DestroyActor`))

(event `self.ReceiveTick`
  (params (DeltaSeconds :type "Float (single-precision)"))
  (bind _returnvalue (`self.GetOwner`))
  (bind _returnvalue_2 (/ (- (.z (`self.CurrentActorLocation`)) (`self.PlaneHeight`)) 100.0))
  (`/Engine/EditorBlueprintResources/StandardMacros.IsValid` _returnvalue
    (:`Is Valid`
      (bind _output_get (set `self.CurrentActorLocation` (`self.K2_GetActorLocation` _returnvalue)))
      (bind (_outhit _returnvalue_3) (`KismetSystemLibrary.SphereTraceSingleForObjects` _output_get (- (`self.CurrentActorLocation`) (0.0 0.0 1000.0)) (`CapsuleComponent.CapsuleRadius` (`Character.CapsuleComponent` (cast `/Game/Bobi/BobiCharacter` _returnvalue :!pure true))) (`|MakeArray` "ObjectTypeQuery1" :!type "EObjectTypeQuery Enum")))
      (if _returnvalue_3
        (bind _output_get_2 (set `self.PlaneHeight` (.z (`.Location` (`GameplayStatics.BreakHitResult` _outhit))))))
      (`self.K2_SetActorLocation` (`KismetMathLibrary.MakeVector` (.x (`self.CurrentActorLocation`)) (.y (`self.CurrentActorLocation`)) _output_get_2))
      (`SceneComponent.SetWorldScale3D` (`self.LocationCone`) (`KismetMathLibrary.MakeVector` 1.0 1.0 _returnvalue_2))
      (`MaterialInstanceDynamic.SetScalarParameterValue` (`self.ConeMaterial`) "opacity" (`KismetMathLibrary.MapRangeClamped` (`KismetMathLibrary.Abs` _returnvalue_2) 1.0 5.0 0.0 0.6)))))

(fn `UserConstructionScript`)