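; Charged electric arrow ability actor that fires a projectile along its owner's forward direction.
; BeginPlay starts charge effects and sound, then activation stops them, launches the arrow and enables box collision after a brief delay.
; CastProgress scales launch velocity, damage, knockback and audiovisual intensity.
; Overlapping a non-owner deals damage and knocks back BobiCharacters; hits and projectile stops both spawn impact effects and destroy the arrow.
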(event `self.ReceiveBeginPlay`
  (`parent.ReceiveBeginPlay`)
  (`NiagaraComponent.SetVariableFloat` (`self.NiagaraCharge`) "LoopTime" (`.CastTime_13_A8FA76814444CC207308189C68ECC29B` (break `/Game/AbilitySystem/AbilityDetailsStruct` (`self.AbilityDetails`))))
  (bind _returnvalue (`GameplayStatics.SpawnSoundAtLocation` "/Game/AbilitySystem/Arrow/S_PowerCharge.S_PowerCharge" (`self.K2_GetActorLocation`) (struct) 1.0 1.0 0.0 null null))
  (set `self.ChargeSoundRef` _returnvalue))

(event `self.ActivateAbility`
  (bind _projectilemovement (`self.ProjectileMovement`))
  (bind _returnvalue (`KismetMathLibrary.MapRangeClamped` (`self.CastProgress`) 0.0 1.0 0.15 1.0))
  (`parent.ActivateAbility`)
  (`GameplayStatics.PlaySoundAtLocation` "/Game/AbilitySystem/Arrow/S_ElectricShoot.S_ElectricShoot" (`self.K2_GetActorLocation`) (struct) (`KismetMathLibrary.FClamp` _returnvalue 0.3) 1.0 0.0 null null null)
  (`AudioComponent.Stop` (`self.ChargeSoundRef`))
  (`NiagaraComponent.SetVariableBool` (`self.NiagaraCharge`) "KillChargeParticles" true)
  (set `MovementComponent.Velocity` (+ (* (`self.GetActorForwardVector` (`self.AbilityOwner`)) (* (`self.LaunchSpeed`) _returnvalue)) (`KismetMathLibrary.MakeVector` 0.0 0.0 (* (`self.VerticalSpeed`) _returnvalue))) _projectilemovement)
  (`ActorComponent.Activate` _projectilemovement false)
  (`KismetSystemLibrary.Delay` 0.01)
  (`PrimitiveComponent.SetCollisionEnabled` (`self.Box`) "QueryAndPhysics"))

(event `self.ReceiveDestroyed`
  (`parent.ReceiveDestroyed`)
  (bind _chargesoundref (`self.ChargeSoundRef`)
    (:`then`
      (`AudioComponent.Stop` _chargesoundref))
    (:`else`)))

(event `self.Box.OnComponentBeginOverlap`
  (params (OverlappedComponent :type "PrimitiveComponent Object Reference") (OtherActor :type "Actor Object Reference") (OtherComp :type "PrimitiveComponent Object Reference") (OtherBodyIndex :type Integer) (bFromSweep :type Boolean) (SweepResult :type "HitResult Structure (by ref)"))
  (bind _returnvalue (`KismetMathLibrary.MapRangeClamped` (`self.CastProgress`) 0.0 1.0 0.1 1.0))
  ;[1 1 1] Copy pasted from melee
  (if (not (== OtherActor (`self.AbilityOwner`)))
    (`/Engine/EditorBlueprintResources/StandardMacros.IsValid` OtherActor
      (:`Is Valid`
        (`GameplayStatics.ApplyDamage` OtherActor (* _returnvalue (`.Damage_29_66822423450AE486B2C9FE8E4C4D325E` (break `/Game/AbilitySystem/AbilityDetailsStruct` (`self.AbilityDetails`)))) (`Pawn.GetController` (`self.AbilityOwner`)))
        (`self.ExplosionParticles` (`self.K2_GetActorLocation` OtherActor))
        (`self.K2_DestroyActor`)
        (bind _asbobi_character (cast `/Game/Bobi/BobiCharacter` OtherActor))
        (`/Engine/EditorBlueprintResources/StandardMacros.IsValid` _asbobi_character
          (:`Is Valid`
            (`Character.LaunchCharacter` _asbobi_character (+ (* (* (`KismetMathLibrary.Normal` (`self.GetVelocity`)) 500.0) _returnvalue) (0.0 0.0 300.0)) false false)))))))

(event `self.ProjectileMovement.OnProjectileStop`
  (params (ImpactResult :type "HitResult Structure (by ref)"))
  (`PrimitiveComponent.SetSimulatePhysics` (`self.StaticMesh`) true)
  (`PrimitiveComponent.SetCollisionEnabled` (`self.Box`) "NoCollision")
  (`self.ExplosionParticles` ImpactResult_ImpactPoint))

(event `ExplosionParticles`
  (params (Location :type "Vector Structure"))
  (bind _castprogress (`self.CastProgress`))
  (bind _returnvalue (`NiagaraFunctionLibrary.SpawnSystemAtLocation` "/Game/AbilitySystem/Arrow/P_ArrowImpact.P_ArrowImpact" Location))
  (`NiagaraComponent.SetVariableInt` _returnvalue "MultiplyFactor" (`KismetMathLibrary.FTrunc` (`KismetMathLibrary.MapRangeClamped` (`self.CastProgress`) 0.0 1.0 2.0 8.0)))
  (`GameplayStatics.PlaySoundAtLocation` "/Game/AbilitySystem/Arrow/S_ElectricImpact.S_ElectricImpact" (`self.K2_GetActorLocation`) (struct) (`KismetMathLibrary.MapRangeClamped` _castprogress 0.0 1.0 0.1 0.7) (`KismetMathLibrary.MapRangeClamped` _castprogress 0.0 1.0 1.0 0.7) 0.0 null null null)
  (`self.K2_DestroyActor`))

(fn `UserConstructionScript`
  (`parent.UserConstructionScript`))