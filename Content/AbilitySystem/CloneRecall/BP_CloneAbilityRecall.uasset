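; BP_CloneAbilityRecall is a clone ability actor that recalls its owner to its own position.
; When InteractPress receives the default key, it sends InteractAlternative to BP_AbilityCloneHandler actors overlapping the owner, passing the owner along.
; It then moves the owner to its location without sweeping and destroys itself.
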(event `/Game/AbilitySystem/BPI_AbilityParent.InteractPress`
  (params (Key :type "Key Structure"))
  (bind _abilityowner (`self.AbilityOwner`))
  (if (== Key (`self.DefaultKey`))
    (message `/Game/AbilitySystem/BPI_AbilityParent.InteractAlternativeEvent` (`self.GetOverlappingActors` _abilityowner "/Game/AbilitySystem/CloneStationary/BP_AbilityCloneHandler.BP_AbilityCloneHandler_C") _abilityowner)
    (`self.K2_SetActorLocation` (`self.AbilityOwner`) (`self.K2_GetActorLocation`) false false)
    (`self.K2_DestroyActor`)))

(fn `UserConstructionScript`
  (`parent.UserConstructionScript`))