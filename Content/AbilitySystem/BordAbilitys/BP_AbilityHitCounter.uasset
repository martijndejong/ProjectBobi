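; Combo ability actor that attaches to its owner and rewards consecutive hits with bonus damage and a movement speed modifier.
; Each valid hit raises a capped counter and restarts a timeout timer, while an invalid hit clears the counter.
; Registered hits push the scaled multipliers to the owner through SetDamageMultiplier and AddSlowEffect.
; The timeout only zeroes and prints the counter, leaving applied multipliers unchanged until the next registered hit.
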(event `self.ReceiveBeginPlay`
  (`self.K2_AttachToActor` (`self.AbilityOwner`) "None" "SnapToTarget" "SnapToTarget" "SnapToTarget" false))

(event `ResetHits`
  (bind _output_get (set `self.ConsecutiveHits` 0))
  (`KismetSystemLibrary.PrintString` (`KismetStringLibrary.Conv_IntToString` _output_get)))

(event `RegisteredHit`
  (params (ValidHit :type Boolean))
  (if ValidHit
    (set `self.ConsecutiveHits` (+ (`self.ConsecutiveHits`) 1))
    (`KismetSystemLibrary.K2_SetTimerDelegate` (delegate `ResetHits`) (`self.TimeBetweenHits`))
    (if (> (`self.ConsecutiveHits`) 5)
      (set `self.ConsecutiveHits` 5)
      (else
        (bind _output_get (set `self.ConsecutiveHits` (`self.ConsecutiveHits`)))))
    (set `self.BonusDamage` (+ (* (`self.BonusDamagePerHit`) (`KismetMathLibrary.Conv_IntToDouble` _output_get)) 1.0))
    (else
      (set `self.ConsecutiveHits` 0)
      (set `self.BonusDamage` 1.0)))
  (`/Game/Bobi/BobiCharacter.SetDamageMultiplier` (`self.AbilityOwner`) (`self.BonusDamage`))
  (`/Game/Bobi/BobiCharacter.AddSlowEffect` (`self.AbilityOwner`) (+ (* (`self.ConsecutiveHits`) (`self.BonusMovmentSpeedPerHit`)) 1.0)))

(fn `UserConstructionScript`
  (`parent.UserConstructionScript`))