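; Electric arrow ability actor that charges during the cast, then launches as a projectile along the owner's forward vector with added lift.
; While charging it plays looping-timed Niagara and sound, and after a second raises the owner's left-hand IK until release.
; CastProgress scales launch speed, damage, stun, knockback and impact effects.
; Box overlap or projectile stop spawns the impact burst and destroys the arrow; hit-counter logic is unwired.
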(event `self.ReceiveBeginPlay`
  (`parent.ReceiveBeginPlay`)
  (`self.K2_SetActorRotation` (struct :`Pitch` -80.0 :`Yaw` -30.0) true)
  (`NiagaraComponent.SetVariableFloat` (`self.NiagaraCharge`) "LoopTime" (`.CastTime_13_A8FA76814444CC207308189C68ECC29B` (break `/Game/AbilitySystem/AbilityDetailsStruct` (`self.AbilityDetails`))))
  (bind _returnvalue (`GameplayStatics.SpawnSoundAtLocation` "/Game/AbilitySystem/BordAbilitys/Arrow/S_PowerCharge.S_PowerCharge" (`self.K2_GetActorLocation`) (struct) 1.0 1.0 0.0 null null))
  (set `self.ChargeSoundRef` _returnvalue)
  (bind _returnvalue_2 (`KismetSystemLibrary.K2_SetTimer` null "SetIKforward" 1.0)))

(event `self.ActivateAbility`
  (bind _projectilemovement (`self.ProjectileMovement`))
  (bind _returnvalue (`KismetMathLibrary.MapRangeClamped` (`self.CastProgress`) 0.0 1.0 0.3 1.0))
  (`parent.ActivateAbility`)
  (`GameplayStatics.PlaySoundAtLocation` "/Game/AbilitySystem/BordAbilitys/Arrow/S_ElectricShoot.S_ElectricShoot" (`self.K2_GetActorLocation`) (struct) (`KismetMathLibrary.FClamp` _returnvalue 0.3) 1.0 0.0 null null null)
  (`AudioComponent.Stop` (`self.ChargeSoundRef`))
  (`NiagaraComponent.SetVariableBool` (`self.NiagaraCharge`) "KillChargeParticles" true)
  (set `MovementComponent.Velocity` (+ (* (`self.GetActorForwardVector` (`self.AbilityOwner`)) (* (`self.LaunchSpeed`) _returnvalue)) (`KismetMathLibrary.MakeVector` 0.0 0.0 (* (`self.VerticalSpeed`) _returnvalue))) _projectilemovement)
  (`ActorComponent.Activate` _projectilemovement false)
  (`KismetSystemLibrary.Delay` 0.01)
  (`PrimitiveComponent.SetCollisionEnabled` (`self.Box`) "QueryAndPhysics")
  (`KismetSystemLibrary.K2_ClearAndInvalidateTimerHandle` (stale `self.ReceiveBeginPlay` _returnvalue_2))
  (`/Game/Bobi/BobiCharacter.SetIKinfo` (`self.AbilityOwner`) 0.0 (0.0 0.0 0.0) 0.0 (0.0 0.0 0.0)))

(event `self.Box.OnComponentBeginOverlap`
  (params (OverlappedComponent :type "PrimitiveComponent Object Reference") (OtherActor :type "Actor Object Reference") (OtherComp :type "PrimitiveComponent Object Reference") (OtherBodyIndex :type Integer) (bFromSweep :type Boolean) (SweepResult :type "HitResult Structure (by ref)"))
  (bind _returnvalue (`KismetMathLibrary.MapRangeClamped` (`self.CastProgress`) 0.0 1.0 0.25 1.0))
  ;[1 1 1] Copy pasted from melee
  (if (not (== OtherActor (`self.AbilityOwner`)))
    (`/Engine/EditorBlueprintResources/StandardMacros.IsValid` OtherActor
      (:`Is Valid`
        (`GameplayStatics.ApplyDamage` OtherActor (* (`/Game/Bobi/BobiCharacter.DamageMultiplier` (`self.AbilityOwner`)) (* _returnvalue (`.Damage_29_66822423450AE486B2C9FE8E4C4D325E` (break `/Game/AbilitySystem/AbilityDetailsStruct` (`self.AbilityDetails`))))) (`Pawn.GetController` (`self.AbilityOwner`)))
        (message `/Game/Bobi/BPI_BobiCharacter.AddStunEffect` OtherActor (* _returnvalue (`self.StunDuration`)))
        (`self.ExplosionParticles` (`self.K2_GetActorLocation` OtherActor))
        (`self.K2_DestroyActor`)
        (`self.Knockback` OtherActor _returnvalue)))))

(event `self.ProjectileMovement.OnProjectileStop`
  (params (ImpactResult :type "HitResult Structure (by ref)"))
  (`PrimitiveComponent.SetSimulatePhysics` (`self.StaticMesh`) true)
  (`PrimitiveComponent.SetCollisionEnabled` (`self.Box`) "NoCollision")
  (`self.ExplosionParticles` ImpactResult_ImpactPoint))

(event `self.ReceiveDestroyed`
  (`parent.ReceiveDestroyed`)
  (bind _chargesoundref (`self.ChargeSoundRef`)
    (:`then`
      (`AudioComponent.Stop` _chargesoundref))
    (:`else`)))

(event `ExplosionParticles`
  (params (Location :type "Vector Structure"))
  (bind _castprogress (`self.CastProgress`))
  (bind _returnvalue (`NiagaraFunctionLibrary.SpawnSystemAtLocation` "/Game/AbilitySystem/BordAbilitys/Arrow/P_ArrowImpact.P_ArrowImpact" Location))
  (`NiagaraComponent.SetVariableInt` _returnvalue "MultiplyFactor" (`KismetMathLibrary.FTrunc` (`KismetMathLibrary.MapRangeClamped` (`self.CastProgress`) 0.0 1.0 2.0 8.0)))
  (`GameplayStatics.PlaySoundAtLocation` "/Game/AbilitySystem/BordAbilitys/Arrow/S_ElectricImpact.S_ElectricImpact" (`self.K2_GetActorLocation`) (struct) (`KismetMathLibrary.MapRangeClamped` _castprogress 0.0 1.0 0.1 0.7) (`KismetMathLibrary.MapRangeClamped` _castprogress 0.0 1.0 1.0 0.7) 0.0 null null null)
  (`self.K2_DestroyActor`))

(fn `SetHitCounterRef`
  (for _array_element (`PrimitiveComponent.GetOverlappingActors` (`Character.CapsuleComponent` (`self.AbilityOwner`)) "/Game/AbilitySystem/BordAbilitys/BP_AbilityHitCounter.BP_AbilityHitCounter_C")
    (if (== (`GameplayStatics.GetObjectClass` _array_element) "/Game/AbilitySystem/BordAbilitys/BP_AbilityHitCounter.BP_AbilityHitCounter_C")
      (set `self.HitCounterRef` (cast `/Game/AbilitySystem/BordAbilitys/BP_AbilityHitCounter` _array_element :!pure true)))))

(fn `SetIKforward`
  (`/Game/Bobi/BobiCharacter.SetIKinfo` (`self.AbilityOwner`) 0.0 (0.0 0.0 0.0) 0.5 (30.0 60.0 120.0)))

(fn `UserConstructionScript`
  (`parent.UserConstructionScript`))