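; Jetpack ability actor that launches its owning character upward on spawn and keeps it hovering until the ability is activated or the actor is destroyed.
; While flying, it lowers gravity and raises air control and falling deceleration, then restores them on exit.
; After a short delay, Tick traces downward, nudging the character up over detected objects and zeroing vertical velocity below the flight ceiling.
; Activating the ability ends flight and destroys the actor.
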(event `self.ReceiveBeginPlay`
  (bind (_returnvalue_x _returnvalue_y _returnvalue_z) (`KismetMathLibrary.BreakVector` (`self.K2_GetActorLocation`)))
  (`parent.ReceiveBeginPlay`)
  (set `self.InitialHeight` _returnvalue_z)
  (`Character.LaunchCharacter` (`self.AbilityOwner`) (0.0 0.0 300.0) false true)
  (`self.SetFlying` true)
  (`KismetSystemLibrary.Delay` 0.5)
  (set `self.CheckHeight` true))

(event `self.ActivateAbility`
  (`parent.ActivateAbility`)
  (`self.SetFlying` false)
  (`self.K2_DestroyActor`))

(event `self.ReceiveTick`
  (params (DeltaSeconds :type "Float (single-precision)"))
  (bind _returnvalue (`self.K2_GetActorLocation`))
  (bind (_returnvalue_x _returnvalue_y _returnvalue_z) (`KismetMathLibrary.BreakVector` (`self.K2_GetActorLocation`)))
  (bind (_returnvalue_x_2 _returnvalue_y_2 _returnvalue_z_2) (`KismetMathLibrary.BreakVector` (`self.K2_GetActorLocation`)))
  (if (`self.CheckHeight`)
    (bind (_outhit _returnvalue_2) (`KismetSystemLibrary.LineTraceSingleForObjects` _returnvalue (- _returnvalue (`KismetMathLibrary.MakeVector` 0.0 0.0 (+ (`self.FlightHeight`) 50.0))) (`self.Object Types`)))
    (if _returnvalue_2
      (`Character.LaunchCharacter` (`self.AbilityOwner`) (0.0 0.0 10.0) false true)
      (set `self.InitialHeight` _returnvalue_z_2))
    (if (and (< _returnvalue_z (+ (`self.InitialHeight`) (`self.FlightHeight`))) (`self.CheckHeight`))
      (`self.SetVerticalVelocity` 0.0))))

(event `self.ReceiveDestroyed`
  (`parent.ReceiveDestroyed`)
  (`self.SetFlying` false))

(fn `SetFlying`
  (params (Flying :type Boolean))
  (bind _abilityowner (`self.AbilityOwner`)
    (:`then`
      (if Flying
        (bind _charactermovement (`Character.CharacterMovement` _abilityowner))
        (set `CharacterMovementComponent.GravityScale` 0.3 _charactermovement)
        (set `CharacterMovementComponent.AirControl` 0.8 _charactermovement)
        (set `CharacterMovementComponent.BrakingDecelerationFalling` 700.0 _charactermovement)
        (else
          (set `CharacterMovementComponent.GravityScale` 1.0 _charactermovement)
          (set `CharacterMovementComponent.AirControl` (`/Game/Bobi/BobiCharacter.BobiAirControl` (`self.AbilityOwner`)) _charactermovement)
          (set `CharacterMovementComponent.BrakingDecelerationFalling` 0.0 _charactermovement))))
    (:`else`)))

(fn `SetVerticalVelocity`
  (params (ZVelocity :type "Float (double-precision)"))
  (bind _charactermovement (`Character.CharacterMovement` (`self.AbilityOwner`)))
  (bind (_velocity_x _velocity_y) (`KismetMathLibrary.BreakVector` (`MovementComponent.Velocity` _charactermovement)))
  (set `MovementComponent.Velocity` (`KismetMathLibrary.MakeVector` _velocity_x _velocity_y ZVelocity) _charactermovement))

(fn `UserConstructionScript`
  (`parent.UserConstructionScript`))