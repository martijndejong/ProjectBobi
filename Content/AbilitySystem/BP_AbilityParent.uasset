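; Base actor for abilities, handling the cast phase, activation and interruption.
; It attaches to its owner with box collision disabled, and a looping timer turns cast timer progress into radius parameters on a cast circle material.
; Activation clears the cast timer, detaches the actor and sets its lifespan from the ability details.
; Interrupting an interruptible cast destroys the actor and starts the cooldown in the ability handler.
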(event `self.ReceiveBeginPlay`
  (`KismetSystemLibrary.K2_SetTimer` null "UpdateAbility" 0.01 true)
  (`PrimitiveComponent.SetCollisionEnabled` (`self.Box`) "NoCollision")
  (`self.K2_AttachToActor` (`self.AbilityOwner`) "None" "SnapToTarget" "SnapToTarget" "SnapToTarget"))

(event `UpdateAbility`
  (bind _casttimer (`self.CastTimer`))
  (bind _castcirclematerial (`self.CastCircleMaterial`))
  (bind _castprogress (`self.CastProgress`))
  (bind _returnvalue (`KismetSystemLibrary.K2_GetTimerElapsedTimeHandle` _casttimer))
  ;[1 1 1] Update Cast Time progress (for all abilities)
  (if (`KismetSystemLibrary.K2_IsValidTimerHandle` (`self.CastTimer`))
    (set `self.CastProgress` (`KismetMathLibrary.NormalizeToRange` _returnvalue 0.0 (+ _returnvalue (`KismetSystemLibrary.K2_GetTimerRemainingTimeHandle` _casttimer))))
    (`MaterialInstanceDynamic.SetScalarParameterValue` _castcirclematerial "InnerBaseRadius" (`KismetMathLibrary.MapRangeClamped` _castprogress 0.0 0.95 0.0 0.5))
    (`MaterialInstanceDynamic.SetScalarParameterValue` _castcirclematerial "InnerSubtractionRadius" (`KismetMathLibrary.MapRangeClamped` _castprogress 0.85 1.0 0.0 0.6))))

(event `ActivateAbility`
  (`KismetSystemLibrary.K2_ClearAndInvalidateTimerHandle` (`self.CastTimer`))
  (`self.K2_DetachFromActor` "KeepWorld" "KeepWorld" "KeepWorld")
  (`self.SetLifeSpan` (`.LifeSpan_41_814073994EF667A76BBDB0902D721D2E` (break `/Game/AbilitySystem/AbilityDetailsStruct` (`self.AbilityDetails`)))))

(fn `Interrupt`
  (returns (Interrupted :type Boolean))
  ;[1 0.4199 0.4937] interrupt
  (if (and (`.IsInterutable_16_A1901039465D48E9CB6CECA23ADDADD9` (break `/Game/AbilitySystem/AbilityDetailsStruct` (`self.AbilityDetails`))) (`KismetSystemLibrary.K2_IsTimerActiveHandle` (`self.CastTimer`)))
    (`KismetSystemLibrary.K2_ClearAndInvalidateTimerHandle` (`self.CastTimer`))
    (`self.K2_DestroyActor`)
    ;;[1 0 0] Start cooldown in ability handler
    (`/Game/AbilitySystem/BP_AbilityHandler_ActorComponent.StartCooldown` (`self.AbilityHandlerRef`))
    (return true)
    (else
      (return false))))

(fn `UserConstructionScript`)