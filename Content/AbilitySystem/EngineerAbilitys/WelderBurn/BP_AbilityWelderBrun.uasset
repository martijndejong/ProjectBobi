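; Engineer welder-burn ability for Lars: a held beam that damages characters inside a box, closing his mask while firing.
; It starts firing on spawn or key press, with a looping timer that applies line-of-sight-checked damage each tick.
; Each hit spends ammo, updates the HUD bar and destroys the ability at zero.
; Releasing the key opens the mask and, after a short delay, starts timer-driven reloading until full or firing resumes.
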(event `/Game/AbilitySystem/BPI_AbilityParent.InteractRelease`
  (params (Key :type "Key Structure"))
  (if (== Key (`self.DefaultKey`))
    (`KismetSystemLibrary.K2_ClearAndInvalidateTimerHandle` (`self.TimerShooting`))
    (`self.SetCurrentlyShooting` false)
    (`KismetSystemLibrary.Delay` 0.5)
    (if (not (`KismetSystemLibrary.K2_IsTimerActiveHandle` (`self.TimerReload`)))
      (bind _returnvalue (`KismetSystemLibrary.K2_SetTimer` null "AutomaticReload" 0.1 true))
      (set `self.TimerReload` _returnvalue))))

(event `/Game/AbilitySystem/BPI_AbilityParent.InteractPress`
  (params (Key :type "Key Structure"))
  (bind _currentammo (`self.CurrentAmmo`))
  (bind _abilityowner (`self.AbilityOwner`))
  (if (== Key (`self.DefaultKey`))
    (if (not (`KismetSystemLibrary.K2_IsTimerActiveHandle` (`self.TimerShooting`)))
      (bind _returnvalue (`KismetSystemLibrary.K2_SetTimerDelegate` (delegate `ShootBullet`) (`.TickRate_44_026DC71E4BD359F38832A4B45B536C31` (break `/Game/AbilitySystem/AbilityDetailsStruct` (`self.AbilityDetails`))) true :!label _label))
      (set `self.TimerShooting` _returnvalue)
      (`self.SetCurrentlyShooting` true :!label _label_2)
      (bind _output_get (set `self.Overlapping Actors` (`PrimitiveComponent.GetOverlappingActors` (`self.Box`) "/Game/Bobi/BobiCharacter.BobiCharacter_C")))
      (for _array_element _output_get
        (bind _tracedactor (`self.CheckLOS` true _array_element))
        (if (not (== _tracedactor _abilityowner))
          (`GameplayStatics.ApplyDamage` _tracedactor (`.Damage_29_66822423450AE486B2C9FE8E4C4D325E` (break `/Game/AbilitySystem/AbilityDetailsStruct` (`self.AbilityDetails`))) null _abilityowner)
          (bind _result (`/Engine/EditorBlueprintResources/StandardMacros.DecrementFloat` _currentammo)
            (:`  `
              (`/Game/HUD/HUD_Overhaul/HUD_Ability.SetResourcePercent` (`/Game/AbilitySystem/BP_AbilityHandler_ActorComponent.AbilityHUDRef` (`self.AbilityHandlerRef`)) (/ _result (`self.MaxAmmo`)))
              (if (<= _currentammo 0.0)
                (`self.K2_DestroyActor`)
                (`KismetSystemLibrary.K2_ClearAndInvalidateTimerHandle` (`self.TimerShooting`))))))))))

(event `self.ReceiveBeginPlay`
  (`parent.ReceiveBeginPlay`)
  (set `self.CurrentAmmo` (`self.MaxAmmo`))
  (`self.SetCurrentlyShooting` true)
  (goto _label))

(event `ShootBullet`
  (`self.StopReload`)
  (goto _label_2))

(event `self.ActivateAbility`
  ;[1 1 1 1 12] Empty - to overwrite parent behavior
)

(fn `AutomaticReload`
  (bind _output_get (set `self.CurrentAmmo` (`KismetMathLibrary.FClamp` (+ (`self.CurrentAmmo`) 1.0) 0.0 (`self.MaxAmmo`))))
  (bind _returnvalue (/ _output_get (`self.MaxAmmo`)))
  (`/Game/HUD/HUD_Overhaul/HUD_Ability.SetResourcePercent` (`/Game/AbilitySystem/BP_AbilityHandler_ActorComponent.AbilityHUDRef` (`self.AbilityHandlerRef`)) _returnvalue)
  (if (== _returnvalue 1.0)
    (`self.StopReload`)))

(fn `SetCurrentlyShooting`
  (params (boolShooting :type Boolean))
  (if (and (not boolShooting) (`self.IsShooting`))
    (set `self.IsShooting` false)
    (`KismetSystemLibrary.K2_ClearAndInvalidateTimerHandle` (`self.TimerShooting`))
    (bind _asbobi_character_lars (cast `/Game/Characters/Lars/BobiCharacter_Lars` (`self.AbilityOwner`)))
    (`/Game/Characters/Lars/BobiCharacter_Lars.OpenMask` _asbobi_character_lars)
    (elif (and (not (`self.IsShooting`)) (`local.boolShooting`))
      (set `self.IsShooting` true)
      (`self.StopReload`)
      (bind _asbobi_character_lars_2 (cast `/Game/Characters/Lars/BobiCharacter_Lars` (`self.AbilityOwner`)))
      (`/Game/Characters/Lars/BobiCharacter_Lars.CloseMask` _asbobi_character_lars_2))))

(fn `StopReload`
  (`KismetSystemLibrary.K2_ClearAndInvalidateTimerHandle` (`self.TimerReload`)))

(fn `UserConstructionScript`
  (`parent.UserConstructionScript`))