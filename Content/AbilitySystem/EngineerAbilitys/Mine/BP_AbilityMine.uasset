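; Engineer ability actor for a thrown mine that explodes on a key press or automatically just before its lifespan ends.
; Activation launches it along the owner's forward vector with upward lift, scaled by cast progress, and starts the detonation timer.
; Manual detonation requires a brief arming delay.
; The explosion applies distance-scaled damage and knockback to line-of-sight-checked actors in its sphere, sparing the owner damage but still launching them.
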(event `self.ActivateAbility`
  (bind _projectilemovement (`self.ProjectileMovement`))
  (bind _returnvalue (`KismetMathLibrary.MapRangeClamped` (`self.CastProgress`) 0.0 1.0 0.3 1.0))
  (`parent.ActivateAbility`)
  (set `MovementComponent.Velocity` (+ (* (`self.GetActorForwardVector` (`self.AbilityOwner`)) (* (`self.Launch Speed`) _returnvalue)) (`KismetMathLibrary.MakeVector` 0.0 0.0 (* (`self.Vertical Speed`) _returnvalue))) _projectilemovement)
  (`ActorComponent.Activate` _projectilemovement false)
  (`KismetSystemLibrary.Delay` 0.01)
  (`PrimitiveComponent.SetCollisionEnabled` (`self.Box`) "QueryAndPhysics")
  (`SphereComponent.SetSphereRadius` (`self.Sphere`) (`self.ExplosionRadius`) true)
  ;[1 1 1] Auto detonate right before life span ends
  (bind _returnvalue_2 (`KismetSystemLibrary.K2_SetTimerDelegate` (delegate `AutoDetonate`) (* (`.LifeSpan_41_814073994EF667A76BBDB0902D721D2E` (break `/Game/AbilitySystem/AbilityDetailsStruct` (`self.AbilityDetails`))) 0.99)))
  (set `self.AutoDetonateTimer` _returnvalue_2))

(event `AutoDetonate`
  (bind _returnvalue (`self.K2_GetActorLocation`))
  (bind _explosionradius (`self.ExplosionRadius`))
  (`NiagaraFunctionLibrary.SpawnSystemAtLocation` "/Game/AbilitySystem/EngineerAbilitys/Mine/P_Explosion.P_Explosion" (+ _returnvalue (0.0 0.0 10.0)) :!label _label)
  (`NiagaraFunctionLibrary.SpawnSystemAtLocation` "/Game/AbilitySystem/EngineerAbilitys/Mine/P_Poof.P_Poof" _returnvalue)
  (`GameplayStatics.SpawnSoundAtLocation` "/Game/AbilitySystem/EngineerAbilitys/Mine/S_Bomb_mixkit-fuel-explosion-1705.S_Bomb_mixkit-fuel-explosion-1705" _returnvalue (struct) 1.0 (`KismetMathLibrary.FClamp` (`KismetMathLibrary.RandomFloat`) 0.8) 0.0 null null)
  (for _array_element (`PrimitiveComponent.GetOverlappingActors` (`self.Sphere`) null)
    (bind _tracedactor (`self.CheckLOS` false _array_element))
    ;[1 1 1] Copy pasted from melee
    (if (not (== _tracedactor (`self.AbilityOwner`)))
      (`/Engine/EditorBlueprintResources/StandardMacros.IsValid` _tracedactor
        (:`Is Valid`
          (bind _returnvalue_2 (`KismetMathLibrary.MapRangeClamped` (`self.GetDistanceTo` _tracedactor) (* _explosionradius 0.75) _explosionradius 1.0 0.1))
          (`GameplayStatics.ApplyDamage` _tracedactor (* _returnvalue_2 (`.Damage_29_66822423450AE486B2C9FE8E4C4D325E` (break `/Game/AbilitySystem/AbilityDetailsStruct` (`self.AbilityDetails`)))) (`Pawn.GetController` (`self.AbilityOwner`))))))
    (bind _asbobi_character (cast `/Game/Bobi/BobiCharacter` _tracedactor))
    (`/Engine/EditorBlueprintResources/StandardMacros.IsValid` _asbobi_character
      (:`Is Valid`
        (`Character.LaunchCharacter` _asbobi_character (+ (* (* (`KismetMathLibrary.GetDirectionUnitVector` (`self.K2_GetActorLocation`) (`self.K2_GetActorLocation` _tracedactor)) 1000.0) _returnvalue_2) (0.0 0.0 100.0)) false false))))
  (`self.K2_DestroyActor`))

(event `/Game/AbilitySystem/BPI_AbilityParent.InteractPress`
  (params (Key :type "Key Structure"))
  (if (== Key (`self.DefaultKey`))
    (if (>= (`KismetSystemLibrary.K2_GetTimerElapsedTimeHandle` (`self.AutoDetonateTimer`)) 0.3)
      (goto _label))))

(fn `UserConstructionScript`
  (`parent.UserConstructionScript`))