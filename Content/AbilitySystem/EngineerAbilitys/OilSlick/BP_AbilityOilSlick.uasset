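; Engineer oil slick ability that lays a trail of BP_OilSpot actors forward from its origin, along the owner's facing.
; On activation, a looping timer lerps along the range over the cast duration, spawning a spot at the interpolated point whenever a downward trace hits.
; An alternative interaction starts a one-second timer loop that spawns spots at the Instigator's location, also trace-gated.
; Each spot receives this ability and its owner.
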(event `StopSecondaryTick`
  (`KismetSystemLibrary.K2_ClearAndInvalidateTimerHandle` (`self.SecondaryTickTimer`)))

(event `Secondary tick`
  (bind _returnvalue (`self.K2_GetActorLocation` (stale `/Game/AbilitySystem/BPI_AbilityParent.InteractAlternativeEvent` instigator)))
  (bind (_outhit _returnvalue_2) (`KismetSystemLibrary.LineTraceSingle` _returnvalue (0.0 0.0 -5000.0) "TraceTypeQuery1"))
  (if _returnvalue_2
    (`|SpawnActorFromClass` "/Game/AbilitySystem/EngineerAbilitys/OilSlick/BP_OilSpot.BP_OilSpot_C" (`KismetMathLibrary.Conv_VectorToTransform` _returnvalue) "Undefined" "OverrideRootScale" null self (`self.AbilityOwner`) null null (struct) null)))

(event `/Game/AbilitySystem/BPI_AbilityParent.InteractAlternativeEvent`
  (params (instigator :type "/Game/Bobi/BobiCharacter Object Reference"))
  (bind _returnvalue (`KismetSystemLibrary.K2_SetTimerDelegate` (delegate `Secondary tick`) 0.1 true))
  (set `self.SecondaryTickTimer` _returnvalue)
  (`KismetSystemLibrary.K2_SetTimerDelegate` (delegate `StopSecondaryTick`) 1.0))

(event `StopSpittingOil`
  (`KismetSystemLibrary.K2_ClearAndInvalidateTimerHandle` (`self.PrimaryTickTimer`)))

(event `self.ActivateAbility`
  (`parent.ActivateAbility`)
  (bind _returnvalue (`KismetSystemLibrary.K2_SetTimerDelegate` (delegate `StopSpittingOil`) (`self.Cast duration`)))
  (set `self.PrimaryDurationTimer` _returnvalue)
  (bind _returnvalue_2 (`KismetSystemLibrary.K2_SetTimerDelegate` (delegate `Tick`) (`.TickRate_44_026DC71E4BD359F38832A4B45B536C31` (break `/Game/AbilitySystem/AbilityDetailsStruct` (`self.AbilityDetails`))) true))
  (set `self.PrimaryTickTimer` _returnvalue_2)
  (bind _output_get (set `self.AbilityOrigin` (`self.K2_GetActorLocation`)))
  (set `self.AbilityEnd` (+ _output_get (* (`KismetMathLibrary.Normal` (`self.GetActorForwardVector` (`self.AbilityOwner`))) (`self.Range`)))))

(event `Tick`
  (bind _returnvalue (`KismetMathLibrary.VLerp` (`self.AbilityOrigin`) (`self.AbilityEnd`) (/ (`KismetSystemLibrary.K2_GetTimerElapsedTimeHandle` (`self.PrimaryDurationTimer`)) (`self.Cast duration`))))
  (bind (_outhit _returnvalue_2) (`KismetSystemLibrary.LineTraceSingle` _returnvalue (- _returnvalue (0.0 0.0 1000.0)) "TraceTypeQuery1"))
  (if _returnvalue_2
    (`|SpawnActorFromClass` "/Game/AbilitySystem/EngineerAbilitys/OilSlick/BP_OilSpot.BP_OilSpot_C" (`KismetMathLibrary.Conv_VectorToTransform` _returnvalue) "Undefined" "OverrideRootScale" null self (`self.AbilityOwner`) null null (struct) null)))

(fn `UserConstructionScript`
  (`parent.UserConstructionScript`))