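; Ability actor for a teleport dart: it launches a projectile from the owner, who can press the ability key to teleport to it, consuming the dart.
; Cast progress scales launch velocity, damage and knockback.
; Hit BobiCharacters are launched and get the dart attached behind them, while other overlapped actors take damage and destroy it.
; A bounce disables the dart's hit box, and teleporting also passes the box's rotation to the owner.
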(event `self.ActivateAbility`
  (bind _projectilemovement (`self.ProjectileMovement`))
  (bind _returnvalue (`KismetMathLibrary.MapRangeClamped` (`self.CastProgress`) 0.0 1.0 0.3 1.0))
  ;[1 1 1] Copy pasted from mine
  (`parent.ActivateAbility`)
  (set `MovementComponent.Velocity` (+ (* (`self.GetActorForwardVector` (`self.AbilityOwner`)) (* (`self.Launch Speed`) _returnvalue)) (`KismetMathLibrary.MakeVector` 0.0 0.0 (* (`self.Vertical Speed`) _returnvalue))) _projectilemovement)
  (`ActorComponent.Activate` _projectilemovement false)
  (`KismetSystemLibrary.Delay` 0.01)
  (`PrimitiveComponent.SetCollisionEnabled` (`self.Box`) "QueryAndPhysics"))

(event `/Game/AbilitySystem/BPI_AbilityParent.InteractPress`
  (params (Key :type "Key Structure"))
  (bind _abilityowner (`self.AbilityOwner`))
  (bind _box (`self.Box`))
  (if (== Key (`self.DefaultKey`))
    (`self.K2_SetActorLocation` _abilityowner (`SceneComponent.K2_GetComponentLocation` _box) false true)
    (message `/Game/Bobi/BPI_ControllerToCharacter.SetRotation` _abilityowner (`SceneComponent.K2_GetComponentRotation` _box))
    (`self.K2_DestroyActor`)))

(event `self.Box.OnComponentBeginOverlap`
  (params (OverlappedComponent :type "PrimitiveComponent Object Reference") (OtherActor :type "Actor Object Reference") (OtherComp :type "PrimitiveComponent Object Reference") (OtherBodyIndex :type Integer) (bFromSweep :type Boolean) (SweepResult :type "HitResult Structure (by ref)"))
  (bind _returnvalue (`KismetMathLibrary.MapRangeClamped` (`self.CastProgress`) 0.0 1.0 0.1 1.0))
  ;[1 1 1] Copy pasted from arrow
  (if (not (== OtherActor (`self.AbilityOwner`)))
    (`/Engine/EditorBlueprintResources/StandardMacros.IsValid` OtherActor
      (:`Is Valid`
        (`GameplayStatics.ApplyDamage` OtherActor (* _returnvalue (`.Damage_29_66822423450AE486B2C9FE8E4C4D325E` (break `/Game/AbilitySystem/AbilityDetailsStruct` (`self.AbilityDetails`)))))
        (bind _asbobi_character (cast `/Game/Bobi/BobiCharacter` OtherActor)
          (:`then`
            (`/Engine/EditorBlueprintResources/StandardMacros.IsValid` _asbobi_character
              (:`Is Valid`
                (`self.StickToEnemy` _asbobi_character)
                (`Character.LaunchCharacter` _asbobi_character (+ (* (* (`KismetMathLibrary.Normal` (`self.GetVelocity`)) 500.0) _returnvalue) (0.0 0.0 300.0)) false false))))
          (:`CastFailed`
            (`self.K2_DestroyActor`)))))))

(event `self.ProjectileMovement.OnProjectileBounce`
  (params (ImpactResult :type "HitResult Structure (by ref)") (ImpactVelocity :type "Vector Structure (by ref)"))
  (`PrimitiveComponent.SetCollisionEnabled` (`self.Box`) "NoCollision"))

(fn `StickToEnemy`
  (params (BobiCharacter :type "/Game/Bobi/BobiCharacter Object Reference"))
  (`ActorComponent.Deactivate` (`self.ProjectileMovement`))
  (`PrimitiveComponent.SetCollisionEnabled` (`self.Box`) "NoCollision")
  (`PrimitiveComponent.SetCollisionEnabled` (`self.StaticMesh`) "NoCollision")
  (`self.K2_AttachToActor` (`local.BobiCharacter`) "None" "SnapToTarget" "SnapToTarget" "SnapToTarget" false)
  (`SceneComponent.K2_SetRelativeLocation` (`self.Box`) (-120.0 0.0 0.0) false true))

(fn `UserConstructionScript`
  (`parent.UserConstructionScript`))