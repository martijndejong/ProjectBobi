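; Holy Ground area ability that repeatedly applies damage to its own owner while they stand inside its area.
; Activation calls the parent, shows the decal, enables collision on AreaOfEffect and starts a looping timer at the ability's tick rate.
; Each tick scans the overlapping actors and applies the configured Damage only to the one matching AbilityOwner, ignoring all others.
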(event `self.ActivateAbility`
  (bind (_abilitydetails_name _abilitydetails_icon _abilitydetails_cooldown _abilitydetails_damage _abilitydetails_tickrate) (break `/Game/AbilitySystem/AbilityDetailsStruct` (`self.AbilityDetails`)))
  (`parent.ActivateAbility`)
  (`SceneComponent.SetVisibility` (`self.Decal`) true false)
  (`PrimitiveComponent.SetCollisionEnabled` (`self.AreaOfEffect`) "QueryAndPhysics")
  (`KismetSystemLibrary.K2_SetTimerDelegate` (delegate `Tick`) _abilitydetails_tickrate true))

(event `Tick`
  (bind (_abilitydetails_name _abilitydetails_icon _abilitydetails_cooldown _abilitydetails_damage _abilitydetails_tickrate) (break `/Game/AbilitySystem/AbilityDetailsStruct` (`self.AbilityDetails`)))
  (for _array_element (`PrimitiveComponent.GetOverlappingActors` (`self.AreaOfEffect`) null)
    (if (== _array_element (`self.AbilityOwner`))
      (`GameplayStatics.ApplyDamage` _array_element _abilitydetails_damage))))

(fn `UserConstructionScript`
  (`parent.UserConstructionScript`))