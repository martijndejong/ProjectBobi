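; Melee ability actor that dashes its owner and performs a sword slash, with strength scaled by cast progress.
; Updates scale the arrow and slash effect; activation attaches the actor to the owner, enables the hit box and plays the effect and sound.
; Cast progress also scales dash, damage, volume and pitch.
; Overlaps run a line-of-sight check and damage the traced actor, using an ignore list to prevent repeat hits.
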(event `self.ActivateAbility`
  (bind _returnvalue (`KismetMathLibrary.MapRangeClamped` (`self.CastProgress`) 0.0 1.0 0.4 1.0))
  (bind _returnvalue_2 (`KismetMathLibrary.MapRangeClamped` (`self.CastProgress`) 0.0 1.0 0.4 1.0))
  (`parent.ActivateAbility`)
  (message `/Game/Bobi/BPI_BobiCharacter.Dash` (`self.AbilityOwner`) (* _returnvalue_2 (`self.Duration`)) (* (`self.Distance`) _returnvalue_2) false false true)
  (`PrimitiveComponent.SetCollisionEnabled` (`self.Box`) "QueryAndPhysics")
  (`ActorComponent.Activate` (`self.P_SwordSlash`) false)
  (`self.K2_AttachToActor` (`self.AbilityOwner`) "None" "SnapToTarget" "SnapToTarget" "SnapToTarget")
  (`GameplayStatics.PlaySoundAtLocation` "/Game/AbilitySystem/Melee/S_Sword_mixkit-metal-hit-woosh-1485.S_Sword_mixkit-metal-hit-woosh-1485" (`self.K2_GetActorLocation`) (struct) _returnvalue (`KismetMathLibrary.MapRangeClamped` _returnvalue 0.5 1.0 1.0 0.7) 0.0 null null null))

(event `self.UpdateAbility`
  (bind _returnvalue (`KismetMathLibrary.Conv_DoubleToVector` (`KismetMathLibrary.MapRangeClamped` (`self.CastProgress`) 0.0 1.0 0.6 1.0)))
  (`parent.UpdateAbility`)
  (`SceneComponent.SetWorldScale3D` (`self.Arrow`) _returnvalue)
  (`SceneComponent.SetWorldScale3D` (`self.P_SwordSlash`) _returnvalue))

(event `self.Box.OnComponentBeginOverlap`
  (params (OverlappedComponent :type "PrimitiveComponent Object Reference") (OtherActor :type "Actor Object Reference") (OtherComp :type "PrimitiveComponent Object Reference") (OtherBodyIndex :type Integer) (bFromSweep :type Boolean) (SweepResult :type "HitResult Structure (by ref)"))
  (bind (_abilitydetails_name _abilitydetails_icon _abilitydetails_cooldown _abilitydetails_damage) (break `/Game/AbilitySystem/AbilityDetailsStruct` (`self.AbilityDetails`)))
  (bind _tracedactor (`self.CheckLOS` true OtherActor))
  (if (and (not (== _tracedactor (`self.AbilityOwner`))) (not (`KismetArrayLibrary.Array_Contains` (`self.ActorIgnoreList`) _tracedactor)))
    (`GameplayStatics.ApplyDamage` _tracedactor (* (`KismetMathLibrary.MapRangeClamped` (`self.CastProgress`) 0.0 1.0 0.4 1.0) _abilitydetails_damage) (`Pawn.GetController` (`self.AbilityOwner`)))
    (`self.AddActorToIgnoreList` _tracedactor)))

(fn `UserConstructionScript`
  (`parent.UserConstructionScript`))