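; Shield ability actor that wears down under damage and destroys itself when activated.
; Each hit shortens the ability handler's remaining cast timer in proportion to damage by replacing it with a new timer.
; When that timer expires or damage exhausts it, the shield tells the handler to activate the ability.
; Non-exhausting hits also play a timeline driving ring radii on the sphere's dynamic material for an impact wave.
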(event `self.ReceiveBeginPlay`
  (`parent.ReceiveBeginPlay`)
  (bind _returnvalue (`PrimitiveComponent.CreateDynamicMaterialInstance` (`self.ShieldSphere`) 0 null "None"))
  (set `self.ShieldMaterial` _returnvalue)
  (`TimelineComponent.SetPlayRate` (`self.WaveTimeLine`) (/ 1.0 (`self.WaveLength`))))

(event `self.ActivateAbility`
  ;[1 1 1] Activate = destroy actor
  (`parent.ActivateAbility`)
  (`self.K2_DestroyActor`))

(event `self.ReceiveAnyDamage`
  (params (Damage :type "Float (single-precision)") (DamageType :type "DamageType Object Reference") (InstigatedBy :type "Controller Object Reference") (DamageCauser :type "Actor Object Reference"))
  (bind _shieldmaterial (`self.ShieldMaterial`))
  (bind _abilityhandlerref (`self.AbilityHandlerRef`))
  (bind _returnvalue (- (`KismetSystemLibrary.K2_GetTimerRemainingTimeHandle` (`/Game/AbilitySystem/BP_AbilityHandler_ActorComponent.CastTimer` (`self.AbilityHandlerRef`))) (/ Damage 50.0)))
  ;[1 1 1] Increase cast time when taking damage
  (if (> _returnvalue 0.0)
    (bind _returnvalue_2 (`KismetSystemLibrary.K2_SetTimerDelegate` (delegate `TellHandlerToActivate`) _returnvalue))
    (`KismetSystemLibrary.K2_ClearAndInvalidateTimerHandle` (`/Game/AbilitySystem/BP_AbilityHandler_ActorComponent.CastTimer` _abilityhandlerref))
    (set `/Game/AbilitySystem/BP_AbilityHandler_ActorComponent.CastTimer` _returnvalue_2 _abilityhandlerref)
    ;[1 1 1] Animate impact on shield (purely visual)
    (bind (_direction _inner _outer) (`Timeline|WaveTimeLine` :!via `PlayFromStart`)
      (:`Update`
        (`/Engine/EditorBlueprintResources/StandardMacros.IsValid` _shieldmaterial
          (:`Is Valid`
            (`MaterialInstanceDynamic.SetScalarParameterValue` _shieldmaterial "innerRadius" _inner)
            (`MaterialInstanceDynamic.SetScalarParameterValue` _shieldmaterial "outerRadius" _outer)))))
    (else
      (`/Game/AbilitySystem/BP_AbilityHandler_ActorComponent.ActivateAbility` (`self.AbilityHandlerRef`) :!label _label))))

(event `TellHandlerToActivate`
  ;[1 1 1] Increase cast time when taking damage
  (goto _label))

(fn `UserConstructionScript`
  (`parent.UserConstructionScript`))