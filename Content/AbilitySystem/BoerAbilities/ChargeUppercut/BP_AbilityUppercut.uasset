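; Uppercut ability, filed under Boer's ChargeUppercut set, that launches its owner upward and hits actors caught in its box.
; Activation enables the box and, only if not already initiated, plays the montage's Uppercut section, cancels dash and launches the owner.
; Box overlaps passing line-of-sight damage and knock back each traced actor, using an ignore list against repeat hits.
; UppercutFactor scales damage, launch and vertical knockback.
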(event `self.ReceiveBeginPlay`
  (`parent.ReceiveBeginPlay`))

(event `self.ActivateAbility`
  (`parent.ActivateAbility`)
  (`PrimitiveComponent.SetCollisionEnabled` (`self.Box`) "QueryAndPhysics")
  (`self.StartUppercut`))

(event `self.Box.OnComponentBeginOverlap`
  (params (OverlappedComponent :type "PrimitiveComponent Object Reference") (OtherActor :type "Actor Object Reference") (OtherComp :type "PrimitiveComponent Object Reference") (OtherBodyIndex :type Integer) (bFromSweep :type Boolean) (SweepResult :type "HitResult Structure (by ref)"))
  (bind (_tracedactor _returnvalue) (`self.CheckLOS` true OtherActor))
  (if _returnvalue
    (if (and (not (== _tracedactor (`self.AbilityOwner`))) (not (`KismetArrayLibrary.Array_Contains` (`self.ActorIgnoreList`) _tracedactor)))
      (`GameplayStatics.ApplyDamage` _tracedactor (* (`.Damage_29_66822423450AE486B2C9FE8E4C4D325E` (break `/Game/AbilitySystem/AbilityDetailsStruct` (`self.AbilityDetails`))) (`self.UppercutFactor`)) (`Pawn.GetController` (`self.AbilityOwner`)))
      (`self.AddActorToIgnoreList` _tracedactor)
      (`self.Knockback` _tracedactor 1.0 -200.0 (* (`self.UppercutStrength`) (`self.UppercutFactor`))))))

(fn `StartUppercut`
  (bind _abilityowner (`self.AbilityOwner`))
  (if (not (`self.InitiatedUppercut`))
    (`Character.PlayAnimMontage` (`self.AbilityOwner`) "/Game/AbilitySystem/BoerAbilities/ChargeUppercut/Animation_ChargeUppercut_Montage.Animation_ChargeUppercut_Montage" 1.0 "Uppercut")
    (message `/Game/Bobi/BPI_ControllerToCharacter.CancelDash` _abilityowner)
    (`Character.LaunchCharacter` _abilityowner (`KismetMathLibrary.MakeVector` 0.0 0.0 (* (`self.UppercutStrength`) (`self.UppercutFactor`))) true true)
    (set `self.InitiatedUppercut` true)))

(fn `UserConstructionScript`
  (`parent.UserConstructionScript`))