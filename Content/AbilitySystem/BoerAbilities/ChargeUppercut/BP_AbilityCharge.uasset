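; Charge uppercut ability actor that dashes its owner forward and strikes actors caught in its hit box.
; Cast progress scales dash distance, duration and an uppercut factor for damage and knockback.
; A line-of-sight-checked overlap damages and launches the target, cancels its dash, and ends the charge.
; EndCharge stops the dash and plays the montage's end section once, adding a short extra dash when the timer expires without a hit.
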(event `self.ReceiveBeginPlay`
  (`parent.ReceiveBeginPlay`))

(event `EndChargeEvent`
  (`self.EndCharge` true))

(event `self.ActivateAbility`
  (bind _returnvalue (`KismetMathLibrary.MapRangeClamped` (`self.CastProgress`) 0.0 1.0 0.1 1.0))
  (bind _returnvalue_2 (* (`self.Duration`) _returnvalue))
  (`parent.ActivateAbility`)
  (`PrimitiveComponent.SetCollisionEnabled` (`self.Box`) "QueryAndPhysics")
  (message `/Game/Bobi/BPI_ControllerToCharacter.Dash` (`self.AbilityOwner`) _returnvalue_2 (* _returnvalue (`self.Distance`)) false false true)
  (`KismetSystemLibrary.K2_SetTimerDelegate` (delegate `EndChargeEvent`) _returnvalue_2)
  (`self.SetLifeSpan` (+ _returnvalue_2 0.01))
  (set `self.UppercutFactor` (`KismetMathLibrary.MapRangeClamped` (`self.CastProgress`) 0.0 1.0 0.6 1.0)))

(event `self.Box.OnComponentBeginOverlap`
  (params (OverlappedComponent :type "PrimitiveComponent Object Reference") (OtherActor :type "Actor Object Reference") (OtherComp :type "PrimitiveComponent Object Reference") (OtherBodyIndex :type Integer) (bFromSweep :type Boolean) (SweepResult :type "HitResult Structure (by ref)"))
  (bind (_tracedactor _returnvalue) (`self.CheckLOS` true OtherActor))
  (if _returnvalue
    (if (and (not (== _tracedactor (`self.AbilityOwner`))) (not (`KismetArrayLibrary.Array_Contains` (`self.ActorIgnoreList`) _tracedactor)))
      (`GameplayStatics.ApplyDamage` _tracedactor (* (`.Damage_29_66822423450AE486B2C9FE8E4C4D325E` (break `/Game/AbilitySystem/AbilityDetailsStruct` (`self.AbilityDetails`))) (`self.UppercutFactor`)) (`Pawn.GetController` (`self.AbilityOwner`)))
      (`self.AddActorToIgnoreList` _tracedactor)
      (message `/Game/Bobi/BPI_ControllerToCharacter.CancelDash` _tracedactor)
      (`self.Knockback` _tracedactor 1.0 (* (`self.ChargeStrength`) (`self.UppercutFactor`)) 150.0)
      (`self.EndCharge` false))))

(fn `EndCharge`
  (params (ExtraEndDash :type Boolean :default true))
  (locals (ExtraDashTime :type "Float (double-precision)" :default 0.25))
  (bind _abilityowner (`self.AbilityOwner`))
  (bind _extradashtime (`local.ExtraDashTime`))
  (if (not (`self.InitiatedUppercut`))
    (`Character.PlayAnimMontage` (`self.AbilityOwner`) "/Game/AbilitySystem/BoerAbilities/ChargeUppercut/Animation_Charge_Montage.Animation_Charge_Montage" 1.0 "EndCharge")
    (message `/Game/Bobi/BPI_ControllerToCharacter.CancelDash` _abilityowner)
    (set `self.InitiatedUppercut` true)
    (if (`local.ExtraEndDash`)
      (`self.SetLifeSpan` _extradashtime)
      (message `/Game/Bobi/BPI_ControllerToCharacter.Dash` _abilityowner _extradashtime 175.0 false false false))))

(fn `UserConstructionScript`
  (`parent.UserConstructionScript`))