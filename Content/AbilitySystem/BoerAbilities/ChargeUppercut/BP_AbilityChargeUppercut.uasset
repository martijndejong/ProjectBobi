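; Charged dash-uppercut ability for the Boer character that rushes the owner forward, then launches them upward.
; Cast progress scales dash distance, duration and lifespan, plus an uppercut factor for damage and launch strength.
; The hitbox damages and knocks line-of-sight targets upward once each, triggering the uppercut early.
; Otherwise a timer fires it at dash end; a guard keeps it to one launch.
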(event `self.ReceiveBeginPlay`
  (`parent.ReceiveBeginPlay`))

(event `self.ActivateAbility`
  (bind _returnvalue (`KismetMathLibrary.MapRangeClamped` (`self.CastProgress`) 0.0 1.0 0.1 1.0))
  (bind _returnvalue_2 (* (`self.Duration`) _returnvalue))
  (`parent.ActivateAbility`)
  (`PrimitiveComponent.SetCollisionEnabled` (`self.Box`) "QueryAndPhysics")
  (message `/Game/Bobi/BPI_ControllerToCharacter.Dash` (`self.AbilityOwner`) _returnvalue_2 (* _returnvalue (`self.Distance`)) false false true)
  (`KismetSystemLibrary.K2_SetTimer` null "StartUppercut" _returnvalue_2)
  (`self.SetLifeSpan` _returnvalue_2)
  (set `self.UppercutFactor` (`KismetMathLibrary.MapRangeClamped` (`self.CastProgress`) 0.0 1.0 0.6 1.0)))

(event `self.Box.OnComponentBeginOverlap`
  (params (OverlappedComponent :type "PrimitiveComponent Object Reference") (OtherActor :type "Actor Object Reference") (OtherComp :type "PrimitiveComponent Object Reference") (OtherBodyIndex :type Integer) (bFromSweep :type Boolean) (SweepResult :type "HitResult Structure (by ref)"))
  (bind (_tracedactor _returnvalue) (`self.CheckLOS` true OtherActor))
  (if _returnvalue
    (if (and (not (== _tracedactor (`self.AbilityOwner`))) (not (`KismetArrayLibrary.Array_Contains` (`self.ActorIgnoreList`) _tracedactor)))
      (`GameplayStatics.ApplyDamage` _tracedactor (* (`.Damage_29_66822423450AE486B2C9FE8E4C4D325E` (break `/Game/AbilitySystem/AbilityDetailsStruct` (`self.AbilityDetails`))) (`self.UppercutFactor`)) (`Pawn.GetController` (`self.AbilityOwner`)))
      (`self.AddActorToIgnoreList` _tracedactor)
      (`self.Knockback` _tracedactor 1.0 0.0 (* (`self.UppercutStrength`) (`self.UppercutFactor`)))
      (`self.StartUppercut`))))

(fn `StartUppercut`
  (bind _abilityowner (`self.AbilityOwner`))
  (if (not (`self.InitiatedUppercut`))
    (message `/Game/Bobi/BPI_ControllerToCharacter.CancelDash` _abilityowner)
    (`Character.LaunchCharacter` _abilityowner (`KismetMathLibrary.MakeVector` 0.0 0.0 (* (`self.UppercutStrength`) (`self.UppercutFactor`))) true true)
    (set `self.InitiatedUppercut` true)))

(fn `UserConstructionScript`
  (`parent.UserConstructionScript`))