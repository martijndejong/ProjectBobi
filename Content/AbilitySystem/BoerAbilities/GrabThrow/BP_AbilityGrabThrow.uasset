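; Grab-and-throw ability actor that snatches characters in front of its owner and launches them forward and upward.
; On spawn it dashes the owner briefly, then enables a box overlap that collects line-of-sight targets during a short grab window, disabling their Pawn collision.
; While Holding, Tick teleports captives in front of the owner.
; Activation launches them with force scaled by cast progress; collision returns after a delay or on destruction.
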(event `self.ReceiveBeginPlay`
  (bind _abilityowner (`self.AbilityOwner`))
  (bind (_returnvalue_x _returnvalue_y _returnvalue_z) (`KismetMathLibrary.BreakVector` (`self.GetVelocity` _abilityowner)))
  (`parent.ReceiveBeginPlay`)
  (message `/Game/Bobi/BPI_ControllerToCharacter.Dash` _abilityowner 0.1 40.0 false false (< _returnvalue_z 0.0))
  (`KismetSystemLibrary.Delay` 0.25)
  (`PrimitiveComponent.SetCollisionEnabled` (`self.Box`) "QueryOnly")
  (`KismetSystemLibrary.K2_SetTimerDelegate` (delegate `SetGrabbingFalse`) 0.3))

(event `SetGrabbingFalse`
  (set `self.Grabbing` false))

(event `self.ActivateAbility`
  (`parent.ActivateAbility`)
  (set `self.Holding` false)
  (for _array_element (`self.GrabbedCharacters`)
    (bind _asbobi_character (cast `/Game/Bobi/BobiCharacter` _array_element))
    (`Character.LaunchCharacter` _asbobi_character (* (* (+ (`self.GetActorForwardVector` (`self.AbilityOwner`)) (0.0 0.0 1.5)) (`self.ThrowStrength`)) (`KismetMathLibrary.MapRangeClamped` (`self.CastProgress`) 0.0 1.0 0.3 1.0)) true true)
    (`KismetSystemLibrary.Delay` 0.5)
    (`self.SetPawnCollision` _asbobi_character)))

(event `self.ReceiveDestroyed`
  (`parent.ReceiveDestroyed`)
  (for _array_element (`self.GrabbedCharacters`)
    (`self.SetPawnCollision` _array_element)))

(event `self.Box.OnComponentBeginOverlap`
  (params (OverlappedComponent :type "PrimitiveComponent Object Reference") (OtherActor :type "Actor Object Reference") (OtherComp :type "PrimitiveComponent Object Reference") (OtherBodyIndex :type Integer) (bFromSweep :type Boolean) (SweepResult :type "HitResult Structure (by ref)"))
  (if (`self.Grabbing`)
    (bind (_tracedactor _returnvalue) (`self.CheckLOS` true OtherActor))
    (if _returnvalue
      (if (not (`KismetArrayLibrary.Array_Contains` (`self.ActorIgnoreList`) _tracedactor))
        (`self.AddActorToIgnoreList` _tracedactor)
        (`self.SetPawnCollision` _tracedactor false)
        (`KismetArrayLibrary.Array_AddUnique` (`self.GrabbedCharacters`) _tracedactor)))))

(event `self.ReceiveTick`
  (params (DeltaSeconds :type "Float (single-precision)"))
  (bind _abilityowner (`self.AbilityOwner`))
  (bind (_returnvalue_x _returnvalue_y _returnvalue_z) (`KismetMathLibrary.BreakVector` (`self.K2_GetActorLocation` _abilityowner)))
  (if (`self.Holding`)
    (for _array_element (`self.GrabbedCharacters`)
      (`self.K2_SetActorLocation` _array_element (+ (`KismetMathLibrary.MakeVector` _returnvalue_x _returnvalue_y (+ _returnvalue_z (* (`CapsuleComponent.GetScaledCapsuleHalfHeight` (`Character.CapsuleComponent` _abilityowner)) 0.5))) (* (`self.GetActorForwardVector` (`self.AbilityOwner`)) 75.0)) false true))))

(fn `SetPawnCollision`
  (params (Object :type "Object Object Reference") (Enable :type Boolean :default true))
  (bind _capsulecomponent (`Character.CapsuleComponent` (cast `/Game/Bobi/BobiCharacter` Object :!pure true)))
  (if Enable
    (`PrimitiveComponent.SetCollisionResponseToChannel` _capsulecomponent "ECC_Pawn" "ECR_Block")
    (else
      (`PrimitiveComponent.SetCollisionResponseToChannel` _capsulecomponent "ECC_Pawn" "ECR_Ignore"))))

(fn `UserConstructionScript`
  (`parent.UserConstructionScript`))