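; Punch ability Blueprint for the Boer ability set: a short forward lunge with a melee hit.
; On activation it sends a brief dash message to the owner and enables the hit box for overlap queries.
; Overlaps pass a line-of-sight check, then the traced actor takes damage and knockback and joins an ignore list to prevent repeat hits.
; A stun effect call exists but is disconnected.
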(event `self.ActivateAbility`
  (`parent.ActivateAbility`)
  (message `/Game/Bobi/BPI_BobiCharacter.Dash` (`self.AbilityOwner`) 0.1 60.0 false false false)
  (`PrimitiveComponent.SetCollisionEnabled` (`self.Box`) "QueryOnly"))

(event `self.Box.OnComponentBeginOverlap`
  (params (OverlappedComponent :type "PrimitiveComponent Object Reference") (OtherActor :type "Actor Object Reference") (OtherComp :type "PrimitiveComponent Object Reference") (OtherBodyIndex :type Integer) (bFromSweep :type Boolean) (SweepResult :type "HitResult Structure (by ref)"))
  (bind _tracedactor (`self.CheckLOS` true OtherActor))
  (if (and (not (== _tracedactor (`self.AbilityOwner`))) (not (`KismetArrayLibrary.Array_Contains` (`self.ActorIgnoreList`) _tracedactor)))
    (`GameplayStatics.ApplyDamage` _tracedactor (`.Damage_29_66822423450AE486B2C9FE8E4C4D325E` (break `/Game/AbilitySystem/AbilityDetailsStruct` (`self.AbilityDetails`))) (`Pawn.GetController` (`self.AbilityOwner`)))
    (`self.Knockback` _tracedactor 1.0 200.0 50.0)
    (`self.AddActorToIgnoreList` _tracedactor)))

(fn `UserConstructionScript`
  (`parent.UserConstructionScript`))