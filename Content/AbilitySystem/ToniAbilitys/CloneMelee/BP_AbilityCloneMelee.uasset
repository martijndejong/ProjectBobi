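; Sword slash dash ability that works for both the ability owner and a BP_AbilityStationaryClone.
; Activation sends a dash message to the ability owner, plays effects and briefly enables a damage box.
; When clone-owned, a timeline lerps the clone forward without sweep, and hits skip clone and ability owner.
; Otherwise, BeginPlay sends interact presses to overlapping clone handlers, and damage goes through a line-of-sight check.
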(event `self.ReceiveBeginPlay`
  (`self.K2_AttachToActor` (`self.GetOwner`) "None" "SnapToTarget" "SnapToTarget" "SnapToTarget" false)
  (if (!= (`GameplayStatics.GetObjectClass` (`self.GetOwner`)) "/Game/AbilitySystem/ToniAbilitys/CloneStationary/BP_AbilityStationaryClone.BP_AbilityStationaryClone_C")
    (message `/Game/AbilitySystem/BPI_AbilityParent.InteractPress` (`self.GetOverlappingActors` (`self.AbilityOwner`) "/Game/AbilitySystem/ToniAbilitys/CloneStationary/BP_AbilityCloneHandler.BP_AbilityCloneHandler_C") (`self.DefaultKey`))))

(event `self.ActivateAbility`
  (bind _distance (`self.Distance`))
  (bind _duration (`self.Duration`))
  (`self.CloneDash` _distance _duration)
  (message `/Game/Bobi/BPI_BobiCharacter.Dash` (`self.AbilityOwner`) _duration _distance false false true)
  (`PrimitiveComponent.SetCollisionEnabled` (`self.Box`) "QueryAndPhysics")
  (`ActorComponent.Activate` (`self.P_SwordSlash`) false)
  (`self.K2_AttachToActor` (`self.GetOwner`) "None" "SnapToTarget" "SnapToTarget" "SnapToTarget")
  (`GameplayStatics.PlaySoundAtLocation` "/Game/AbilitySystem/Melee/S_Sword_mixkit-metal-hit-woosh-1485.S_Sword_mixkit-metal-hit-woosh-1485" (`self.K2_GetActorLocation`) (struct) 1.0 1.0 0.0 null null null)
  (`KismetSystemLibrary.Delay` 0.1)
  (`PrimitiveComponent.SetCollisionEnabled` (`self.Box`) "NoCollision"))

(event `self.Box.OnComponentBeginOverlap`
  (params (OverlappedComponent :type "PrimitiveComponent Object Reference") (OtherActor :type "Actor Object Reference") (OtherComp :type "PrimitiveComponent Object Reference") (OtherBodyIndex :type Integer) (bFromSweep :type Boolean) (SweepResult :type "HitResult Structure (by ref)"))
  (bind (_abilitydetails_name _abilitydetails_icon _abilitydetails_cooldown _abilitydetails_damage) (break `/Game/AbilitySystem/AbilityDetailsStruct` (`self.AbilityDetails`)))
  (if (== (`GameplayStatics.GetObjectClass` (`self.GetOwner`)) "/Game/AbilitySystem/ToniAbilitys/CloneStationary/BP_AbilityStationaryClone.BP_AbilityStationaryClone_C")
    (if (and (!= OtherActor (`self.AbilityOwner`)) (!= OtherActor (`self.GetOwner`)))
      (`self.ApplyDamageOnce` OtherActor _abilitydetails_damage))
    (else
      (bind _tracedactor (`self.CheckLOS` true OtherActor))
      (`self.ApplyDamageOnce` _tracedactor _abilitydetails_damage))))

(event `CloneDash`
  (params (Distance :type "Float (double-precision)") (Duration :type "Float (double-precision)"))
  (bind _returnvalue (`self.GetOwner`))
  (bind _returnvalue_2 (`self.GetOwner`))
  ;[1 1 1] Copied from bobi character parent
  (if (== (`GameplayStatics.GetObjectClass` (`self.GetOwner`)) "/Game/AbilitySystem/ToniAbilitys/CloneStationary/BP_AbilityStationaryClone.BP_AbilityStationaryClone_C")
    (bind _output_get (set `self.DashStartPoint` (`self.K2_GetActorLocation` _returnvalue_2)))
    (set `self.DashEndPoint` (+ _output_get (* (`self.GetActorForwardVector` _returnvalue_2) Distance)))
    (`TimelineComponent.SetPlayRate` (`self.DashTimeLine`) (/ 1.0 Duration))
    (bind (_direction _progressed) (`Timeline|DashTimeLine` :!via `PlayFromStart`)
      (:`Update`
        (`/Engine/EditorBlueprintResources/StandardMacros.IsValid` _returnvalue
          (:`Is Valid`
            (`self.K2_SetActorLocation` _returnvalue (`KismetMathLibrary.VLerp` (`self.DashStartPoint`) (`self.DashEndPoint`) _progressed) false false)))))))

(fn `UserConstructionScript`
  (`parent.UserConstructionScript`))