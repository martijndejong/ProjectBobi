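; Ability projectile that throws a dart its owner can teleport to by pressing the default key.
; Launch velocity scales with cast progress; overlaps deal damage, and hit characters are knocked back with the dart attached.
; Hitting or stopping shows a player-colored floor icon and starts the lifespan.
; Teleporting notifies the owner's clone handler, moves and rotates the owner to the dart, destroys it and spawns a poof.
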(event `self.ActivateAbility`
  (bind _projectilemovement (`self.ProjectileMovement`))
  (bind _returnvalue (`KismetMathLibrary.MapRangeClamped` (`self.CastProgress`) 0.0 1.0 0.3 1.0))
  ;[1 1 1] Copy pasted from mine
  (`parent.ActivateAbility`)
  (set `MovementComponent.Velocity` (+ (* (`self.GetActorForwardVector` (`self.AbilityOwner`)) (* (`self.Launch Speed`) _returnvalue)) (`KismetMathLibrary.MakeVector` 0.0 0.0 (* (`self.Vertical Speed`) _returnvalue))) _projectilemovement)
  (`ActorComponent.Activate` _projectilemovement false)
  (`KismetSystemLibrary.Delay` 0.01)
  (`PrimitiveComponent.SetCollisionEnabled` (`self.Box`) "QueryAndPhysics")
  (bind _rectlight (`self.RectLight`)
    (:`then`
      (`LightComponent.SetLightColor` _rectlight (`/Game/Bobi/BobiCharacter.PlayerColor` (`self.AbilityOwner`)) true))
    (:`else`)))

(event `/Game/AbilitySystem/BPI_AbilityParent.InteractPress`
  (params (Key :type "Key Structure"))
  (bind _abilityowner (`self.AbilityOwner`))
  (bind _abilityowner_2 (`self.AbilityOwner`))
  (bind _box (`self.Box`))
  (if (== Key (`self.DefaultKey`))
    (message `/Game/AbilitySystem/BPI_AbilityParent.InteractAlternativeEvent` (`/Game/Characters/Toni/BobiCharacter_Martijn.CloneHandlerRef` (cast `/Game/Characters/Toni/BobiCharacter_Martijn` _abilityowner :!pure true)) _abilityowner)
    (`self.K2_SetActorLocation` _abilityowner_2 (+ (`SceneComponent.K2_GetComponentLocation` _box) (0.0 0.0 150.0)) false true)
    (message `/Game/Bobi/BPI_BobiCharacter.SetRotation` _abilityowner_2 (`SceneComponent.K2_GetComponentRotation` _box))
    (`self.K2_DestroyActor`)
    (`self.SpawnNiagaraPoof`)))

(event `self.Box.OnComponentBeginOverlap`
  (params (OverlappedComponent :type "PrimitiveComponent Object Reference") (OtherActor :type "Actor Object Reference") (OtherComp :type "PrimitiveComponent Object Reference") (OtherBodyIndex :type Integer) (bFromSweep :type Boolean) (SweepResult :type "HitResult Structure (by ref)"))
  ;[1 1 1] Copy pasted from arrow
  (if (not (== OtherActor (`self.AbilityOwner`)))
    (`/Engine/EditorBlueprintResources/StandardMacros.IsValid` OtherActor
      (:`Is Valid`
        (`ActorComponent.Deactivate` (`self.RotatingMovement`))
        (`GameplayStatics.ApplyDamage` OtherActor (`.Damage_29_66822423450AE486B2C9FE8E4C4D325E` (break `/Game/AbilitySystem/AbilityDetailsStruct` (`self.AbilityDetails`))) (`Pawn.GetController` (`self.AbilityOwner`)))
        (bind _asbobi_character (cast `/Game/Bobi/BobiCharacter` OtherActor)
          (:`then`
            (`/Engine/EditorBlueprintResources/StandardMacros.IsValid` _asbobi_character
              (:`Is Valid`
                (`self.StickToEnemy` _asbobi_character)
                (`Character.LaunchCharacter` _asbobi_character (+ (* (* (`KismetMathLibrary.Normal` (`self.GetVelocity`)) 500.0) (`KismetMathLibrary.MapRangeClamped` (`self.CastProgress`) 0.0 1.0 0.1 1.0)) (0.0 0.0 300.0)) false false))))
          (:`CastFailed`
            (`self.ActivateNiagaraAndSetLifeSpan`)))))))

(event `self.ProjectileMovement.OnProjectileBounce`
  (params (ImpactResult :type "HitResult Structure (by ref)") (ImpactVelocity :type "Vector Structure (by ref)"))
  (`PrimitiveComponent.SetCollisionEnabled` (`self.Box`) "NoCollision")
  (`ActorComponent.Deactivate` (`self.RotatingMovement`)))

(event `self.ProjectileMovement.OnComponentActivated`
  (params (Component :type "ActorComponent Object Reference") (bReset :type Boolean))
  (`ActorComponent.Activate` (`self.RotatingMovement`) false))

(event `self.ProjectileMovement.OnProjectileStop`
  (params (ImpactResult :type "HitResult Structure (by ref)"))
  (`self.ActivateNiagaraAndSetLifeSpan`))

(fn `ActivateNiagaraAndSetLifeSpan`
  (bind _niagaraflooricon (`self.NiagaraFloorIcon`))
  (bind (_name _icon _cooldown _damage _tickrate _casttime _lifespan) (break `/Game/AbilitySystem/AbilityDetailsStruct` (`self.AbilityDetails`)))
  (`FXSystemComponent.SetColorParameter` _niagaraflooricon "PlayerColor" (`/Game/Bobi/BobiCharacter.PlayerColor` (`self.AbilityOwner`)))
  (`FXSystemComponent.SetFloatParameter` _niagaraflooricon "LifeSpan" _lifespan)
  (`ActorComponent.Activate` _niagaraflooricon false)
  (`self.SetLifeSpan` _lifespan))

(fn `SpawnNiagaraPoof`
  (`NiagaraFunctionLibrary.SpawnSystemAtLocation` "/Game/AbilitySystem/ToniAbilitys/CloneStationary/P_ClonePoof.P_ClonePoof" (`self.K2_GetActorLocation` (`self.AbilityOwner`))))

(fn `StickToEnemy`
  (params (BobiCharacter :type "/Game/Bobi/BobiCharacter Object Reference"))
  (`ActorComponent.Deactivate` (`self.ProjectileMovement`))
  (`PrimitiveComponent.SetCollisionEnabled` (`self.Box`) "NoCollision")
  (`PrimitiveComponent.SetCollisionEnabled` (`self.StaticMesh`) "NoCollision")
  (`self.K2_AttachToActor` (`local.BobiCharacter`) "None" "SnapToTarget" "SnapToTarget" "SnapToTarget" false)
  (`SceneComponent.K2_SetRelativeLocation` (`self.Box`) (-120.0 0.0 -100.0) false true)
  (`self.ActivateNiagaraAndSetLifeSpan`))

(fn `UserConstructionScript`
  (`parent.UserConstructionScript`))