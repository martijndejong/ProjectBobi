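; BP_AbilityCloneHandler manages the stationary clone ability, attaching itself to the ability owner on begin play.
; The owner's alternative interact spawns a clone at the handler's transform and adds it to CloneArray.
; Key presses matching the melee or dash key lists make every valid clone melee or dash-melee.
; TraceNearestEnemy sphere-traces toward a forward-vector endpoint, ignoring owner and clones, and returns the hit actor.
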(event `self.ReceiveBeginPlay`
  (`self.K2_AttachToActor` (`self.AbilityOwner`) "None" "SnapToTarget" "SnapToTarget" "SnapToTarget" false)
  (`PrimitiveComponent.SetCollisionEnabled` (`self.Box`) "QueryOnly"))

(event `/Game/AbilitySystem/BPI_AbilityParent.InteractAlternativeEvent`
  (params (instigator :type "/Game/Bobi/BobiCharacter Object Reference"))
  (bind _abilityowner (`self.AbilityOwner`))
  (if (== instigator _abilityowner)
    (bind _returnvalue (`|SpawnActorFromClass` "/Game/AbilitySystem/ToniAbilitys/CloneStationary/BP_AbilityStationaryClone.BP_AbilityStationaryClone_C" (`self.GetTransform`) "AlwaysSpawn" "OverrideRootScale" null self _abilityowner null null (struct) null))
    (`KismetArrayLibrary.Array_AddUnique` (`self.CloneArray`) _returnvalue)))

(event `/Game/AbilitySystem/BPI_AbilityParent.InteractPress`
  (params (Key :type "Key Structure"))
  (for _array_element (`self.CloneArray`)
    (`|ExecutionSequence`
      (:`then_0`
        (if (`KismetArrayLibrary.Array_Contains` (`self.MeleeKeys`) Key)
          (`/Engine/EditorBlueprintResources/StandardMacros.IsValid` _array_element
            (:`Is Valid`
              (`/Game/AbilitySystem/ToniAbilitys/CloneStationary/BP_AbilityStationaryClone.CloneMelee` _array_element)))))
      (:`then_1`
        (if (`KismetArrayLibrary.Array_Contains` (`self.DashKeys`) Key)
          (`/Engine/EditorBlueprintResources/StandardMacros.IsValid` _array_element
            (:`Is Valid`
              (`/Game/AbilitySystem/ToniAbilitys/CloneStationary/BP_AbilityStationaryClone.CloneDashMelee` _array_element))))))))

(fn `TraceNearestEnemy`
  (returns (Continue :type Boolean) (`Out Hit Hit Actor` :type "Actor Object Reference"))
  (locals (ObjectList :type "Array of EObjectTypeQuery Enum") (IgnoreArray :type "Array of Actor Object Reference"))
  (bind _ignorearray (`local.IgnoreArray`))
  (`KismetArrayLibrary.Array_Append` _ignorearray (`self.CloneArray`))
  (`KismetArrayLibrary.Array_Add` _ignorearray (`self.AbilityOwner`))
  (bind (_outhit _returnvalue) (`KismetSystemLibrary.SphereTraceSingleForObjects` (`self.K2_GetActorLocation`) (* (`self.GetActorForwardVector`) 50000.0) 100.0 (`local.ObjectList`) false (`local.IgnoreArray`)))
  (return _returnvalue (`.HitActor` (`GameplayStatics.BreakHitResult` _outhit))))

(fn `UserConstructionScript`
  (`parent.UserConstructionScript`))