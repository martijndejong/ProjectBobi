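; Clone recall ability actor: a kunai marker that lets its owning player teleport back to its position.
; On spawn it enables the knife's wallhack outline, tints its light and Niagara effect with the player color, and feeds the effect the ability lifespan.
; Pressing the default key notifies the owner's clone handler, moves the owner just above the marker, destroys it and spawns a poof at the owner's new location.
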(event `self.ReceiveBeginPlay`
  (bind _niagara (`self.Niagara`))
  (bind _playercolor (`/Game/Bobi/BobiCharacter.PlayerColor` (`self.AbilityOwner`)))
  (`parent.ReceiveBeginPlay`)
  (`self.SetWallhackOutline` (`self.KunaiKnife`))
  (`LightComponent.SetLightColor` (`self.RectLight`) _playercolor true)
  (`FXSystemComponent.SetColorParameter` _niagara "PlayerColor" _playercolor)
  (`FXSystemComponent.SetFloatParameter` _niagara "LifeSpan" (`.LifeSpan_41_814073994EF667A76BBDB0902D721D2E` (break `/Game/AbilitySystem/AbilityDetailsStruct` (`self.AbilityDetails`))))
  (`ActorComponent.Activate` _niagara false))

(event `/Game/AbilitySystem/BPI_AbilityParent.InteractPress`
  (params (Key :type "Key Structure"))
  (bind _abilityowner (`self.AbilityOwner`))
  (if (== Key (`self.DefaultKey`))
    (message `/Game/AbilitySystem/BPI_AbilityParent.InteractAlternativeEvent` (`/Game/Characters/Toni/BobiCharacter_Martijn.CloneHandlerRef` (cast `/Game/Characters/Toni/BobiCharacter_Martijn` _abilityowner :!pure true)) _abilityowner)
    (`self.K2_SetActorLocation` (`self.AbilityOwner`) (+ (`self.K2_GetActorLocation`) (0.0 0.0 50.0)) false false)
    (`self.K2_DestroyActor`)
    (`self.SpawnNiagaraPoof`)))

(fn `SpawnNiagaraPoof`
  (`NiagaraFunctionLibrary.SpawnSystemAtLocation` "/Game/AbilitySystem/ToniAbilitys/CloneStationary/P_ClonePoof.P_ClonePoof" (`self.K2_GetActorLocation` (`self.AbilityOwner`))))

(fn `UserConstructionScript`
  (`parent.UserConstructionScript`))