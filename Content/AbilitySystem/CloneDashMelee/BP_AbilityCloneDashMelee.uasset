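; Dash melee ability that damages actors its collision box overlaps, behaving differently when owned by a player character or a stationary clone.
; For a non-clone owner, it sends an interact message to overlapping clone handlers and dashes with distance and duration scaled by cast progress.
; A clone owner waits briefly, then timeline-lerps past the ability owner's position at distance-compensated speed, slashing on hit before both clone and ability are destroyed.
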(event `self.ReceiveBeginPlay`
  (if (!= (`GameplayStatics.GetObjectClass` (`self.GetOwner`)) "/Game/AbilitySystem/CloneStationary/BP_AbilityStationaryClone.BP_AbilityStationaryClone_C")
    (`parent.ReceiveBeginPlay`)))

(event `self.ActivateAbility`
  (bind _returnvalue (`KismetMathLibrary.MapRangeClamped` (`self.CastProgress`) 0.0 1.0 0.1 1.0))
  (if (!= (`GameplayStatics.GetObjectClass` (`self.GetOwner`)) "/Game/AbilitySystem/CloneStationary/BP_AbilityStationaryClone.BP_AbilityStationaryClone_C")
    (`parent.ActivateAbility`)
    (`|ExecutionSequence`
      (:`then_0`
        (message `/Game/AbilitySystem/BPI_AbilityParent.InteractPress` (`self.GetOverlappingActors` (`self.AbilityOwner`) "/Game/AbilitySystem/CloneStationary/BP_AbilityCloneHandler.BP_AbilityCloneHandler_C") (`self.DefaultKey`)))
      (:`then_1`
        (message `/Game/Bobi/BPI_ControllerToCharacter.Dash` (`self.AbilityOwner`) (* (`self.Distance`) _returnvalue) (* _returnvalue (`self.Duration`)))
        (`PrimitiveComponent.SetCollisionEnabled` (`self.Box`) "QueryAndPhysics")
        (`ActorComponent.Activate` (`self.P_SwordSlash`) false)
        (`GameplayStatics.PlaySoundAtLocation` "/Game/AbilitySystem/Melee/S_Sword_mixkit-metal-hit-woosh-1485.S_Sword_mixkit-metal-hit-woosh-1485" (`self.K2_GetActorLocation`) (struct) 1.0 1.0 0.0 null null null)
        (`self.K2_AttachToActor` (`self.GetOwner`) "None" "SnapToTarget" "SnapToTarget" "SnapToTarget")))
    (else
      (`KismetSystemLibrary.Delay` 0.2)
      (`self.CloneDash` (`self.K2_GetActorLocation` (`self.AbilityOwner`)))
      (`PrimitiveComponent.SetCollisionEnabled` (`self.Box`) "QueryAndPhysics")
      (`self.K2_AttachToActor` (`self.GetOwner`) "None" "SnapToTarget" "SnapToTarget" "SnapToTarget"))))

(event `self.Box.OnComponentBeginOverlap`
  (params (OverlappedComponent :type "PrimitiveComponent Object Reference") (OtherActor :type "Actor Object Reference") (OtherComp :type "PrimitiveComponent Object Reference") (OtherBodyIndex :type Integer) (bFromSweep :type Boolean) (SweepResult :type "HitResult Structure (by ref)"))
  (bind (_abilitydetails_name _abilitydetails_icon _abilitydetails_cooldown _abilitydetails_damage) (break `/Game/AbilitySystem/AbilityDetailsStruct` (`self.AbilityDetails`)))
  (if (and (!= OtherActor (`self.AbilityOwner`)) (!= OtherActor (`self.GetOwner`)))
    (`GameplayStatics.ApplyDamage` OtherActor _abilitydetails_damage (`Pawn.GetController` (`self.AbilityOwner`)))
    (if (== (`GameplayStatics.GetObjectClass` (`self.GetOwner`)) "/Game/AbilitySystem/CloneStationary/BP_AbilityStationaryClone.BP_AbilityStationaryClone_C")
      (`ActorComponent.Activate` (`self.P_SwordSlash`) false)
      (`GameplayStatics.PlaySoundAtLocation` "/Game/AbilitySystem/Melee/S_Sword_mixkit-metal-hit-woosh-1485.S_Sword_mixkit-metal-hit-woosh-1485" (`self.K2_GetActorLocation`) (struct) 1.0 1.0 0.0 null null null))))

(event `CloneDash`
  (params (EndPoint :type "Vector Structure"))
  (bind _returnvalue (`self.GetOwner`))
  (bind _dashstartpoint (`self.DashStartPoint`))
  (bind _dashendpoint (`self.DashEndPoint`))
  ;[1 1 1] Copied from bobi character parent
  (if (and (`KismetSystemLibrary.IsValid` _returnvalue) (== (`GameplayStatics.GetObjectClass` _returnvalue) "/Game/AbilitySystem/CloneStationary/BP_AbilityStationaryClone.BP_AbilityStationaryClone_C"))
    (bind _output_get (set `self.DashStartPoint` (`self.K2_GetActorLocation` (`self.GetOwner`))))
    (bind _output_get_2 (set `self.DashEndPoint` EndPoint))
    (`TimelineComponent.SetPlayRate` (`self.DashTimeLine`) (/ 1.0 (/ (+ (`KismetMathLibrary.Vector_Distance` _output_get _output_get_2) (`self.CloneDashOvershoot`)) (`self.CloneDashSpeed`))))
    (`self.K2_SetActorRotation` (`self.GetOwner`) (`KismetMathLibrary.FindLookAtRotation` (`self.DashStartPoint`) (`self.DashEndPoint`)) false)
    (bind (_direction _progressed) (`Timeline|DashTimeLine` :!via `PlayFromStart`)
      (:`Update`
        (`self.K2_SetActorLocation` (`self.GetOwner`) (`KismetMathLibrary.VLerp` _dashstartpoint (+ (* (`KismetMathLibrary.GetDirectionUnitVector` _dashstartpoint _dashendpoint) (`self.CloneDashOvershoot`)) _dashendpoint) _progressed) false false))
      (:`Finished`
        (`self.K2_DestroyActor` (`self.GetOwner`))
        (`self.K2_DestroyActor`)))))

(fn `UserConstructionScript`
  (`parent.UserConstructionScript`))