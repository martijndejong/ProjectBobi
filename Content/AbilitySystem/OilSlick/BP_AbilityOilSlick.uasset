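; Oil slick ability that lays a line of OilSpot actors forward from its origin along the owner's facing, out to Range.
; A looping tick lerps along that line using the cast timer's elapsed fraction, spawning spots where downward traces hit.
; Alternative interaction starts a second looping timer that spawns spots at the Instigator's location on trace hits, clearing itself one second after a hit.
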(event `Secondary tick`
  (bind _returnvalue (`self.K2_GetActorLocation` (stale `/Game/AbilitySystem/BPI_AbilityParent.InteractAlternativeEvent` instigator)))
  (bind (_outhit _returnvalue_2) (`KismetSystemLibrary.LineTraceSingle` :`Start` _returnvalue :`End` (0.0 0.0 -5000.0) :`TraceChannel` "TraceTypeQuery1" :`DrawDebugType` "ForDuration"))
  (if _returnvalue_2
    (`|SpawnActorFromClass` "/Game/AbilitySystem/OilSlick/OilSpot.OilSpot_C" (`KismetMathLibrary.Conv_VectorToTransform` _returnvalue) "Undefined" "OverrideRootScale" null null null null null "None" null)
    (`KismetSystemLibrary.Delay` 1.0)
    (`KismetSystemLibrary.K2_ClearAndInvalidateTimerHandle` (`self.SecondaryTickTimer`))))

(event `/Game/AbilitySystem/BPI_AbilityParent.InteractAlternativeEvent`
  (params (instigator :type "/Game/Bobi/BobiCharacter Object Reference"))
  (if (not (`KismetSystemLibrary.K2_IsTimerActiveHandle` (`self.SecondaryTickTimer`)))
    (bind _returnvalue (`KismetSystemLibrary.K2_SetTimerDelegate` (delegate `Secondary tick`) 0.2 true))
    (set `self.SecondaryTickTimer` _returnvalue)))

(event `StopSpittingOil`
  (`KismetSystemLibrary.K2_ClearAndInvalidateTimerHandle` (`self.TimerOilThrow`)))

(event `self.ActivateAbility`
  (`parent.ActivateAbility`)
  (bind _returnvalue (`KismetSystemLibrary.K2_SetTimerDelegate` (delegate `StopSpittingOil`) (`self.Cast duration`)))
  (set `self.TimerOilThrow` _returnvalue)
  (bind _returnvalue_2 (`KismetSystemLibrary.K2_SetTimerDelegate` (delegate `Tick`) (`.TickRate_44_026DC71E4BD359F38832A4B45B536C31` (break `/Game/AbilitySystem/AbilityDetailsStruct` (`self.AbilityDetails`))) true))
  (set `self.PrimaryTickTimer` _returnvalue_2)
  (bind _output_get (set `self.AbilityOrigin` (`self.K2_GetActorLocation`)))
  (set `self.AbilityEnd` (+ _output_get (* (`KismetMathLibrary.Normal` (`self.GetActorForwardVector` (`self.AbilityOwner`))) (`self.Range`)))))

(event `Tick`
  (bind _returnvalue (`KismetMathLibrary.VLerp` (`self.AbilityOrigin`) (`self.AbilityEnd`) (/ (`KismetSystemLibrary.K2_GetTimerElapsedTimeHandle` (`self.TimerOilThrow`)) (`self.Cast duration`))))
  (bind (_outhit _returnvalue_2) (`KismetSystemLibrary.LineTraceSingle` :`Start` _returnvalue :`End` (- _returnvalue (0.0 0.0 1000.0)) :`TraceChannel` "TraceTypeQuery1" :`DrawDebugType` "ForDuration"))
  (if _returnvalue_2
    (`|SpawnActorFromClass` "/Game/AbilitySystem/OilSlick/OilSpot.OilSpot_C" (`KismetMathLibrary.Conv_VectorToTransform` _returnvalue) "Undefined" "OverrideRootScale" null self null null null "None" null)))

(fn `UserConstructionScript`
  (`parent.UserConstructionScript`))