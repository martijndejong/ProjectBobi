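; Oil spot actor from the OilSlick ability that alters the movement of actors overlapping it.
; On overlap it sends a slow-effect message that boosts the ability owner and heavily slows anyone else, then resets the multiplier on exit.
; Its lifespan comes from the ability details, and alternative interact events are forwarded to the main oil actor.
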(event `/Game/AbilitySystem/BPI_AbilityParent.InteractAlternativeEvent`
  (params (instigator :type "/Game/Bobi/BobiCharacter Object Reference"))
  (`/Game/AbilitySystem/BPI_AbilityParent.InteractAlternativeEvent` (`self.MainOil`) instigator))

(event `self.ReceiveActorBeginOverlap`
  (params (OtherActor :type "Actor Object Reference"))
  (if (== OtherActor (`self.AbilityOwner`))
    (message `/Game/Bobi/BPI_ControllerToCharacter.AddSlowEffect` OtherActor 1.5)
    (else
      (message `/Game/Bobi/BPI_ControllerToCharacter.AddSlowEffect` OtherActor 0.2))))

(event `self.ReceiveBeginPlay`
  (`self.SetLifeSpan` (`.LifeSpan_41_814073994EF667A76BBDB0902D721D2E` (break `/Game/AbilitySystem/AbilityDetailsStruct` (`self.AbilityDetails`)))))

(event `self.ReceiveActorEndOverlap`
  (params (OtherActor :type "Actor Object Reference"))
  (message `/Game/Bobi/BPI_ControllerToCharacter.AddSlowEffect` OtherActor 1.0))

(fn `UserConstructionScript`)