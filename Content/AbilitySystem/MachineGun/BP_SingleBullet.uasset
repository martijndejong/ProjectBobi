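; BP_SingleBullet is a bullet actor for the MachineGun ability that damages what it hits.
; On spawn it plays a gunshot sound with randomized, clamped volume and pitch.
; Its Box overlap ignores the ability owner, applies the ability's damage credited to the owner's controller, then destroys the bullet.
; BobiCharacter targets also get a small knockback along the bullet's velocity with slight lift, launched after the destroy call.
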(event `self.ReceiveBeginPlay`
  (`GameplayStatics.PlaySoundAtLocation` "/Game/AbilitySystem/MachineGun/GunShot.GunShot" (`self.K2_GetActorLocation`) (struct) (`KismetMathLibrary.FClamp` (`KismetMathLibrary.RandomFloat`) 0.7) (`KismetMathLibrary.FClamp` (`KismetMathLibrary.RandomFloat`) 0.9) 0.1 null null null))

(event `self.Box.OnComponentBeginOverlap`
  (params (OverlappedComponent :type "PrimitiveComponent Object Reference") (OtherActor :type "Actor Object Reference") (OtherComp :type "PrimitiveComponent Object Reference") (OtherBodyIndex :type Integer) (bFromSweep :type Boolean) (SweepResult :type "HitResult Structure (by ref)"))
  ;[1 1 1] Copy pasted from melee
  (if (not (== OtherActor (`self.AbilityOwner`)))
    (`/Engine/EditorBlueprintResources/StandardMacros.IsValid` OtherActor
      (:`Is Valid`
        (`GameplayStatics.ApplyDamage` OtherActor (`.Damage_29_66822423450AE486B2C9FE8E4C4D325E` (break `/Game/AbilitySystem/AbilityDetailsStruct` (`self.AbilityDetails`))) (`Pawn.GetController` (`self.AbilityOwner`)) self)
        (`self.K2_DestroyActor`)
        (bind _asbobi_character (cast `/Game/Bobi/BobiCharacter` OtherActor))
        (`/Engine/EditorBlueprintResources/StandardMacros.IsValid` _asbobi_character
          (:`Is Valid`
            (`Character.LaunchCharacter` _asbobi_character (+ (* (`KismetMathLibrary.Normal` (`self.GetVelocity`)) 100.0) (0.0 0.0 10.0)) false false)))))))

(fn `UserConstructionScript`)