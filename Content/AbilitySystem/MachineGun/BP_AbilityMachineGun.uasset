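; Machine gun ability that fires BP_SingleBullet actors from the owner's transform while the default key is held.
; A looping timer at the ability's tick rate repeats shots; firing starts immediately on BeginPlay or press and stops on release.
; Each shot decrements ammo and updates a special HUD overlay; running out or pressing a reload key destroys the ability and removes the overlay.
; ActivateAbility is left empty to override parent behavior.
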(event `/Game/AbilitySystem/BPI_AbilityParent.InteractRelease`
  (params (Key :type "Key Structure"))
  (if (== Key (`self.DefaultKey`))
    (`KismetSystemLibrary.K2_ClearAndInvalidateTimerHandle` (`self.TimerShooting`))))

(event `/Game/AbilitySystem/BPI_AbilityParent.InteractPress`
  (params (Key :type "Key Structure"))
  (bind _abilityowner (`self.AbilityOwner`))
  (if (== Key (`self.DefaultKey`))
    (if (not (`KismetSystemLibrary.K2_IsTimerActiveHandle` (`self.TimerShooting`)))
      (bind _returnvalue (`KismetSystemLibrary.K2_SetTimerDelegate` (delegate `ShootBullet`) (`.TickRate_44_026DC71E4BD359F38832A4B45B536C31` (break `/Game/AbilitySystem/AbilityDetailsStruct` (`self.AbilityDetails`))) true :!label _label))
      (set `self.TimerShooting` _returnvalue)
      (`|SpawnActorFromClass` "/Game/AbilitySystem/MachineGun/BP_SingleBullet.BP_SingleBullet_C" (`self.GetTransform` _abilityowner) "AlwaysSpawn" "OverrideRootScale" null (`self.AbilityDetails`) _abilityowner null :!label _label_2)
      (bind _result (`/Engine/EditorBlueprintResources/StandardMacros.DecrementInt` (`self.CurrentAmmo`))
        (:`  `
          (`/Game/AbilitySystem/MachineGun/HUD_AmmoCount.SetAmmoCounter` (cast `/Game/AbilitySystem/MachineGun/HUD_AmmoCount` (`self.AmmoCountHUDRef`) :!pure true) _result)
          (if (<= _result 0)
            (`self.K2_DestroyActor` :!label _label_3)
            (`Widget.RemoveFromParent` (`self.AmmoCountHUDRef`))))))
    (elif (`KismetArrayLibrary.Array_Contains` (`self.ReloadKeys`) Key)
      (goto _label_3))))

(event `self.ReceiveBeginPlay`
  (`parent.ReceiveBeginPlay`)
  (bind _specialoverlayref (`/Game/HUD/HUD_Overhaul/HUD_Ability.AddSpecialOverlay` (`/Game/AbilitySystem/BP_AbilityHandler_ActorComponent.AbilityHUDRef` (`self.AbilityHandlerRef`)) null))
  (set `self.AmmoCountHUDRef` _specialoverlayref)
  (goto _label))

(event `ShootBullet`
  (goto _label_2))

(event `self.ActivateAbility`
  ;[1 1 1 1 12] Empty - to overwrite parent behavior
)

(fn `UserConstructionScript`
  (`parent.UserConstructionScript`))