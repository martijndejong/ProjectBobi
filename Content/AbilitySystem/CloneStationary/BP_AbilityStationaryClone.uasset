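; Stationary clone ability actor that copies its owner's skeletal mesh and materials and expires after a short life span or any damage.
; While FollowOwner is set, Tick faces it toward the handler's traced nearest enemy, otherwise matches the handler's rotation.
; CloneMelee and CloneDashMelee spawn and activate separate ability actors, with the dash also clearing life span, collision and tracking.
; On destruction, it leaves the handler's CloneArray with a poof effect.
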(event `self.ReceiveBeginPlay`
  (bind _mesh (`Character.Mesh` (`self.AbilityOwner`)))
  ;[1 1 1] Life span
  (`self.SetLifeSpan` 5.0)
  (`SkinnedMeshComponent.SetSkinnedAssetAndUpdate` (`self.SkeletalMesh`) (`SkinnedMeshComponent.SkeletalMesh` _mesh) true)
  (for (_array_element _array_index) (`MeshComponent.GetMaterials` _mesh)
    (`PrimitiveComponent.SetMaterial` (`self.SkeletalMesh`) _array_index _array_element)))

(event `self.ReceiveAnyDamage`
  (params (Damage :type "Float (single-precision)") (DamageType :type "DamageType Object Reference") (InstigatedBy :type "Controller Object Reference") (DamageCauser :type "Actor Object Reference"))
  (`KismetSystemLibrary.Delay` 0.01)
  (`self.K2_DestroyActor`))

(event `self.ReceiveDestroyed`
  (bind _clonehandlerref (`self.CloneHandlerRef`)
    (:`then`
      (`KismetArrayLibrary.Array_RemoveItem` (`/Game/AbilitySystem/CloneStationary/BP_AbilityCloneHandler.CloneArray` _clonehandlerref) self)
      (`NiagaraFunctionLibrary.SpawnSystemAtLocation` "/Game/AbilitySystem/CloneStationary/P_ClonePoof.P_ClonePoof" (`self.K2_GetActorLocation`)))
    (:`else`)))

(event `CloneMelee`
  (bind _returnvalue (`|SpawnActorFromClass` "/Game/AbilitySystem/CloneMelee/BP_AbilityCloneMelee.BP_AbilityCloneMelee_C" (`self.GetTransform`) "Undefined" "OverrideRootScale" self (`self.AbilityOwner`) null null (struct) null))
  (`self.ActivateAbility` _returnvalue))

(event `self.ReceiveTick`
  (params (DeltaSeconds :type "Float (single-precision)"))
  (if (`self.FollowOwner`)
    (bind _clonehandlerref (`self.CloneHandlerRef`)
      (:`then`
        (bind (_continue _out_hit_hit_actor) (`/Game/AbilitySystem/CloneStationary/BP_AbilityCloneHandler.TraceNearestEnemy` _clonehandlerref))
        (if _continue
          (`self.K2_SetActorRotation` (`KismetMathLibrary.FindLookAtRotation` (`self.K2_GetActorLocation`) (`self.K2_GetActorLocation` _out_hit_hit_actor)))
          (else
            (`self.K2_SetActorRotation` (`self.K2_GetActorRotation` (`self.CloneHandlerRef`))))))
      (:`else`))))

(event `CloneDashMelee`
  (`self.SetLifeSpan` 0.0)
  (`PrimitiveComponent.SetCollisionEnabled` (`self.Capsule`) "NoCollision")
  (set `self.FollowOwner` false)
  (bind _returnvalue (`|SpawnActorFromClass` "/Game/AbilitySystem/CloneDashMelee/BP_AbilityCloneDashMelee.BP_AbilityCloneDashMelee_C" (`self.GetTransform`) "Undefined" "OverrideRootScale" self (`self.AbilityOwner`) null null (struct) null))
  (`self.ActivateAbility` _returnvalue))

(fn `UserConstructionScript`
  (`parent.UserConstructionScript`))