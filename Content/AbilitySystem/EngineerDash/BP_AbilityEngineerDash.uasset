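; Ability actor for the Engineer dash, which moves its owner a set distance along its current horizontal direction of travel.
; On BeginPlay it zeroes the owner's vertical velocity, then computes the end point from the ability actor's own location and the owner's normalized horizontal velocity.
; A timeline with play rate scaled by dash duration lerps the owner between those points, setting location without sweep, so collisions do not block it.
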(event `self.ReceiveBeginPlay`
  (bind _abilityowner (`self.AbilityOwner`))
  (bind (_returnvalue_x _returnvalue_y) (`KismetMathLibrary.BreakVector` (`self.GetVelocity` _abilityowner)))
  (`parent.ReceiveBeginPlay`)
  ;[1 1 1] stop fall speed
  (set `MovementComponent.Velocity` (`KismetMathLibrary.MakeVector` _returnvalue_x _returnvalue_y) (`Pawn.GetMovementComponent` _abilityowner))
  (bind _output_get (set `self.DashStartPoint` (`self.K2_GetActorLocation`)))
  (set `self.DashEndPoint` (+ _output_get (* (`KismetMathLibrary.Normal` (`KismetMathLibrary.MakeVector` _returnvalue_x _returnvalue_y)) (`self.Dash Distance`))))
  (`TimelineComponent.SetPlayRate` (`self.EngineerDashTimeLine`) (/ 1.0 (`self.Dash Duration`)))
  (bind (_direction _progressed) (`Timeline|EngineerDashTimeLine` :!via `PlayFromStart`)
    (:`Update`
      (`self.K2_SetActorLocation` (`self.AbilityOwner`) (`KismetMathLibrary.VLerp` (`self.DashStartPoint`) (`self.DashEndPoint`) _progressed) false false))))

(fn `UserConstructionScript`
  (`parent.UserConstructionScript`))