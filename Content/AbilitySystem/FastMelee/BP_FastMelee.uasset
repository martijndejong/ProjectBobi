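; Fast melee ability that damages actors touched by its box hitbox.
; Activation runs the parent logic, then enables the box's collision for queries and physics.
; Overlaps apply damage to anyone but the ability owner, scaling the configured damage from a reduced fraction up to full with cast progress.
; The update event is overridden empty, leaving its parent call and cast-progress arrow scaling disconnected.
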(event `self.UpdateAbility`)

(event `self.ActivateAbility`
  (`parent.ActivateAbility`)
  (`PrimitiveComponent.SetCollisionEnabled` (`self.Box`) "QueryAndPhysics"))

(event `self.Box.OnComponentBeginOverlap`
  (params (OverlappedComponent :type "PrimitiveComponent Object Reference") (OtherActor :type "Actor Object Reference") (OtherComp :type "PrimitiveComponent Object Reference") (OtherBodyIndex :type Integer) (bFromSweep :type Boolean) (SweepResult :type "HitResult Structure (by ref)"))
  (bind (_abilitydetails_name _abilitydetails_icon _abilitydetails_cooldown _abilitydetails_damage) (break `/Game/AbilitySystem/AbilityDetailsStruct` (`self.AbilityDetails`)))
  (if (not (== OtherActor (`self.AbilityOwner`)))
    (`GameplayStatics.ApplyDamage` OtherActor (* (`KismetMathLibrary.MapRangeClamped` (`self.CastProgress`) 0.0 1.0 0.2 1.0) _abilitydetails_damage))))

(fn `UserConstructionScript`
  (`parent.UserConstructionScript`))