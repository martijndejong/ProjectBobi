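; Holy Ground ability actor that creates a ground area applying periodic damage to its owner while they stand inside it.
; On activation it line-traces downward, teleports to the hit location, then reveals its decal and enables area-of-effect collision.
; A looping timer at the ability's tick rate scans overlapping actors and calls ApplyDamage with the configured damage only on the ability owner.
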(event `self.ActivateAbility`
  (bind _returnvalue (`self.K2_GetActorLocation`))
  (bind (_abilitydetails_name _abilitydetails_icon _abilitydetails_cooldown _abilitydetails_damage _abilitydetails_tickrate) (break `/Game/AbilitySystem/AbilityDetailsStruct` (`self.AbilityDetails`)))
  (`parent.ActivateAbility`)
  (bind _outhit (`KismetSystemLibrary.LineTraceSingle` :`Start` _returnvalue :`End` (- _returnvalue (0.0 0.0 1000.0)) :`TraceChannel` "TraceTypeQuery1" :`DrawDebugType` "ForDuration"))
  (`self.K2_SetActorLocation` (`.Location` (`GameplayStatics.BreakHitResult` _outhit)) false true)
  (`SceneComponent.SetVisibility` (`self.Decal`) true false)
  (`PrimitiveComponent.SetCollisionEnabled` (`self.AreaOfEffect`) "QueryAndPhysics")
  (`KismetSystemLibrary.K2_SetTimerDelegate` (delegate `Tick`) _abilitydetails_tickrate true))

(event `Tick`
  (bind (_abilitydetails_name _abilitydetails_icon _abilitydetails_cooldown _abilitydetails_damage _abilitydetails_tickrate) (break `/Game/AbilitySystem/AbilityDetailsStruct` (`self.AbilityDetails`)))
  (for _array_element (`PrimitiveComponent.GetOverlappingActors` (`self.AreaOfEffect`) null)
    (if (== _array_element (`self.AbilityOwner`))
      (`GameplayStatics.ApplyDamage` _array_element _abilitydetails_damage))))

(fn `UserConstructionScript`
  (`parent.UserConstructionScript`))