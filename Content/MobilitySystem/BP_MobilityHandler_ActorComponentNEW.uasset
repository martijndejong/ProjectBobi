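; Mobility handler actor component that spends HUD-tracked dash charges to make the owning Bobi character dash.
; On a short delay after BeginPlay, it creates the mobility HUD from the character's dash count, fills its charge array and links it to the owner.
; Press spends a charge through the HUD and, on success, sends the character a dash message with duration and distance.
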(event `self.ReceiveBeginPlay`
  ;[1 1 1] Prevent "none" trying access Mobility Owner
  (`KismetSystemLibrary.Delay` 0.1)
  (bind _mobilitybar (message `/Game/Bobi/BPI_CharacterToController.AddMobilityHUD` (`self.PlayerController`) (`.NumberOfDashes_35_421618FC4D1A470408CD5D8E37AAD2C5` (break `/Game/Bobi/CharacterSpecs` (`/Game/Bobi/BobiCharacter.CharacterSpecs` (`self.MobilityOwner`))))))
  (bind _output_get (set `self.Mobility HUD Ref` _mobilitybar))
  (`/Game/MobilitySystem/WBP_HUD_Mobility.PopulateChargeArray` _output_get)
  (`self.SetBobiReference` (`self.MobilityOwner`)))

(event `Press`
  (bind _succes (`/Game/MobilitySystem/WBP_HUD_Mobility.SpendCharge` (`self.Mobility HUD Ref`)))
  (if _succes
    (bind _mobilityowner (`self.MobilityOwner`)
      (:`then`
        (message `/Game/Bobi/BPI_BobiCharacter.Dash` _mobilityowner (`self.Duration`) (`self.Distance`) true true true))
      (:`else`))))

(fn `SetBobiReference`
  (params (BobiCharacter :type "/Game/Bobi/BobiCharacter Object Reference"))
  (bind _output_get (set `self.MobilityOwner` BobiCharacter))
  (bind _mobility_hud_ref (`self.Mobility HUD Ref`)
    (:`then`
      (`/Game/MobilitySystem/WBP_HUD_Mobility.SetMobilityOwner` _mobility_hud_ref _output_get))
    (:`else`)))