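; BP_MobilitySprint is a mobility-system Blueprint that makes its owning character sprint for as long as it exists.
; On BeginPlay it sets the owner's walk speed to double the RunSpeed from its CharacterSpecs and starts a looping timer that repeatedly calls SpendStamina with StaminaCost.
; When destroyed, it restores normal run speed and clears the timer.
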(event `self.ReceiveBeginPlay`
  (bind _mobilityowner (`self.MobilityOwner`))
  (`parent.ReceiveBeginPlay`)
  (set `CharacterMovementComponent.MaxWalkSpeed` (* (`.RunSpeed_6_BCF94D1048B54DEC85D13DAA043A2916` (break `/Game/Bobi/CharacterSpecs` (`/Game/Bobi/BobiCharacter.CharacterSpecs` _mobilityowner))) 2.0) (`Character.CharacterMovement` _mobilityowner))
  (bind _returnvalue (`KismetSystemLibrary.K2_SetTimerDelegate` (delegate `Update`) 0.1 true))
  (set `self.TimerSpendStamina` _returnvalue))

(event `Update`
  (`self.SpendStamina` (`self.StaminaCost`)))

(event `self.ReceiveDestroyed`
  (bind _mobilityowner (`self.MobilityOwner`))
  (set `CharacterMovementComponent.MaxWalkSpeed` (`.RunSpeed_6_BCF94D1048B54DEC85D13DAA043A2916` (break `/Game/Bobi/CharacterSpecs` (`/Game/Bobi/BobiCharacter.CharacterSpecs` _mobilityowner))) (`Character.CharacterMovement` _mobilityowner))
  (`KismetSystemLibrary.K2_ClearAndInvalidateTimerHandle` (`self.TimerSpendStamina`)))

(fn `UserConstructionScript`
  (`parent.UserConstructionScript`))