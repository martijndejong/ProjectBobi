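; Actor component that handles a player's mobility ability and the stamina that powers it.
; On press it interrupts any casting ability handler, then, given enough stamina, spawns the mobility ability actor and pauses regeneration.
; Releasing a hold-down ability, forced destruction or running out of stamina destroys that actor and restarts timer-based regeneration.
; Stamina changes are pushed to a mobility HUD created through the player controller on BeginPlay.
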(event `Press`
  (bind _mobilityowner (`self.MobilityOwner`))
  (bind _mobilityability (`self.MobilityAbility`))
  (bind _continue (`self.AttemptInterruptAllOtherAbilities`))
  (if _continue
    (if (>= (`self.CurrentStamina`) (`.StaminaCost` (defaults `Object` _mobilityability)))
      (bind _returnvalue (`|SpawnActorFromClass` _mobilityability (`Actor.GetTransform` _mobilityowner) "Undefined" "OverrideRootScale" null _mobilityowner self null))
      (set `self.MobilityActorRef` _returnvalue)
      (`KismetSystemLibrary.K2_ClearAndInvalidateTimerHandle` (`self.StaminaRegenTimer`)))))

(event `ForcedDestroy`
  (bind _mobilityactorref (`self.MobilityActorRef` :!label _label)
    (:`then`
      (`Actor.K2_DestroyActor` _mobilityactorref)
      (bind _returnvalue (`KismetSystemLibrary.K2_SetTimerDelegate` (delegate `RegenStamina`) 0.1 true :!label _label_2))
      (set `self.StaminaRegenTimer` _returnvalue))
    (:`else`)))

(event `Release`
  (if (`.IsHoldDown` (defaults `Object` (`self.MobilityAbility`)))
    (goto _label)))

(event `SpendStamina`
  (params (StaminaCost :type "Float (double-precision)"))
  (set `self.CurrentStamina` (`KismetMathLibrary.FClamp` (- (`self.CurrentStamina`) StaminaCost) 0.0 (`self.MaxStamina`)))
  (`/Game/HUD/HUD_Mobility.UpdateState` (`self.MobilityHUDRef`) self)
  (if (<= (`self.CurrentStamina`) 0.0)
    (bind _mobilityactorref (`self.MobilityActorRef`)
      (:`then`
        (`Actor.K2_DestroyActor` _mobilityactorref)
        (goto _label_2))
      (:`else`))))

(event `RegenStamina`
  (set `self.CurrentStamina` (`KismetMathLibrary.FClamp` (+ (`self.CurrentStamina`) 1.0) 0.0 (`self.MaxStamina`)))
  (`/Game/HUD/HUD_Mobility.UpdateState` (`self.MobilityHUDRef`) self)
  (if (>= (`self.CurrentStamina`) (`self.MaxStamina`))
    (`KismetSystemLibrary.K2_ClearAndInvalidateTimerHandle` (`self.StaminaRegenTimer`))))

(event `self.ReceiveBeginPlay`
  (bind _mobilityhud (message `/Game/Bobi/BPI_CharacterToController.AddMobilityHUD` (`self.PlayerController`)))
  (bind _output_get (set `self.MobilityHUDRef` _mobilityhud))
  (`/Game/HUD/HUD_Mobility.UpdateState` _output_get self))

(event `PlayerSpawnedMH`
  (params (BobiCharacter :type "/Game/Bobi/BobiCharacter Object Reference"))
  (set `self.MobilityOwner` BobiCharacter))

(fn `AttemptInterruptAllOtherAbilities`
  (returns (Continue :type Boolean))
  (locals (FoundCasting :type Boolean))
  ;[1 1 1] For each ability handler (except self), see if it is casting
  (set `local.FoundCasting` false)
  (for _array_element (`Actor.K2_GetComponentsByClass` (`self.GetOwner`) "/Game/AbilitySystem/BP_AbilityHandler_ActorComponent.BP_AbilityHandler_ActorComponent_C")
    (if (`/Game/AbilitySystem/BP_AbilityHandler_ActorComponent.IsCasting` _array_element)
      ;[1 1 1] If it is -> interrupt (if not self) it
      (set `local.FoundCasting` true)
      (bind _activeabilityref (`/Game/AbilitySystem/BP_AbilityHandler_ActorComponent.ActiveAbilityRef` _array_element))
      (`/Engine/EditorBlueprintResources/StandardMacros.IsValid` _activeabilityref
        (:`Is Valid`
          (if (!= self _array_element)
            (bind _interrupted (message `/Game/AbilitySystem/BPI_AbilityParent.Interrupt` _activeabilityref))
            ;;[1 1 1 1 12] Continue if succesfully interupted (i.e., if ability was interruptable)
            (return _interrupted)))
        (:`Is Not Valid`
          ;[1 1 1 1 12] Also continue if ability was destroyed within time frame that 'IsCasting' was still true
          (return true)))))
  (if (not (`local.FoundCasting`))
    ;[1 1 1 1 12] Also continue if none of the ability handlers were casting
    (return true)))