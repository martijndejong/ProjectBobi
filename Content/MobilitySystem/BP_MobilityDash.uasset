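; Mobility ability that dashes its owner a set distance along its horizontal velocity on BeginPlay, spending stamina and zeroing vertical speed.
; A timeline scaled to the dash duration lerps the owner's location without sweep, then has the mobility handler force-destroy.
; As the dash starts, a debug-drawn multi-object line trace along the path sends an alternative interact interface message to each actor hit.
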(event `self.ReceiveBeginPlay`
  (bind _mobilityowner (`self.MobilityOwner`))
  (bind (_returnvalue_x _returnvalue_y) (`KismetMathLibrary.BreakVector` (`self.GetVelocity` _mobilityowner)))
  (`parent.ReceiveBeginPlay`)
  ;[1 1 1] stop fall speed
  (set `MovementComponent.Velocity` (`KismetMathLibrary.MakeVector` _returnvalue_x _returnvalue_y) (`Pawn.GetMovementComponent` _mobilityowner))
  (`self.SpendStamina` (`self.StaminaCost`))
  (bind _output_get (set `self.DashStartPoint` (`self.K2_GetActorLocation`)))
  (set `self.DashEndPoint` (+ _output_get (* (`KismetMathLibrary.Normal` (`KismetMathLibrary.MakeVector` _returnvalue_x _returnvalue_y)) (`self.DashDistance`))))
  (`TimelineComponent.SetPlayRate` (`self.DashTimeLine`) (/ 1.0 (`self.DashDuration`)))
  (`|ExecutionSequence`
    (:`then_0`
      (bind (_direction _progressed) (`Timeline|DashTimeLine` :!via `PlayFromStart`)
        (:`Update`
          (`self.K2_SetActorLocation` (`self.MobilityOwner`) (`KismetMathLibrary.VLerp` (`self.DashStartPoint`) (`self.DashEndPoint`) _progressed) false false))
        (:`Finished`
          (`/Game/MobilitySystem/BP_MobilityHandler_ActorComponent.ForcedDestroy` (`self.MobilityHandlerRef`)))))
    (:`then_1`
      (bind _outhits (`KismetSystemLibrary.LineTraceMultiForObjects` :`Start` (`self.DashStartPoint`) :`End` (`self.DashEndPoint`) :`ObjectTypes` (`self.Object Types`) :`DrawDebugType` "ForDuration" :`DrawTime` 2.0))
      (for _array_element _outhits
        (message `/Game/AbilitySystem/BPI_AbilityParent.InteractAlternativeEvent` (`.HitActor` (`GameplayStatics.BreakHitResult` _array_element)) (`self.MobilityOwner`))))))

(fn `UserConstructionScript`
  (`parent.UserConstructionScript`))