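; BP_MobilityHandler_ActorComponent is an actor component that gates the Bobi character's dash behind HUD-tracked charges.
; After a short delay on BeginPlay, it has the player controller create a mobility HUD sized by the character's dash count and fills its charge array.
; On Press, it asks the HUD to spend a charge and, if that succeeds, sends a dash message with distance and duration to the owner set through SetBobiReference.
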(event `self.ReceiveBeginPlay`
  ;[1 1 1 1 10] Prevent: "accessed NONE trying to read 'Mobility Owner'
  (`KismetSystemLibrary.Delay` 0.2)
  (bind _mobilitybar (message `/Game/Bobi/BPI_CharacterToController.AddMobilityHUD` (`self.PlayerController`) (`.NumberOfDashes_35_421618FC4D1A470408CD5D8E37AAD2C5` (break `/Game/Bobi/CharacterSpecs` (`/Game/Bobi/BobiCharacter.CharacterSpecs` (`self.MobilityOwner`))))))
  (bind _output_get (set `self.Mobility HUD Ref` _mobilitybar))
  (`/Game/MobilitySystem/New/WBP_HUD_Mobility.PopulateChargeArray` _output_get))

(event `Press`
  (bind _succes (`/Game/MobilitySystem/New/WBP_HUD_Mobility.SpendCharge` (`self.Mobility HUD Ref`)))
  (if _succes
    (message `/Game/Bobi/BPI_ControllerToCharacter.Dash` (`self.MobilityOwner`) (`self.Distance`) (`self.Duration`))))

(fn `SetBobiReference`
  (params (BobiCharacter :type "/Game/Bobi/BobiCharacter Object Reference"))
  (set `self.MobilityOwner` BobiCharacter))