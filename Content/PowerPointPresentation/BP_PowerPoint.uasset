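; BP_PowerPoint runs an in-game slideshow that the player pages through with the left and right arrow inputs.
; On BeginPlay it fills a hardcoded slide array and adds a WBP_PowerPoint widget to the viewport.
; UpdateSlide steps a clamped index and pushes that slide's image to the widget, opening MenuJoinedLevel once the index passes the last slide.
; No slide is pushed to the widget until the first arrow press.
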(event `self.ReceiveBeginPlay`
  (set `self.slides` (`|MakeArray` "/Game/PowerPointPresentation/slides/Slide1.Slide1" "/Game/PowerPointPresentation/slides/Slide2.Slide2" "/Game/PowerPointPresentation/slides/Slide3.Slide3" "/Game/PowerPointPresentation/slides/Slide4.Slide4" "/Game/PowerPointPresentation/slides/Slide5.Slide5" "/Game/PowerPointPresentation/slides/Slide6.Slide6" "/Game/PowerPointPresentation/slides/Slide7.Slide7" "/Game/PowerPointPresentation/slides/Slide8.Slide8" "/Game/PowerPointPresentation/slides/Slide9.Slide9" "/Game/PowerPointPresentation/slides/Slide10.Slide10" "/Game/PowerPointPresentation/slides/Slide11.Slide11" "/Game/PowerPointPresentation/slides/Slide12.Slide12" "/Game/PowerPointPresentation/slides/Slide13.Slide13" "/Game/PowerPointPresentation/slides/Slide14.Slide14" "/Game/PowerPointPresentation/slides/Slide15.Slide15" "/Game/PowerPointPresentation/slides/Slide16.Slide16" "/Game/PowerPointPresentation/slides/Slide17.Slide17" "/Game/PowerPointPresentation/slides/Slide18.Slide18" "/Game/PowerPointPresentation/slides/Slide19.Slide19" "/Game/PowerPointPresentation/slides/Slide20.Slide20" "/Game/PowerPointPresentation/slides/Slide21.Slide21" :!type "Texture2D Object Reference"))
  (bind _returnvalue (`|CreateWidget` "/Game/PowerPointPresentation/WBP_PowerPoint.WBP_PowerPoint_C"))
  (`UserWidget.AddToViewport` _returnvalue 0)
  (set `self.PowerPointREF` _returnvalue))

(event `InputAction|ArrowLeft`
  (params (Key :type "Key Structure"))
  (:`Pressed`
    (`self.UpdateSlide` -1)))

(event `InputAction|ArrowRight`
  (params (Key :type "Key Structure"))
  (:`Pressed`
    (`self.UpdateSlide` 1)))

(fn `UpdateSlide`
  (params (increment :type Integer))
  (bind _output_get (set `self.CurrentSlideID` (`KismetMathLibrary.Clamp` (+ (`self.CurrentSlideID`) increment) 0 100)))
  (if (>= _output_get (`KismetArrayLibrary.Array_Length` (`self.slides`)))
    (`GameplayStatics.OpenLevel` "MenuJoinedLevel")
    (else
      (`/Game/PowerPointPresentation/WBP_PowerPoint.SetImage` (`self.PowerPointREF`) (`|GetArrayItem` (`self.slides`) _output_get)))))

(fn `UserConstructionScript`)