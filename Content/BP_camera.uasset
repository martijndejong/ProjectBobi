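; BP_camera is a shared multiplayer camera that follows the group and zooms with player spread.
; GameStarted stores the active players and enables Tick, where CameraMovment lerps a Sphere toward their average location by a fixed per-tick alpha.
; Tick also measures pairwise distances between all Character actors, not just active players, and sets the spring arm length to the largest, clamped between minimum and maximum limits.
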(event `self.ReceiveTick`
  (params (DeltaSeconds :type "Float (single-precision)"))
  (if (`self.bGameStarted`)
    (`self.CameraMovment`)
    (bind _outactors (`GameplayStatics.GetAllActorsOfClass` "/Script/Engine.Character"))
    (for (_array_element _array_index) _outactors
      (set `self.CurrentPlayer` null)
      (for _index (range (+ _array_index 1) (`KismetArrayLibrary.Array_Length` _outactors))
        (`KismetArrayLibrary.Array_Add` (`self.Distance`) (`self.GetDistanceTo` _array_element (`|GetArrayItem` _outactors _index)))))
    (set `SpringArmComponent.TargetArmLength` (`KismetMathLibrary.FClamp` (`.MaxValue` (`KismetMathLibrary.MaxOfFloatArray` (`self.Distance`))) (`self.MinArmLenght`) (`self.MaxArmLengt`)) (`self.SpringArm`))
    (`KismetArrayLibrary.Array_Clear` (`self.Distance`))))

(fn `CameraMovment`
  (set `self.PreviouseLocation` (`SceneComponent.K2_GetComponentLocation` (`self.Sphere`)))
  (bind _returnvalue (`GameplayStatics.GetActorArrayAverageLocation` (`self.Active Players`)))
  (`SceneComponent.K2_SetWorldLocation` (`self.Sphere`) (`KismetMathLibrary.VLerp` (`self.PreviouseLocation`) _returnvalue (`self.CameraMoveSpeed`)) false false))

(fn `GameStarted`
  (params (ActivePlayers :type "Array of /Game/Bobi/BobiCharacter_Copy Object Reference"))
  (set `self.Active Players` ActivePlayers)
  (set `self.bGameStarted` true))

(fn `UserConstructionScript`)