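; Health pack pickup that hides on overlap and respawns after a recharge time.
; Overlapping the capsule passes HealAmount to ApplyDamage on any actor, with no filtering, then disables collision and starts recharging.
; While available, a timeline spins and bobs the cross mesh.
; During recharge, a looping timer writes elapsed progress to the plane's dynamic clock material until respawn restores the cross and collision.
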(event `self.ReceiveBeginPlay`
  (bind _returnvalue (`PrimitiveComponent.CreateDynamicMaterialInstance` (`self.Plane`) 0 null "None"))
  (bind _output_get (set `self.DynMatClock` _returnvalue))
  (`MaterialInstanceDynamic.SetVectorParameterValue` _output_get "Color" (struct :`G` 3.83031 :`B` 5.0 :`A` 1.0))
  (`self.SpawnHealthPack`)
  (bind _returnvalue_2 (`PrimitiveComponent.CreateDynamicMaterialInstance` (`self.Cross`) 0 null "None"))
  (`MaterialInstanceDynamic.SetVectorParameterValue` _returnvalue_2 "Color" (`self.Color`)))

(event `StartTimeLine`
  (bind _cross (`self.Cross`))
  (bind (_direction _rotation _position) (`Timeline|TimelineMoveCross` :!label _label)
    (:`Update`
      (`SceneComponent.K2_SetWorldRotation` _cross (`KismetMathLibrary.MakeRotator` 0.0 0.0 _rotation) false false)
      (`SceneComponent.K2_SetRelativeLocation` _cross (`KismetMathLibrary.MakeVector` 0.0 0.0 (+ _position 95.0)) false false))))

(event `StopTimeline`
  (goto _label :!via `Stop`))

(event `self.Capsule.OnComponentBeginOverlap`
  (params (OverlappedComponent :type "PrimitiveComponent Object Reference") (OtherActor :type "Actor Object Reference") (OtherComp :type "PrimitiveComponent Object Reference") (OtherBodyIndex :type Integer) (bFromSweep :type Boolean) (SweepResult :type "HitResult Structure (by ref)"))
  (`GameplayStatics.ApplyDamage` OtherActor (`self.HealAmount`))
  (`self.RemoveHealthPack`))

(fn `RemoveHealthPack`
  (`SceneComponent.SetVisibility` (`self.Cross`) false false)
  (`PrimitiveComponent.SetCollisionEnabled` (`self.Capsule`) "NoCollision")
  (`self.StopTimeline`)
  (`self.StartRecharge`))

(fn `SpawnHealthPack`
  (`KismetSystemLibrary.K2_ClearAndInvalidateTimerHandle` (`self.RechargeTimer`))
  (`KismetSystemLibrary.K2_ClearAndInvalidateTimerHandle` (`self.UpdateTimer`))
  (`SceneComponent.SetVisibility` (`self.Cross`) true false)
  (`PrimitiveComponent.SetCollisionEnabled` (`self.Capsule`) "QueryAndPhysics")
  (`self.StartTimeLine`)
  (`MaterialInstanceDynamic.SetScalarParameterValue` (`self.DynMatClock`) "Percent" 1.0))

(fn `StartRecharge`
  (bind _returnvalue (`KismetSystemLibrary.K2_SetTimer` null "SpawnHealthPack" (`self.RechargeTime`)))
  (set `self.RechargeTimer` _returnvalue)
  (bind _returnvalue_2 (`KismetSystemLibrary.K2_SetTimer` null "UpdateClock" 0.1 true))
  (set `self.UpdateTimer` _returnvalue_2))

(fn `UpdateClock`
  (bind _rechargetimer (`self.RechargeTimer`))
  (bind _returnvalue (`KismetSystemLibrary.K2_GetTimerElapsedTimeHandle` _rechargetimer))
  (`MaterialInstanceDynamic.SetScalarParameterValue` (`self.DynMatClock`) "Percent" (/ _returnvalue (+ _returnvalue (`KismetSystemLibrary.K2_GetTimerRemainingTimeHandle` _rechargetimer)))))

(fn `UserConstructionScript`)