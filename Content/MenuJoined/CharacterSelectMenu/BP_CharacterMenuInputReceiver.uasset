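; Per-controller input receiver for the character select menu, letting a player join or leave, browse, select and deselect characters, and request game start.
; Join, leave, widget creation and level load go through GameMode messages, while selection calls go to the returned character select widget.
; AcceptingControls locks browsing after selection, and a delayed DoOnce reset throttles stick input.
; Button prompts update per state, with a screen-space widget component showing the initial join prompt.
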(event `InputAction|MenuSelect`
  (params (Key :type "Key Structure"))
  (bind _returnvalue (`GameplayStatics.GetGameMode`))
  (bind _controllerid (`self.ControllerID`))
  ;[1 1 1] Display character select / select character
  (:`Pressed`
    (if (`self.AcceptingControls`)
      ;;[1 1 1 1 10] See if CharacterMenuRef has already been created. If not: Create, if Yes: Select
      (bind _characterselectref (`self.CharacterSelectRef`)
        (:`then`
          (if (`Widget.IsVisible` _characterselectref)
            (`/Game/MenuJoined/CharacterSelectMenu/UI/WBP_PlayerSelectSlot.SelectCharacter` _characterselectref)
            (set `self.AcceptingControls` false)
            (`self.RemoveInstructions`)
            (bind _returnvalue_2 (`/Game/MenuJoined/CharacterSelectMenu/UI/WBP_PlayerSelectSlot.AddInstruction` (`self.CharacterSelectRef`) "B" "deselect character"))
            (`KismetArrayLibrary.Array_Add` (`self.InstructionsArray`) _returnvalue_2)
            (else
              (bind _activeindex (message `/Game/MenuJoined/CharacterSelectMenu/BPI_CharacterSelect.JoinGame` _returnvalue _controllerid :!label _label))
              (bind _output_get (set `self.ActivePlayerIndex` _activeindex))
              (bind _selectwidget (message `/Game/MenuJoined/CharacterSelectMenu/BPI_CharacterSelect.DisplayCharacterSelect` _returnvalue _output_get _controllerid))
              (bind _output_get_2 (set `self.CharacterSelectRef` _selectwidget))
              (`self.RemoveInstructions` :!label _label_2)
              (bind _returnvalue_3 (`/Game/MenuJoined/CharacterSelectMenu/UI/WBP_PlayerSelectSlot.AddInstruction` _output_get_2 "A" "select character"))
              (`KismetArrayLibrary.Array_Add` (`self.InstructionsArray`) _returnvalue_3)
              (bind _returnvalue_4 (`/Game/MenuJoined/CharacterSelectMenu/UI/WBP_PlayerSelectSlot.AddInstruction` _output_get_2 "B" "leave game"))
              (`KismetArrayLibrary.Array_Add` (`self.InstructionsArray`) _returnvalue_4))))
        (:`else`
          (goto _label))))))

(event `InputAction|MenuDeselect`
  (params (Key :type "Key Structure"))
  ;[1 1 1] Deselect character
  (:`Pressed`
    (bind _characterselectref (`self.CharacterSelectRef`)
      (:`then`
        (if (`self.AcceptingControls`)
          (`Widget.RemoveFromParent` _characterselectref)
          (`KismetSystemLibrary.CollectGarbage`)
          (message `/Game/MenuJoined/CharacterSelectMenu/BPI_CharacterSelect.LeaveGame` (`GameplayStatics.GetGameMode`) (`self.ControllerID`))
          (else
            (`/Game/MenuJoined/CharacterSelectMenu/UI/WBP_PlayerSelectSlot.DeselectCharacter` _characterselectref 0)
            (set `self.AcceptingControls` true)
            (goto _label_2))))
      (:`else`))))

(event `InputAction|start_game`
  (params (Key :type "Key Structure"))
  (bind _characterselectref (`self.CharacterSelectRef`))
  ;[1 1 1] Start game (Open Level) (happens in GameMode)
  (:`Pressed`
    ;;[1 1 1 1 9] can only start game when opened character select
    (`/Engine/EditorBlueprintResources/StandardMacros.IsValid` _characterselectref
      (:`Is Valid`
        (if (`Widget.IsVisible` _characterselectref)
          (message `/Game/MenuJoined/CharacterSelectMenu/BPI_CharacterSelect.LoadLevel` (`GameplayStatics.GetGameMode`)))))))

(event `InputAction|ArrowRight`
  (params (Key :type "Key Structure"))
  ;[1 1 1] Switch character selection
  (:`Pressed`
    (if (`self.AcceptingControls`) :!label _label_3
      (`/Engine/EditorBlueprintResources/StandardMacros.IsValid` (`self.CharacterSelectRef`)
        (:`Is Valid`
          (`/Game/MenuJoined/CharacterSelectMenu/UI/WBP_PlayerSelectSlot.SwitchCharacter` (`self.CharacterSelectRef`) 1)
          (`KismetSystemLibrary.Delay` 0.2 :!label _label_4)
          (`self.ResetDoOnce`))))))

(event `InputAxis|MoveRight`
  (params (AxisValue :type "Float (single-precision)"))
  ;[1 1 1] Switch character selection
  (if (> (`KismetMathLibrary.Abs` AxisValue) 0.8)
    (`/Engine/EditorBlueprintResources/StandardMacros.DoOnce` false :!label _label_5
      (:`Completed`
        (if (> AxisValue 0.0)
          (goto _label_3)
          (else
            (if (`self.AcceptingControls`) :!label _label_6
              (`/Engine/EditorBlueprintResources/StandardMacros.IsValid` (`self.CharacterSelectRef`)
                (:`Is Valid`
                  (`/Game/MenuJoined/CharacterSelectMenu/UI/WBP_PlayerSelectSlot.SwitchCharacter` (`self.CharacterSelectRef`) -1)
                  (goto _label_4))))))))))

(event `ResetDoOnce`
  ;[1 1 1] Switch character selection
  (goto _label_5 :!via `Reset`))

(event `InputAction|ArrowLeft`
  (params (Key :type "Key Structure"))
  ;[1 1 1] Switch character selection
  (:`Pressed`
    (goto _label_6)))

(event `self.ReceiveBeginPlay`
  ;[0.9999 0.5165 1] Make controller ID visible (debugging)
  (`TextRenderComponent.K2_SetText` (`self.Text`) (`|FormatText` "ControllerID: {id}" (`self.ControllerID`)))
  (`self.ShowJoinGame`))

(fn `AddInstructionOutsideSelect`
  (params (Button :type String) (Instruction :type Text))
  (returns (OutputPin :type "WidgetComponent Object Reference"))
  (bind _returnvalue (`|CreateWidget` "/Game/MenuJoined/CharacterSelectMenu/UI/WBP_ButtonInstruction.WBP_ButtonInstruction_C" null Button Instruction))
  (`/Engine/EditorBlueprintResources/StandardMacros.IsValid` _returnvalue
    (:`Is Valid`
      (bind _returnvalue_2 (`AddComponent|NODE_AddWidgetComponent-0` :`RelativeTransform` (`KismetMathLibrary.MakeTransform` (0.0 0.0 100.0))))
      (`/Engine/EditorBlueprintResources/StandardMacros.IsValid` _returnvalue_2
        (:`Is Valid`
          (`WidgetComponent.SetDrawAtDesiredSize` _returnvalue_2 true)
          (`WidgetComponent.SetWidgetSpace` _returnvalue_2 "Screen")
          (`WidgetComponent.SetWidget` _returnvalue_2 _returnvalue)
          (return _returnvalue_2))))))

(fn `HideJoinGame`
  (for _array_element (`self.JoinGameInstruction`)
    (`ActorComponent.K2_DestroyComponent` _array_element))
  (`KismetArrayLibrary.Array_Clear` (`self.JoinGameInstruction`)))

(fn `RemoveInstructions`
  (for _array_element (`self.InstructionsArray`)
    (`/Engine/EditorBlueprintResources/StandardMacros.IsValid` _array_element
      (:`Is Valid`
        (`Widget.RemoveFromParent` _array_element))))
  (`KismetArrayLibrary.Array_Clear` (`self.InstructionsArray`)))

(fn `ShowJoinGame`
  (bind _outputpin (`self.AddInstructionOutsideSelect` "A" "join game"))
  (`KismetArrayLibrary.Array_Add` (`self.JoinGameInstruction`) _outputpin))

(fn `UserConstructionScript`)