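; Game mode for the local multiplayer character select menu, handling player join, leave and lock-in before loading the arena map.
; On BeginPlay it sorts BP_CustomStart actors by index, creates a local player and possessed input receiver at each, then shows the menu widget.
; Joiners get the first free slot index, stored with lock states in GameInstance maps.
; Start prompt and level load require every joined player locked.
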(event `self.ReceiveBeginPlay`
  (`self.OrganizeCustomStartArray`)
  (`self.SpawnMenuInputReceivers`)
  (bind _returnvalue (`|CreateWidget` "/Game/MenuJoined/CharacterSelectMenu/UI/WBP_Menu.WBP_Menu_C"))
  (bind _output_get (set `self.MenuWidgetRef` _returnvalue))
  (`UserWidget.AddToViewport` _output_get 0))

(event `/Game/MenuJoined/CharacterSelectMenu/BPI_CharacterSelect.LoadLevel`
  ;[1 1 1] Start level by request (if everyone is locked)
  (bind _values (`BlueprintMapLibrary.Map_Values` (`/Game/BP_GameInstance.MapLockedPlayers` (cast `/Game/BP_GameInstance` (`GameplayStatics.GetGameInstance`) :!pure true))))
  (if (not (`KismetArrayLibrary.Array_Contains` _values))
    (`GameplayStatics.OpenLevel` "Map_AsiaArena")))

(fn `AllTrue`
  (params (BooleanArray :type "Array of Boolean"))
  (returns (AllTrue :type Boolean))
  (locals (FoundFalse :type Boolean))
  (for _array_element BooleanArray
    (if (not _array_element)
      (set `local.FoundFalse` true)))
  (return (not (`local.FoundFalse`))))

(fn `CheckAllLocked`
  (bind _values (`BlueprintMapLibrary.Map_Values` (`/Game/BP_GameInstance.MapLockedPlayers` (cast `/Game/BP_GameInstance` (`GameplayStatics.GetGameInstance`) :!pure true))))
  (`self.ShowStartGame` (not (`KismetArrayLibrary.Array_Contains` _values))))

(fn `DisplayCharacterSelect`
  (params (CurrentPlayerIndex :type Integer) (ControllerID :type Integer))
  (returns (SelectWidget :type "/Game/MenuJoined/CharacterSelectMenu/UI/WBP_PlayerSelectSlot Object Reference"))
  (bind _characterselect (`/Game/MenuJoined/CharacterSelectMenu/UI/WBP_Menu.AddCharacterSelect` (`self.MenuWidgetRef`) CurrentPlayerIndex ControllerID (`self.SelectableCharacters`) (`self.CustomStartArray`)))
  (return _characterselect))

(fn `FirstAvailableIndex`
  (params (Indices :type "Array of Integer"))
  (returns (Available :type Integer))
  (locals (iterator :type Integer))
  (bind _iterator (`local.iterator`))
  (while (and (`KismetArrayLibrary.Array_Contains` (`local.Indices`) _iterator) (< _iterator (`KismetArrayLibrary.Array_Length` (`self.CustomStartArray`))))
    (`/Engine/EditorBlueprintResources/StandardMacros.IncrementInt` (`local.iterator`)))
  (return (`local.iterator`)))

(fn `HideJoinGameAtIndex`
  (params (PlayerIndex :type Integer))
  (`/Game/MenuJoined/CharacterSelectMenu/BP_CharacterMenuInputReceiver.HideJoinGame` (`|GetArrayItem` (`self.InputRecieverArray`) PlayerIndex)))

(fn `JoinGame`
  (params (PlayerControllerID :type Integer))
  (returns (ActiveIndex :type Integer))
  (bind _asbp_game_instance (cast `/Game/BP_GameInstance` (`GameplayStatics.GetGameInstance`) :!pure true))
  (bind _mapplayerindex (`/Game/BP_GameInstance.MapPlayerIndex` _asbp_game_instance))
  (`BlueprintMapLibrary.Map_Add` (`/Game/BP_GameInstance.MapLockedPlayers` _asbp_game_instance) PlayerControllerID)
  (bind _values (`BlueprintMapLibrary.Map_Values` _mapplayerindex))
  (bind _available (`self.FirstAvailableIndex` _values))
  (`BlueprintMapLibrary.Map_Add` _mapplayerindex PlayerControllerID _available)
  (return _available))

(fn `LeaveGame`
  (params (ControllerID :type Integer))
  (returns (Dummy :type Boolean))
  (bind _asbp_game_instance (cast `/Game/BP_GameInstance` (`GameplayStatics.GetGameInstance`) :!pure true))
  (`BlueprintMapLibrary.Map_Remove` (`/Game/BP_GameInstance.MapLockedPlayers` _asbp_game_instance) ControllerID)
  (`BlueprintMapLibrary.Map_Remove` (`/Game/BP_GameInstance.MapPlayerIndex` _asbp_game_instance) ControllerID)
  (return false))

(fn `NameToInt`
  (params (PlayerStart :type "PlayerStart Object Reference"))
  (returns (ReturnValue :type Integer))
  (return (`KismetStringLibrary.Conv_StringToInt` (`KismetStringLibrary.Conv_NameToString` (`PlayerStart.PlayerStartTag` PlayerStart)))))

(fn `OrganizeCustomStartArray`
  (locals (EmptyArray :type "Array of /Game/MenuJoined/CharacterSelectMenu/BP_CustomStart Object Reference"))
  (bind _outactors (`GameplayStatics.GetAllActorsOfClass` "/Game/MenuJoined/CharacterSelectMenu/BP_CustomStart.BP_CustomStart_C"))
  (for _array_element _outactors
    (`KismetArrayLibrary.Array_Set` (`local.EmptyArray`) (`/Game/MenuJoined/CharacterSelectMenu/BP_CustomStart.Index` _array_element) _array_element true)
    (set `self.CustomStartArray` (`local.EmptyArray`))))

(fn `ShowJoinGameAtIndex`
  (params (PlayerIndex :type Integer))
  (`/Game/MenuJoined/CharacterSelectMenu/BP_CharacterMenuInputReceiver.ShowJoinGame` (`|GetArrayItem` (`self.InputRecieverArray`) PlayerIndex)))

(fn `ShowStartGame`
  (params (Show :type Boolean))
  (`/Game/MenuJoined/CharacterSelectMenu/UI/WBP_Menu.ShowStartGame` (`self.MenuWidgetRef`) Show))

(fn `SpawnMenuInputReceivers`
  (for (_array_element _array_index) (`self.CustomStartArray`)
    (`GameplayStatics.CreatePlayer` _array_index)
    (bind _returnvalue (`|SpawnActorFromClass` "/Game/MenuJoined/CharacterSelectMenu/BP_CharacterMenuInputReceiver.BP_CharacterMenuInputReceiver_C" (`self.GetTransform` _array_element) "Undefined" "OverrideRootScale" null _array_index _array_index null))
    (`KismetArrayLibrary.Array_AddUnique` (`self.InputRecieverArray`) _returnvalue)
    (`Controller.Possess` (`GameplayStatics.GetPlayerController` _array_index) _returnvalue)))

(fn `UserConstructionScript`)