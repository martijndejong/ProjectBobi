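; BP_BobiLogo is an animated Bobi logo actor for the joined menu, with rotating blades (Wieken) and a rect light.
; On BeginPlay, the SetAlpha timeline drives an Alpha value.
; Each tick, Alpha scales both the blades' pitch rotation speed and the light's intensity, so spin and glow follow the same curve.
; The pitch accumulates from the current world rotation and wraps at 90 degrees, with yaw held fixed.
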(event `self.ReceiveBeginPlay`
  (bind (_direction _newtrack_0) (`Timeline|SetAlpha` :!via `PlayFromStart`)
    (:`Update`
      (set `self.Alpha` _newtrack_0))))

(event `self.ReceiveTick`
  (params (DeltaSeconds :type "Float (single-precision)"))
  (bind _wieken (`self.Wieken`))
  (bind (_returnvalue_roll _returnvalue_pitch) (`KismetMathLibrary.BreakRotator` (`SceneComponent.K2_GetComponentRotation` _wieken)))
  (`SceneComponent.K2_SetWorldRotation` _wieken (`KismetMathLibrary.MakeRotator` 0.0 (mod (+ (* (* (`self.DegPerSec`) (`self.Alpha`)) DeltaSeconds) _returnvalue_pitch) 90.0) 180.0) false false)
  (`LightComponent.SetIntensity` (`self.RectLight`) (* (`self.Alpha`) 5000.0)))

(fn `UserConstructionScript`)