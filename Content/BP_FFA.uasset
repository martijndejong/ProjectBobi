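; Free-for-all GameMode for local multiplayer that spawns each locked-in player's chosen character and starts the match on a shared camera.
; On BeginPlay it creates the HUD container, finds BP_camera, orders BP_CustomStart actors by index and copies character and player maps from BP_GameInstance.
; Each player spawns at their indexed start, is possessed and views the shared camera; stray CameraActors are destroyed.
; After a short delay the camera is told the game started.
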(event `self.ReceiveBeginPlay`
  ;[1 1 1] Setting up / Starting game (we moeten dit als Parent GameMode houden, en dan children met eigen regels qua respawn en punten etc.)
  ;;[1 1 1] Create container for player HUDs
  (bind _returnvalue (`|CreateWidget` "/Game/HUD/HUD_Container.HUD_Container_C"))
  (bind _output_get (set `self.HUDContainerRef` _returnvalue))
  (`UserWidget.AddToViewport` _output_get 0)
  ;;[1 1 1] Set reference to Camera
  (bind _outactors (`GameplayStatics.GetAllActorsOfClass` "/Game/BP_camera.BP_camera_C"))
  (bind _output_get_2 (set `self.CameraRef` (`|GetArrayItem` _outactors)))
  (`PlayerController.SetViewTargetWithBlend` (`GameplayStatics.GetPlayerController` 0) _output_get_2 0.0 "VTBlend_Linear" 0.0 false)
  ;;[1 1 1] Populate PlayerStartArray
  (`self.OrganizeCustomStartArray`)
  ;;[1 1 1 1 16] Pull selected characters/Active controllers/Locked Players from GameInstance to GameMode and store
  (bind _asbp_game_instance (cast `/Game/BP_GameInstance` (`GameplayStatics.GetGameInstance`)))
  (set `self.GM_MapSelectedCharacters` (`/Game/BP_GameInstance.MapSelectedCharacters` _asbp_game_instance))
  (set `self.GM_MapPlayerIndex` (`/Game/BP_GameInstance.MapPlayerIndex` _asbp_game_instance))
  (set `self.GM_MapLockedPlayers` (`/Game/BP_GameInstance.MapLockedPlayers` _asbp_game_instance))
  ;;[1 1 1] Spawn all locked players, and then start game
  (bind _keys (`BlueprintMapLibrary.Map_Keys` (`self.GM_MapPlayerIndex`)))
  (for _array_element _keys
    (`self.SpawnPlayer` _array_element))
  (`KismetSystemLibrary.Delay` 2.0)
  (`self.StartGame`))

(event `/Game/BPI_gamemode.RequestSpawnPlayer`
  (params (ControllerID :type Integer))
  ;[1 1 1] Spawn logic here
  (`self.SpawnPlayer` ControllerID))

(fn `DisplayPlayerHUD`
  (params (PlayerController :type "PlayerController Object Reference") (PlayerIndex :type Integer))
  (returns (PlayerHUD :type "/Game/HUD/HUD_Player Object Reference"))
  (bind _playerhud (`/Game/HUD/HUD_Container.AddPlayerHUD` (`self.HUDContainerRef`) PlayerController PlayerIndex))
  (return _playerhud))

(fn `NameToInt`
  (params (self2 :type "PlayerStart Object Reference"))
  (returns (ReturnValue :type Integer))
  (return (`KismetStringLibrary.Conv_StringToInt` (`KismetStringLibrary.Conv_NameToString` (`PlayerStart.PlayerStartTag` self2)))))

(fn `OrganizeCustomStartArray`
  (locals (EmptyArray :type "Array of /Game/CharacterSelectMenu/BP_CustomStart Object Reference"))
  (bind _outactors (`GameplayStatics.GetAllActorsOfClass` "/Game/CharacterSelectMenu/BP_CustomStart.BP_CustomStart_C"))
  (for _array_element _outactors
    (`KismetArrayLibrary.Array_Set` (`local.EmptyArray`) (`/Game/CharacterSelectMenu/BP_CustomStart.Index` _array_element) _array_element true)
    (set `self.CustomStartArray` (`local.EmptyArray`))))

(fn `RemindCamera`
  (params (Controller :type "PlayerController Object Reference"))
  (returns (Dummy :type Boolean))
  (`PlayerController.SetViewTargetWithBlend` Controller (`self.CameraRef`) 0.0 "VTBlend_Linear" 0.0 false)
  (return false))

(fn `RemoveUnusedCameras`
  (bind _outactors (`GameplayStatics.GetAllActorsOfClass` "/Script/Engine.CameraActor"))
  (for _array_element _outactors
    (`self.K2_DestroyActor` _array_element)))

(fn `SpawnPlayer`
  (params (PlayerControllerID :type Integer))
  (bind _returnvalue (`|SpawnActorFromClass` (`BlueprintMapLibrary.Map_Find` (`self.GM_MapSelectedCharacters`) PlayerControllerID) (`self.GetTransform` (`|GetArrayItem` (`self.CustomStartArray`) (`BlueprintMapLibrary.Map_Find` (`self.GM_MapPlayerIndex`) PlayerControllerID))) "Undefined" "OverrideRootScale" null PlayerControllerID (`GameplayStatics.GetPlayerController` PlayerControllerID) null))
  (`Controller.Possess` (`GameplayStatics.GetPlayerController` (`local.PlayerControllerID`)) _returnvalue)
  (`PlayerController.SetViewTargetWithBlend` (`GameplayStatics.GetPlayerController` (`local.PlayerControllerID`)) (`self.CameraRef`) 0.0 "VTBlend_Linear" 0.0 false)
  (`self.RemoveUnusedCameras`))

(fn `StartGame`
  (`/Game/BP_camera.GameStarted` (`self.CameraRef`)))

(fn `UserConstructionScript`)