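; BP_CharacterMenuInputReceiver turns one player's input into character select menu actions, identified by its Index.
; The first select press asks the GameMode to display character select; later presses lock in a character on CharacterMenuRef.
; Arrows switch characters while AcceptingControls is true, which selecting clears and deselecting restores.
; The start input asks the GameMode to load the level, regardless of selection state.
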(event `InputAction|MenuSelect`
  (params (Key :type "Key Structure"))
  ;[1 1 1] Display character select / select character
  (:`Pressed`
    (if (`self.AcceptingControls`)
      ;;[1 1 1 1 10] See if CharacterMenuRef has already been created. If not: Create, if Yes: Select
      (bind _charactermenuref (`self.CharacterMenuRef`)
        (:`then`
          (`/Game/CharacterSelectMenu/UI/WBP_PlayerSelectSlot.SelectCharacter` _charactermenuref)
          (set `self.AcceptingControls` false))
        (:`else`
          (message `/Game/CharacterSelectMenu/BPI_CharacterSelect.DisplayCharacterSelect` (`GameplayStatics.GetGameMode`) (`self.Index`)))))))

(event `InputAction|MenuDeselect`
  (params (Key :type "Key Structure"))
  ;[1 1 1] Deselect character
  (:`Pressed`
    (bind _charactermenuref (`self.CharacterMenuRef`)
      (:`then`
        (`/Game/CharacterSelectMenu/UI/WBP_PlayerSelectSlot.DeselectCharacter` _charactermenuref)
        (set `self.AcceptingControls` true))
      (:`else`))))

(event `InputAction|start_game`
  (params (Key :type "Key Structure"))
  ;[1 1 1] Start game (Open Level) (happens in GameMode)
  (:`Pressed`
    (message `/Game/CharacterSelectMenu/BPI_CharacterSelect.LoadLevel` (`GameplayStatics.GetGameMode`))))

(event `InputAction|ArrowLeft`
  (params (Key :type "Key Structure"))
  ;[1 1 1] Switch character selection
  (:`Pressed`
    (if (`self.AcceptingControls`)
      (`/Engine/EditorBlueprintResources/StandardMacros.IsValid` (`self.CharacterMenuRef`)
        (:`Is Valid`
          (`/Game/CharacterSelectMenu/UI/WBP_PlayerSelectSlot.SwitchCharacter` (`self.CharacterMenuRef`) -1))))))

(event `InputAction|ArrowRight`
  (params (Key :type "Key Structure"))
  ;[1 1 1] Switch character selection
  (:`Pressed`
    (if (`self.AcceptingControls`)
      (`/Engine/EditorBlueprintResources/StandardMacros.IsValid` (`self.CharacterMenuRef`)
        (:`Is Valid`
          (`/Game/CharacterSelectMenu/UI/WBP_PlayerSelectSlot.SwitchCharacter` (`self.CharacterMenuRef`) 1))))))

(fn `UserConstructionScript`)