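; Game mode for a local multiplayer character select menu that creates players and loads the level once characters are locked.
; On BeginPlay it creates a player and possessed input receiver for each PlayerStart index matched by an integer tag, then shows the menu widget.
; DisplayCharacterSelect adds a player's selection panel and links it to their receiver.
; LoadLevel requires a locked player in the GameInstance, removes unlocked players, then opens EmptyLevel.
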(event `self.ReceiveBeginPlay`
  (bind _outactors (`GameplayStatics.GetAllActorsOfClass` "/Script/Engine.PlayerStart"))
  (set `self.PlayerStartArray` _outactors)
  (`self.SpawnMenuInputReceivers`)
  (bind _returnvalue (`|CreateWidget` "/Game/CharacterSelectMenu/UI/WBP_Menu.WBP_Menu_C"))
  (bind _output_get (set `self.MenuWidgetRef` _returnvalue))
  (`UserWidget.AddToViewport` _output_get 0))

(event `/Game/CharacterSelectMenu/BPI_CharacterSelect.LoadLevel`
  (bind _lockedplayers (`/Game/BP_GameInstance.LockedPlayers` (cast `/Game/BP_GameInstance` (`GameplayStatics.GetGameInstance`) :!pure true)))
  ;[1 1 1] Check minimum amount of players
  (bind _number (`self.NumberOfTrue` _lockedplayers))
  (if (>= _number 1)
    ;[1 1 1] Remove Players who did not Lock character
    (for (_array_element _array_index) _lockedplayers
      (if (not _array_element)
        (`GameplayStatics.RemovePlayer` (`GameplayStatics.GetPlayerController` _array_index))))
    (`GameplayStatics.OpenLevel` "EmptyLevel")))

(fn `DisplayCharacterSelect`
  (params (CurrentPlayerIndex :type Integer))
  (returns (Return :type Boolean))
  (bind _characterselect (`/Game/CharacterSelectMenu/UI/WBP_Menu.AddCharacterSelect` (`self.MenuWidgetRef`) CurrentPlayerIndex (`self.SelectableCharacters`)))
  ;[1 1 1 1 12] Deze variable zit in de input receiver, wordt hier geset
  (set `/Game/CharacterSelectMenu/BP_CharacterMenuInputReceiver.CharacterMenuRef` _characterselect (`|GetArrayItem` (`self.InputRecieverArray`) (`local.CurrentPlayerIndex`)))
  (return false))

(fn `NameToInt`
  (params (PlayerStart :type "PlayerStart Object Reference"))
  (returns (ReturnValue :type Integer))
  (return (`KismetStringLibrary.Conv_StringToInt` (`KismetStringLibrary.Conv_NameToString` (`PlayerStart.PlayerStartTag` PlayerStart)))))

(fn `NumberOfTrue`
  (params (BoolArray :type "Array of Boolean"))
  (returns (Number :type Integer))
  (locals (Counter :type Integer :default 0))
  (for _array_element BoolArray
    (set `local.Counter` (+ (`KismetMathLibrary.Conv_BoolToInt` _array_element) (`local.Counter`))))
  (return (`local.Counter`)))

(fn `SpawnMenuInputReceivers`
  (for (_ _array_index) (`self.PlayerStartArray`)
    (set `self.Index` _array_index)
    (for _array_element (`self.PlayerStartArray`)
      (if (== (`self.NameToInt` _array_element) (`self.Index`))
        (`GameplayStatics.CreatePlayer` (`self.Index`))
        (bind _returnvalue (`|SpawnActorFromClass` "/Game/CharacterSelectMenu/BP_CharacterMenuInputReceiver.BP_CharacterMenuInputReceiver_C" (`self.GetTransform` (`|GetArrayItem` (`self.PlayerStartArray`) (`self.Index`))) "Undefined" "OverrideRootScale" null (`self.Index`) null))
        (`KismetArrayLibrary.Array_AddUnique` (`self.InputRecieverArray`) _returnvalue)
        (`Controller.Possess` (`GameplayStatics.GetPlayerController` (`self.Index`)) _returnvalue)))))

(fn `UserConstructionScript`)