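; Player-colored ghost that exists for a respawn countdown, then asks the game mode to respawn its player at the ghost's transform.
; BeginPlay tints the mesh, poof effect and ground cast circle, then starts the timer that destroys the actor.
; A looping timer animates the circle's material radii as countdown progress.
; Tick sphere-traces downward and snaps the ghost above the ground when it is too high.
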(event `self.ReceiveBeginPlay`
  (bind _returnvalue (`NiagaraFunctionLibrary.SpawnSystemAtLocation` "/Game/Bobi/BobiGhost/P_GhostPoof.P_GhostPoof" (`self.K2_GetActorLocation`)))
  (`NiagaraComponent.SetVariableLinearColor` _returnvalue "PlayerColor" (`self.PlayerColor`))
  (`SceneComponent.SetVisibility` (`/Game/LocationCone/BP_LocationCone.CastCircle` (`self.LocationCone`)) true false)
  (bind _returnvalue_2 (`PrimitiveComponent.CreateDynamicMaterialInstance` (`self.Mesh`) 0 null "None"))
  (`MaterialInstanceDynamic.SetVectorParameterValue` _returnvalue_2 "PlayerColor" (`self.PlayerColor`))
  (bind _returnvalue_3 (`PrimitiveComponent.CreateDynamicMaterialInstance` (`/Game/LocationCone/BP_LocationCone.CastCircle` (`self.LocationCone`)) 0 null "None"))
  (bind _output_get (set `self.CastCircleMaterial` _returnvalue_3))
  (`MaterialInstanceDynamic.SetVectorParameterValue` _output_get "Color" (`self.PlayerColor`))
  (`KismetSystemLibrary.Delay` 0.2)
  (`SceneComponent.SetVisibility` (`self.Mesh`) true false)
  (bind _returnvalue_4 (`KismetSystemLibrary.K2_SetTimerDelegate` (delegate `DestroyActor`) (`self.RespawnTime`)))
  (set `self.TimeTillRespawn` _returnvalue_4)
  (`KismetSystemLibrary.K2_SetTimerDelegate` (delegate `UpdateCastCircle`) 0.01 true))

(event `DestroyActor`
  (`self.K2_DestroyActor`))

(event `UpdateCastCircle`
  (bind _castcirclematerial (`self.CastCircleMaterial`))
  (bind _returnvalue (/ (`KismetSystemLibrary.K2_GetTimerElapsedTimeHandle` (`self.TimeTillRespawn`)) (`self.RespawnTime`)))
  (`MaterialInstanceDynamic.SetScalarParameterValue` _castcirclematerial "InnerBaseRadius" (`KismetMathLibrary.MapRangeClamped` _returnvalue 0.0 0.95 0.0 0.5))
  (`MaterialInstanceDynamic.SetScalarParameterValue` _castcirclematerial "InnerSubtractionRadius" (`KismetMathLibrary.MapRangeClamped` _returnvalue 0.85 1.0 0.0 0.6)))

(event `self.ReceiveDestroyed`
  (bind _returnvalue (`NiagaraFunctionLibrary.SpawnSystemAtLocation` "/Game/Bobi/BobiGhost/P_GhostPoof.P_GhostPoof" (`self.K2_GetActorLocation`)))
  (`NiagaraComponent.SetVariableLinearColor` _returnvalue "PlayerColor" (`self.PlayerColor`))
  (bind _asbp_game_mode_parent (cast `/Game/GameMode/BP_GameMode_Parent` (`GameplayStatics.GetGameMode`)))
  (`/Game/GameMode/BP_GameMode_Parent.SpawnPlayer` _asbp_game_mode_parent (`self.ControllerID`) (`self.GetTransform`) false false false))

(event `self.ReceiveTick`
  (params (DeltaSeconds :type "Float (single-precision)"))
  (bind _returnvalue (`self.K2_GetActorLocation`))
  (bind (_outhit _returnvalue_2) (`KismetSystemLibrary.SphereTraceSingleForObjects` (+ _returnvalue (0.0 0.0 100.0)) (- _returnvalue (0.0 0.0 5000.0)) (`CapsuleComponent.CapsuleRadius` (`self.CapsuleComponent`)) (`|MakeArray` "ObjectTypeQuery1" :!type "EObjectTypeQuery Enum")))
  (if _returnvalue_2
    (if (> (`.Distance` (`GameplayStatics.BreakHitResult` _outhit)) 200.0)
      (`self.K2_SetActorLocation` (+ (`.ImpactPoint` (`GameplayStatics.BreakHitResult` _outhit)) (`KismetMathLibrary.MakeVector` 0.0 0.0 (+ 25.0 (`CapsuleComponent.CapsuleHalfHeight` (`self.CapsuleComponent`)))))))))

(fn `UserConstructionScript`)