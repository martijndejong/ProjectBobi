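; Actor component that shows icon speech bubbles (sword, shield or heart) as particle effects beside its owner.
; The ArrowRight, ArrowLeft and ArrowUp events each spawn their matching system, but only while no active bubble is valid.
; Tick moves the active bubble to a fixed world-space offset from the owner's location, so it follows the actor.
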(event `self.ReceiveTick`
  (params (DeltaSeconds :type "Float (single-precision)"))
  (bind _activespeechbubble (`self.ActiveSpeechBubble`)
    (:`then`
      (`SceneComponent.K2_SetWorldLocation` _activespeechbubble (+ (`Actor.K2_GetActorLocation` (`self.GetOwner`)) (0.0 100.0 150.0)) true true))
    (:`else`)))

(event `ArrowRight`
  (if (not (`KismetSystemLibrary.IsValid` (`self.ActiveSpeechBubble`)))
    (bind _returnvalue (`NiagaraFunctionLibrary.SpawnSystemAtLocation` "/Game/Bobi/SpeechBubble/P_SpeechBubbleSword.P_SpeechBubbleSword"))
    (set `self.ActiveSpeechBubble` _returnvalue)))

(event `ArrowLeft`
  (if (not (`KismetSystemLibrary.IsValid` (`self.ActiveSpeechBubble`)))
    (bind _returnvalue (`NiagaraFunctionLibrary.SpawnSystemAtLocation` "/Game/Bobi/SpeechBubble/P_SpeechBubbleShield.P_SpeechBubbleShield"))
    (set `self.ActiveSpeechBubble` _returnvalue)))

(event `ArrowUp`
  (if (not (`KismetSystemLibrary.IsValid` (`self.ActiveSpeechBubble`)))
    (bind _returnvalue (`NiagaraFunctionLibrary.SpawnSystemAtLocation` "/Game/Bobi/SpeechBubble/P_SpeechBubbleHeart.P_SpeechBubbleHeart"))
    (set `self.ActiveSpeechBubble` _returnvalue)))