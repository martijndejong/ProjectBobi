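; BP_CameraParent is a shared multiplayer-style camera that keeps all living BobiCharacter actors in view once the game starts.
; Each tick it moves a sphere toward the characters' average location and finds the largest pairwise distance between them.
; That distance, mapped through an ease-out curve, drives the spring arm's length and vertical socket offset, zooming out as characters spread apart.
; Position and zoom are smoothed with per-frame lerps, not scaled by delta time.
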(event `self.ReceiveBeginPlay`
  (set `SpringArmComponent.TargetArmLength` (`self.MaxArmLength`) (`self.SpringArm`)))

(event `self.ReceiveTick`
  (params (DeltaSeconds :type "Float (single-precision)"))
  (bind _springarm (`self.SpringArm`))
  (bind _springarm_2 (`self.SpringArm`))
  (bind (_socketoffset_x _socketoffset_y _socketoffset_z) (`KismetMathLibrary.BreakVector` (`SpringArmComponent.SocketOffset` _springarm)))
  (bind _returnvalue (`KismetMathLibrary.MapRangeClamped` (`.MaxValue` (`KismetMathLibrary.MaxOfFloatArray` (`self.Distance`))) (`self.MinAdaptDistance`) (`self.MaxAdaptDistance`) 0.0 1.0))
  (set `self.CurrentArmLength` (`SpringArmComponent.TargetArmLength` _springarm))
  (set `self.CurrentOffset` _socketoffset_z)
  (bind _outactors (`GameplayStatics.GetAllActorsOfClass` "/Game/Bobi/BobiCharacter.BobiCharacter_C"))
  (set `self.CharactersAlive` _outactors)
  (if (`self.bGameStarted`)
    (`self.CameraMovement`)
    (for (_array_element _array_index) (`self.CharactersAlive`)
      (set `self.CurrentCharacter` _array_element)
      (for _index (range (+ _array_index 1) (`KismetArrayLibrary.Array_Length` (`self.CharactersAlive`)))
        (`KismetArrayLibrary.Array_Add` (`self.Distance`) (`self.GetDistanceTo` (`self.CurrentCharacter`) (`|GetArrayItem` (`self.CharactersAlive`) _index)))))
    (set `self.DesiredArmLength` (`|EaseFunction` "EaseOut" _returnvalue (`self.MinArmLength`) (`self.MaxArmLength`) (`self.ZoomPower`)))
    (set `self.DesiredOffset` (`|EaseFunction` "EaseOut" _returnvalue (`self.MinOffset`) (`self.MaxOffset`) (`self.ZoomPower`)))
    (`KismetArrayLibrary.Array_Clear` (`self.Distance`))
    (set `SpringArmComponent.TargetArmLength` (`KismetMathLibrary.Lerp` (`self.CurrentArmLength`) (`self.DesiredArmLength`) (/ (`self.CameraMoveSpeed`) 2.0)) _springarm_2)
    (set `SpringArmComponent.SocketOffset` (`KismetMathLibrary.MakeVector` 0.0 0.0 (`KismetMathLibrary.Lerp` (`self.CurrentOffset`) (`self.DesiredOffset`) (/ (`self.CameraMoveSpeed`) 2.0))) _springarm_2)))

(fn `CameraMovement`
  (set `self.PreviouseLocation` (`SceneComponent.K2_GetComponentLocation` (`self.Sphere`)))
  (bind _returnvalue (`GameplayStatics.GetActorArrayAverageLocation` (`self.CharactersAlive`)))
  (`SceneComponent.K2_SetWorldLocation` (`self.Sphere`) (`KismetMathLibrary.VLerp` (`self.PreviouseLocation`) _returnvalue (`self.CameraMoveSpeed`)) false false))

(fn `GameStarted`
  (set `self.bGameStarted` true))

(fn `UserConstructionScript`)