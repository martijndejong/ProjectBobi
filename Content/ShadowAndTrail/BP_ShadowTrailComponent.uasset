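; BP_ShadowTrailComponent is a component that gives its owning character or ability a player-colored shadow trail.
; On BeginPlay it takes the color from a BobiCharacter owner, or from the ability owner of a BP_AbilityParent, and does nothing for other owners.
; It then spawns a BP_ShadowTrail at the owner's transform, owned by that actor, passing along the color and its height and Z-offset settings.
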(event `self.ReceiveBeginPlay`
  (bind _returnvalue (`self.GetOwner`))
  (bind _returnvalue_2 (`self.GetOwner`))
  (bind _asbobi_character (cast `/Game/Bobi/BobiCharacter` _returnvalue_2)
    (:`then`
      (set `self.Color` (`/Game/Bobi/BobiCharacter.PlayerColor` _asbobi_character)))
    (:`CastFailed`
      (bind _asbp_ability_parent (cast `/Game/AbilitySystem/BP_AbilityParent` _returnvalue_2))
      (set `self.Color` (`/Game/Bobi/BobiCharacter.PlayerColor` (`/Game/AbilitySystem/BP_AbilityParent.AbilityOwner` _asbp_ability_parent)))))
  (`|SpawnActorFromClass` "/Game/ShadowAndTrail/BP_ShadowTrail.BP_ShadowTrail_C" (`Actor.GetTransform` _returnvalue) "Undefined" "OverrideRootScale" _returnvalue (`self.Color`) (`self.Min Height`) (`self.Max Height`) (`self.TrailDeltaLocationZ`) null))