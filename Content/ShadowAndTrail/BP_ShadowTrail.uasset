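; BP_ShadowTrail is a height-reactive shadow decal and Niagara trail, tinted with PlayerColor, that attaches to its owner and is destroyed with it.
; Each tick it zeroes rotation and traces down against WorldStatic, showing both effects when above MinHeight or nothing is hit.
; A dynamic decal material shrinks radius and raises density with height.
; Near the ground both effects turn off, unless the owner's class is exactly BP_AbilityParent.
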(event `self.ReceiveBeginPlay`
  (bind _niagaratrail (`self.NiagaraTrail`))
  (bind _playercolor (`self.PlayerColor`))
  (`self.K2_AttachToActor` (`self.GetOwner`) "None" "SnapToTarget" "SnapToTarget" "SnapToTarget")
  (bind _returnvalue (`DecalComponent.CreateDynamicMaterialInstance` (`self.Decal`)))
  (bind _output_get (set `self.DynamicMaterial` _returnvalue))
  (`MaterialInstanceDynamic.SetVectorParameterValue` _output_get "PlayerColor" _playercolor)
  (`NiagaraComponent.SetVariableLinearColor` _niagaratrail "TrailColor" _playercolor)
  (`SceneComponent.K2_AddWorldOffset` _niagaratrail (`KismetMathLibrary.MakeVector` 0.0 0.0 (`self.Delta Location Z`)) false true)
  (add `self.OnDestroyed` (`self.GetOwner`) (delegate `DestroyDecal`)))

(event `DestroyDecal` :!signature `self.OnDestroyed`
  (params (DestroyedActor :type "Actor Object Reference"))
  (`self.K2_DestroyActor`))

(event `self.ReceiveTick`
  (params (DeltaSeconds :type "Float (single-precision)"))
  (bind _returnvalue (`self.K2_GetActorLocation`))
  (bind _decal (`self.Decal`))
  (bind _niagaratrail (`self.NiagaraTrail`))
  (bind _dynamicmaterial (`self.DynamicMaterial`))
  (`self.K2_SetActorRotation` (struct))
  (bind (_outhit _returnvalue_2) (`KismetSystemLibrary.LineTraceSingleForObjects` _returnvalue (- _returnvalue (0.0 0.0 5000.0)) (`|MakeArray` "ObjectTypeQuery1" :!type "EObjectTypeQuery Enum")))
  (if (or (not _returnvalue_2) (> (`.Distance` (`GameplayStatics.BreakHitResult` _outhit)) (`self.MinHeight`)))
    (if (not (`ActorComponent.IsActive` _niagaratrail))
      (`NiagaraComponent.ResetSystem` _niagaratrail)
      (`ActorComponent.Activate` _niagaratrail true))
    (`SceneComponent.SetVisibility` _decal true false)
    (`MaterialInstanceDynamic.SetScalarParameterValue` _dynamicmaterial "Radius" (`KismetMathLibrary.MapRangeClamped` (`.Distance` (`GameplayStatics.BreakHitResult` _outhit)) (`self.MinHeight`) (`self.MaxHeight`) 0.5 0.05))
    (`MaterialInstanceDynamic.SetScalarParameterValue` _dynamicmaterial "Density" (`KismetMathLibrary.MapRangeClamped` (`.Distance` (`GameplayStatics.BreakHitResult` _outhit)) (`self.MinHeight`) (`self.MaxHeight`) 0.0 10.0))
    (elif (not (== (`GameplayStatics.GetObjectClass` (`self.GetOwner`)) "/Game/AbilitySystem/BP_AbilityParent.BP_AbilityParent_C"))
      (`ActorComponent.Deactivate` _niagaratrail)
      (`SceneComponent.SetVisibility` _decal false false))))

(fn `UserConstructionScript`)